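; BP_Sound_On_Spline is an actor that plays an ambient sound sliding along a spline to stay nearest the player.
; BeginPlay caches the third-person character, assigns SoundToPlay to the audio component, starts it, and optionally reveals a debug marker.
; Each Tick moves the audio component and debug marker to the spline point closest to the character, approximating a linear sound source such as a river or path.
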(event `self.ReceiveBeginPlay`
  (bind _audio (`self.Audio`))
  (bind _asbp_third_person_character (cast `/Game/Rome/Demo/PawnUE5/Demo/EpicContent/ThirdPersonBP/Blueprints/BP_ThirdPersonCharacter` (`GameplayStatics.GetPlayerCharacter` 0)))
  (set `self.Character Reference` _asbp_third_person_character)
  (`AudioComponent.SetSound` _audio (`self.Sound To Play`))
  (`AudioComponent.Play` _audio 0.0)
  (if (`self.Draw Debug`)
    (`SceneComponent.SetVisibility` (`self.DebugDraw`) true false)))

(event `self.ReceiveTick`
  (params (DeltaSeconds :type "Float (single-precision)"))
  (bind _returnvalue (`SplineComponent.FindLocationClosestToWorldLocation` (`self.Spline`) (`self.K2_GetActorLocation` (`self.Character Reference`)) "World"))
  (`SceneComponent.K2_SetWorldLocation` (`self.Audio`) _returnvalue false false)
  (`SceneComponent.K2_SetWorldLocation` (`self.DebugDraw`) _returnvalue false false))

(fn `UserConstructionScript`)