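; Quad audio emitter Blueprint, named for surrounding the player, that plays separate front-left, front-right, rear-left and rear-right sounds.
; BeginPlay assigns each sound to its audio component (FL, FR, RL, RR) and starts it.
; Tick moves all four components to the owner's root location with no directional offset, so they share one point.
; A debug capsule is also drawn at that location every tick.
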(event `self.ReceiveBeginPlay`
  (bind _fr (`self.FR`))
  (bind _rl (`self.RL`))
  (bind _rr (`self.RR`))
  (bind _fl (`self.FL`))
  (`|ExecutionSequence`
    (:`then_0`
      (`AudioComponent.SetSound` _fl (`self.Front Left`))
      (`AudioComponent.Play` _fl 0.0))
    (:`then_1`
      (`AudioComponent.SetSound` _fr (`self.Front Right`))
      (`AudioComponent.Play` _fr 0.0))
    (:`then_2`
      (`AudioComponent.SetSound` _rl (`self.Rear Left`))
      (`AudioComponent.Play` _rl 0.0))
    (:`then_3`
      (`AudioComponent.SetSound` _rr (`self.Rear Right`))
      (`AudioComponent.Play` _rr 0.0))))

(event `self.ReceiveTick`
  (params (DeltaSeconds :type "Float (single-precision)"))
  (bind _returnvalue (`SceneComponent.K2_GetComponentLocation` (`Actor.RootComponent` (`self.GetOwner`))))
  (`|ExecutionSequence`
    (:`then_0`
      (`SceneComponent.K2_SetWorldLocation` (`self.FL`) _returnvalue false false)
      (`KismetSystemLibrary.DrawDebugCapsule` _returnvalue 0.0 50.0 (struct) (struct :`R` 1.0 :`G` 0.712325 :`A` 1.0)))
    (:`then_1`
      (`SceneComponent.K2_SetWorldLocation` (`self.FR`) _returnvalue false false))
    (:`then_2`
      (`SceneComponent.K2_SetWorldLocation` (`self.RL`) _returnvalue false false))
    (:`then_3`
      (`SceneComponent.K2_SetWorldLocation` (`self.RR`) _returnvalue false false))))