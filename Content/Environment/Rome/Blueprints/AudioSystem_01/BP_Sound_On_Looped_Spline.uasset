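; Area ambience actor that plays four quad sounds (front/rear, left/right) around a looped spline zone, following the player.
; Each tick it finds the closest spline point and uses a dot product with the spline's right vector to detect whether the player is inside.
; Inside, the emitters surround the character's head; outside, they center on that spline point at head height.
; Emitters keep fixed world-axis offsets and zeroed rotation.
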(event `self.ReceiveBeginPlay`
  (bind _fl (`self.FL`))
  (bind _debugdraw (`self.DebugDraw`))
  (bind _rl (`self.RL`))
  (bind _rr (`self.RR`))
  (bind _fr (`self.FR`))
  (bind _asbp_third_person_character (cast `` (`GameplayStatics.GetPlayerCharacter` 0)))
  (set `self.Character Reference` null _asbp_third_person_character)
  (`|ExecutionSequence`
    (:`then_0`
      (`AudioComponent.SetSound` _fl (`self.Front Left`))
      (`AudioComponent.Play` _fl 0.0)
      (if (`self.DrawDebug`)
        (`SceneComponent.SetVisibility` _debugdraw true false)
        (else
          (`SceneComponent.SetVisibility` _debugdraw false false))))
    (:`then_1`
      (`AudioComponent.SetSound` _fr (`self.Front Right`))
      (`AudioComponent.Play` _fr 0.0))
    (:`then_2`
      (`AudioComponent.SetSound` _rl (`self.Rear Left`))
      (`AudioComponent.Play` _rl 0.0))
    (:`then_3`
      (`AudioComponent.SetSound` _rr (`self.Rear Right`))
      (`AudioComponent.Play` _rr 0.0))))

(event `self.ReceiveTick`
  (params (DeltaSeconds :type "Float (single-precision)"))
  (bind (_isinsidespline_ _isinsidesplinechanged_) (`self.GetIsInsideSpline`))
  (`/Engine/EditorBlueprintResources/StandardMacros.IsValid` (`GameplayStatics.GetPlayerController` 0)
    (:`Is Valid`
      (set `self.SplineCurveLocationClosestToPlayer` (`SplineComponent.FindLocationClosestToWorldLocation` (`self.Spline`) (`self.K2_GetActorLocation` (`.Character Reference` (`self.Character Reference`))) "World"))
      (if _isinsidesplinechanged_
        (set `self.IsInsideSpline` _isinsidespline_))
      (`self.SetEmittersLocationAndRotation`))))

(fn `GetControlledPawnLocation`
  (returns (ControlledPawnReference :type "Pawn Object Reference") (ControlledPawnLocation :type "Vector Structure"))
  (bind _returnvalue (`Controller.K2_GetPawn` (`GameplayStatics.GetPlayerController` 0)))
  (return _returnvalue (`self.K2_GetActorLocation` _returnvalue)))

(fn `GetIsInsideSpline`
  (returns (`IsInsideSpline?` :type Boolean) (`IsInsideSplineChanged?` :type Boolean))
  (bind _returnvalue (> (`KismetMathLibrary.Dot_VectorVector` (- (`self.SplineCurveLocationClosestToPlayer`) (`.ControlledPawnLocation` (`self.GetControlledPawnLocation`))) (`SplineComponent.FindRightVectorClosestToWorldLocation` (`self.Spline`) (`.ControlledPawnLocation` (`self.GetControlledPawnLocation`)) "World")) 0.0))
  (return _returnvalue (!= _returnvalue (`self.IsInsideSpline`))))

(fn `SetEmittersLocationAndRotation`
  (bind _fr (`self.FR`))
  (bind _rl (`self.RL`))
  (bind (_character_reference _character_reference_2) (`self.Character Reference`))
  (bind _soundemitterrotation (`self.SoundEmitterRotation`))
  (bind (_splinecurvelocationclosesttoplayer_x _splinecurvelocationclosesttoplayer_y) (`KismetMathLibrary.BreakVector` (`self.SplineCurveLocationClosestToPlayer`)))
  (bind _rr (`self.RR`))
  (bind _fl (`self.FL`))
  (bind (_soundemitterlocation_x _soundemitterlocation_y _soundemitterlocation_z) (`KismetMathLibrary.BreakVector` (`self.SoundEmitterLocation`)))
  (bind (_soundemitterlocation_x_2 _soundemitterlocation_y_2 _soundemitterlocation_z_2) (`KismetMathLibrary.BreakVector` (`self.SoundEmitterLocation`)))
  (bind (_soundemitterlocation_x_3 _soundemitterlocation_y_3 _soundemitterlocation_z_3) (`KismetMathLibrary.BreakVector` (`self.SoundEmitterLocation`)))
  (bind (_soundemitterlocation_x_4 _soundemitterlocation_y_4 _soundemitterlocation_z_4) (`KismetMathLibrary.BreakVector` (`self.SoundEmitterLocation`)))
  (bind _returnvalue (+ _soundemitterlocation_x_2 -100.0))
  (bind _returnvalue_2 (+ _soundemitterlocation_y_2 -100.0))
  (bind _rootcomponent (`Actor.RootComponent` _character_reference_2))
  (bind _returnvalue_3 (`SceneComponent.GetSocketLocation` (`Character.Mesh` _character_reference_2) "head"))
  (bind (_returnvalue_roll _returnvalue_pitch _returnvalue_yaw) (`KismetMathLibrary.BreakRotator` (`SceneComponent.K2_GetComponentRotation` _rootcomponent)))
  (bind (_returnvalue_roll_2 _returnvalue_pitch_2 _returnvalue_yaw_2) (`KismetMathLibrary.BreakRotator` (`SceneComponent.K2_GetComponentRotation` _rootcomponent)))
  (if (`self.IsInsideSpline`)
    (set `self.SoundEmitterLocation` _returnvalue_3)
    (else
      (set `self.SoundEmitterLocation` (`KismetMathLibrary.MakeVector` _splinecurvelocationclosesttoplayer_x _splinecurvelocationclosesttoplayer_y (.z _returnvalue_3)))))
  (set `self.SoundEmitterRotation` (`KismetMathLibrary.MakeRotator` (- _returnvalue_roll _returnvalue_roll_2) (- _returnvalue_pitch _returnvalue_pitch_2) (- _returnvalue_yaw _returnvalue_yaw_2)))
  (`|ExecutionSequence`
    (:`then_0`
      (`SceneComponent.K2_SetWorldRotation` _fl _soundemitterrotation false false)
      (`SceneComponent.K2_SetWorldLocation` _fl (`KismetMathLibrary.MakeVector` _returnvalue _returnvalue_2 _soundemitterlocation_z_2) false false)
      (`SceneComponent.K2_SetWorldLocation` (`self.DebugDraw`) (`KismetMathLibrary.MakeVector` _returnvalue _returnvalue_2 _soundemitterlocation_z_2) false false))
    (:`then_1`
      (`SceneComponent.K2_SetWorldRotation` _fr _soundemitterrotation false false)
      (`SceneComponent.K2_SetWorldLocation` _fr (`KismetMathLibrary.MakeVector` (+ _soundemitterlocation_x_3 100.0) (+ _soundemitterlocation_y_3 -100.0) _soundemitterlocation_z_3) false false))
    (:`then_2`
      (`SceneComponent.K2_SetWorldRotation` _rl _soundemitterrotation false false)
      (`SceneComponent.K2_SetWorldLocation` _rl (`KismetMathLibrary.MakeVector` (+ _soundemitterlocation_x_4 -100.0) (+ _soundemitterlocation_y_4 100.0) _soundemitterlocation_z_4) false false))
    (:`then_3`
      (`SceneComponent.K2_SetWorldRotation` _rr _soundemitterrotation false false)
      (`SceneComponent.K2_SetWorldLocation` _rr (`KismetMathLibrary.MakeVector` (+ _soundemitterlocation_x 100.0) (+ _soundemitterlocation_y 100.0) _soundemitterlocation_z) false false))))

(fn `UserConstructionScript`)