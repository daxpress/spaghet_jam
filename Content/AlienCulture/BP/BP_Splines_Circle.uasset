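; Construction-script actor that builds a closed, roughly circular spline of meshes that follows the ground beneath it.
; It steps around the actor at a radius with random noise, line-tracing downward and adding spline points at hits, with point count scaling with radius.
; It then tiles spline mesh components by mesh length, applying scale, forward axis and Z offset.
; The noise is unseeded, so each reconstruction changes the shape.
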(fn `UserConstructionScript`
  (bind _noise (`self.Noise`))
  (bind _returnvalue (+ (`self.StartLoc`) (* (`KismetMathLibrary.GetForwardVector` (`self.StartRot`)) (+ (`self.Radius multiplier`) (`KismetMathLibrary.RandomFloatInRange` (* _noise -1.0) _noise)))))
  ;[1 1 1] Add spline
  (bind _returnvalue_2 (`AddComponent|NODE_AddSplineComponent-0`))
  ;[1 1 1] Added spline to variable
  (bind _output_get (set `self.Spline` _returnvalue_2))
  ;[1 1 1] Spline loc to variable
  (set `self.StartLoc` (`SceneComponent.K2_GetComponentLocation` _output_get))
  ;[1 1 1] Spline rot to variable
  (set `self.StartRot` (`SceneComponent.K2_GetComponentRotation` (`self.Spline`)))
  ;[1 1 1] Remove default spline points
  (`SplineComponent.ClearSplinePoints` (`self.Spline`) true)
  ;[1 1 1] Point density is determined by the radius multiplier variable
  (set `self.How many segments` (`.ReturnValue` (`KismetMathLibrary.FMod` (`self.Radius multiplier`) 6.0)))
  ;[1 1 1] Loop
  (for _ (range (`self.How many segments`))
    ;[1 1 1] Spline's circle form
    (set `self.StartRot` (`KismetMathLibrary.MakeRotator` (.roll (`self.StartRot`)) (.pitch (`self.StartRot`)) (+ (.yaw (`self.StartRot`)) (`KismetMathLibrary.Conv_IntToDouble` (`.ReturnValue` (`KismetMathLibrary.FMod` 360.0 (`KismetMathLibrary.Conv_IntToDouble` (- (`self.How many segments`) 1))))))))
    ;[1 1 1] Trace
    (bind (_outhit _returnvalue_3) (`KismetSystemLibrary.LineTraceSingle` :`Start` (`KismetMathLibrary.MakeVector` (.x _returnvalue) (.y _returnvalue) (+ (.z _returnvalue) 100.0)) :`End` (`KismetMathLibrary.MakeVector` (.x _returnvalue) (.y _returnvalue) (- (.z _returnvalue) 1000.0)) :`TraceChannel` "TraceTypeQuery1" :`DrawTime` 2.0))
    ;[1 1 1] If there was a hit then add new spline point to ompact location
    (if _returnvalue_3
      (`SplineComponent.AddSplinePoint` (`self.Spline`) (`.ImpactPoint` (`GameplayStatics.BreakHitResult` _outhit)) "World" true)))
  ;[1 1 1] Close spline
  (`SplineComponent.SetClosedLoop` (`self.Spline`) true true)
  ;[1 1 1] Loop as many times the mesh length fits the spline length
  (for _index (range (+ (`.ReturnValue` (`KismetMathLibrary.FMod` (`SplineComponent.GetSplineLength` (`self.Spline`)) (`self.Mesh Length`))) 1))
    ;[1 1 1] Add new spline mesh and set to variable
    (bind _returnvalue_4 (`AddComponent|NODE_AddSplineMeshComponent-0`))
    (set `self.CurrentMesh` _returnvalue_4)
    ;[1 1 1] Set mesh alignment
    (`SplineMeshComponent.SetForwardAxis` (`self.CurrentMesh`) (`self.In Forward Axis`) true)
    ;[1 1 1] Set mesh scale for x and y
    (`SplineMeshComponent.SetEndScale` (`self.CurrentMesh`) (* (1.0 1.0) (`self.Scale`)) true)
    (`SplineMeshComponent.SetStartScale` (`self.CurrentMesh`) (* (1.0 1.0) (`self.Scale`)) true)
    (bind _returnvalue_5 (* _index (`self.Mesh Length`)))
    (bind _returnvalue_6 (* (+ _index 1) (`self.Mesh Length`)))
    ;[1 1 1] Set meshes locations and tangents
    (`SplineMeshComponent.SetStartAndEnd` (`self.CurrentMesh`) (`KismetMathLibrary.MakeVector` (.x (`SplineComponent.GetLocationAtDistanceAlongSpline` (`self.Spline`) _returnvalue_5 "Local")) (.y (`SplineComponent.GetLocationAtDistanceAlongSpline` (`self.Spline`) _returnvalue_5 "Local")) (+ (.z (`SplineComponent.GetLocationAtDistanceAlongSpline` (`self.Spline`) _returnvalue_5 "Local")) (`self.Z offset`))) (`SplineComponent.GetTangentAtDistanceAlongSpline` (`self.Spline`) _returnvalue_5 "Local") (`KismetMathLibrary.MakeVector` (.x (`SplineComponent.GetLocationAtDistanceAlongSpline` (`self.Spline`) _returnvalue_6 "Local")) (.y (`SplineComponent.GetLocationAtDistanceAlongSpline` (`self.Spline`) _returnvalue_6 "Local")) (+ (.z (`SplineComponent.GetLocationAtDistanceAlongSpline` (`self.Spline`) _returnvalue_6 "Local")) (`self.Z offset`))) (`SplineComponent.GetTangentAtDistanceAlongSpline` (`self.Spline`) _returnvalue_6 "Local") true)
    ;[1 1 1] Set mesh
    (`StaticMeshComponent.SetStaticMesh` (`self.CurrentMesh`) (`self.Mesh`))
    ;[1 1 1] Set meshe's location
    (`PrimitiveComponent.SetMaterial` (`self.CurrentMesh`) 0 (`StaticMesh.GetMaterial` (`self.Mesh`) 0))))