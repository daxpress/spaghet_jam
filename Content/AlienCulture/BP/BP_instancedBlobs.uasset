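; Construction-script actor that fills a configurable grid with instances of a single blob mesh, with no runtime logic.
; It assigns the mesh to the instanced component, then derives each row and column position from the loop index, spacing values and location offset.
; Each instance gets a shared scale, a random upright or flipped pitch and an unseeded random yaw within a half turn, with query and physics collision enabled.
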(event `self.ReceiveBeginPlay`)

(fn `UserConstructionScript`
  ;[1 1 1] Set Mesh
  (`StaticMeshComponent.SetStaticMesh` (`self.Mesh`) (`self.Mesh_01`))
  ;[1 1 1] Setting number of instances
  (for _index (range (* (`self.Height`) (`self.Length`)))
    ;[1 1 1] Adding mesh instances
    (`InstancedStaticMeshComponent.AddInstance` (`self.Mesh`) (`KismetMathLibrary.MakeTransform` (+ (`self.Location offset`) (.location (`KismetMathLibrary.Conv_VectorToTransform` (`KismetMathLibrary.MakeVector` (`KismetMathLibrary.Conv_IntToDouble` (* (mod _index (`self.Length`)) (`self.Length distance`))) (`KismetMathLibrary.Conv_IntToDouble` (* (/ _index (`self.Length`)) (`self.Height distance`))))))) (`KismetMathLibrary.MakeRotator` (.roll (.rotation (`KismetMathLibrary.Conv_VectorToTransform` (`KismetMathLibrary.MakeVector` (`KismetMathLibrary.Conv_IntToDouble` (* (mod _index (`self.Length`)) (`self.Length distance`))) (`KismetMathLibrary.Conv_IntToDouble` (* (/ _index (`self.Length`)) (`self.Height distance`))))))) (`|GetArrayItem` (`|MakeArray` 0.0 180.0 :!type "Float (single-precision)") (`KismetMathLibrary.RandomIntegerInRange` 0 1)) (`KismetMathLibrary.RandomFloatInRange` -180.0)) (`KismetMathLibrary.Conv_DoubleToVector` (`self.Scale`))))
    ;[1 1 1] Enable collision
    (`PrimitiveComponent.SetCollisionEnabled` (`self.Mesh`) "QueryAndPhysics")))