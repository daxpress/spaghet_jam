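; Fireplace guard prop for the Old Village meshes, with two adjustable folding wings.
; The construction script sets each wing mesh's relative yaw by lerping between two mirrored angle limits, driven by clamped LeftWingRotate and RightWingRotate values from 0 to 1.
; The event graph is empty, so the wings are posed only at construction, with no runtime logic.
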(fn `UserConstructionScript`
  (`SceneComponent.K2_SetRelativeRotation` (`self.SM_Fireplace_guard_002`) (`KismetMathLibrary.RLerp` (`KismetMathLibrary.MakeRotator` 0.0 0.0 119.0) (`KismetMathLibrary.MakeRotator` 0.0 0.0 -124.0) (`KismetMathLibrary.FClamp` (`self.Left wing rotate`))) false false)
  (`SceneComponent.K2_SetRelativeRotation` (`self.SM_Fireplace_guard_0021`) (`KismetMathLibrary.RLerp` (`KismetMathLibrary.MakeRotator` 0.0 0.0 -119.0) (`KismetMathLibrary.MakeRotator` 0.0 0.0 124.0) (`KismetMathLibrary.FClamp` (`self.Right wing rotate`))) false false))