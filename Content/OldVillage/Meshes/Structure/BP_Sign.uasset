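; BP_Sign is a configurable village sign prop, set up entirely in the Construction Script with no runtime logic.
; It creates a dynamic instance of the sign material and applies two colors, a metallic toggle and roughness.
; A sign choice from eight options maps to a scalar that flips between designs within that one material.
; A second dynamic instance on the wood board slot tints the frame.
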(fn `UserConstructionScript`
  (bind _returnvalue (`PrimitiveComponent.CreateDynamicMaterialInstance` (`self.StaticMesh`) 0 "/Game/OldVillage/Materials/Meshspecific/MI_Signs_001.MI_Signs_001" "None"))
  (`MaterialInstanceDynamic.SetVectorParameterValue` _returnvalue "Color 1" (`self.Sign Color 1`))
  (`MaterialInstanceDynamic.SetVectorParameterValue` _returnvalue "Color 2" (`self.Sign Color 2`))
  (if (`self.Metallic`)
    (set `self.Metallic value` 1.0)
    (else
      (bind _output_get (set `self.Metallic value` 0.0))))
  (`MaterialInstanceDynamic.SetScalarParameterValue` _returnvalue "Metallic" _output_get)
  (`MaterialInstanceDynamic.SetScalarParameterValue` _returnvalue "Roughness" (`self.Roughness`))
  (switch `int` (`self.Choose sign`)
    (:`1`
      (set `self.Set sign value` 0.0))
    (:`2`
      (set `self.Set sign value` 0.2))
    (:`3`
      (set `self.Set sign value` 0.3))
    (:`4`
      (set `self.Set sign value` 0.4))
    (:`5`
      (set `self.Set sign value` 0.5))
    (:`6`
      (set `self.Set sign value` 0.65))
    (:`7`
      (set `self.Set sign value` 0.75))
    (:`8`
      (bind _output_get_2 (set `self.Set sign value` 0.9))))
  (`MaterialInstanceDynamic.SetScalarParameterValue` _returnvalue "Flip between signs" _output_get_2)
  (bind _returnvalue_2 (`PrimitiveComponent.CreateDynamicMaterialInstance` (`self.StaticMesh`) 3 "/Game/OldVillage/Materials/Tileable/MI_Wood_Board_001.MI_Wood_Board_001" "None"))
  (`MaterialInstanceDynamic.SetVectorParameterValue` _returnvalue_2 "Color Multiplier" (`self.Frame Tint`)))