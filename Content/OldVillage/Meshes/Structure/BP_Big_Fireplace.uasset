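; Modular big fireplace prop for the old village, assembled in the Construction Script with no active runtime logic.
; AddHeightToTheFireplaceInMeters stacks up to three one-meter step meshes, with AbbandonedBuilding selecting abandoned mesh variants.
; AddBackWall adds a back piece with matching height steps and an optional bottom piece, all using the exterior material override.
; The body takes the interior override, while decorative stones get a fixed dirty material.
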(fn `UserConstructionScript`
  (bind _staticmesh (`self.StaticMesh`))
  (bind _fireplace (`self.fireplace`))
  (bind _fireplace_2 (`self.fireplace`))
  (bind _fireplace_3 (`self.fireplace`))
  (bind _fireplace_4 (`self.fireplace`))
  (bind _staticmesh_2 (`self.StaticMesh`))
  (bind _staticmesh_3 (`self.StaticMesh`))
  (bind _staticmesh1 (`self.StaticMesh1`))
  (bind _staticmesh1_2 (`self.StaticMesh1`))
  (bind _staticmesh2 (`self.StaticMesh2`))
  (bind _staticmesh_4 (`self.StaticMesh`))
  (bind _staticmesh1_3 (`self.StaticMesh1`))
  (bind _staticmesh_5 (`self.StaticMesh`))
  (bind _staticmesh1_4 (`self.StaticMesh1`))
  (bind _staticmesh2_2 (`self.StaticMesh2`))
  (bind _staticmesh_6 (`self.StaticMesh`))
  (bind _staticmesh3 (`self.StaticMesh3`))
  (bind _staticmesh3_2 (`self.StaticMesh3`))
  (bind _staticmesh3_3 (`self.StaticMesh3`))
  (bind _staticmesh4 (`self.StaticMesh4`))
  (bind _staticmesh3_4 (`self.StaticMesh3`))
  (bind _staticmesh3_5 (`self.StaticMesh3`))
  (bind _staticmesh4_2 (`self.StaticMesh4`))
  (bind _staticmesh4_3 (`self.StaticMesh4`))
  (bind _staticmesh5 (`self.StaticMesh5`))
  (bind _staticmesh3_6 (`self.StaticMesh3`))
  (bind _staticmesh4_4 (`self.StaticMesh4`))
  (bind _staticmesh3_7 (`self.StaticMesh3`))
  (bind _staticmesh4_5 (`self.StaticMesh4`))
  (bind _staticmesh5_2 (`self.StaticMesh5`))
  (bind _staticmesh5_3 (`self.StaticMesh5`))
  (bind _staticmesh3_8 (`self.StaticMesh3`))
  (bind _staticmesh4_6 (`self.StaticMesh4`))
  (bind _staticmesh5_4 (`self.StaticMesh5`))
  (bind _staticmesh6 (`self.StaticMesh6`))
  (bind _staticmesh6_2 (`self.StaticMesh6`))
  (bind _staticmesh7 (`self.StaticMesh7`))
  (`PrimitiveComponent.SetMaterial` (`self.fireplace`) 1 (`self.Interior Material Override`))
  (`PrimitiveComponent.SetMaterial` (`self.StaticMesh1`) 0 (`self.Interior Material Override`))
  (`PrimitiveComponent.SetMaterial` (`self.StaticMesh2`) 0 (`self.Interior Material Override`))
  (`PrimitiveComponent.SetMaterial` (`self.StaticMesh`) 0 (`self.Interior Material Override`))
  (`PrimitiveComponent.SetMaterial` (`self.SM_Decorative_Stone_001`) 0 "/Game/OldVillage/Materials/Meshspecific/MI_Decorative_Stones_001_dirty.MI_Decorative_Stones_001_dirty")
  (`PrimitiveComponent.SetMaterial` (`self.SM_Decorative_Stone_003`) 0 "/Game/OldVillage/Materials/Meshspecific/MI_Decorative_Stones_001_dirty.MI_Decorative_Stones_001_dirty")
  (`PrimitiveComponent.SetMaterial` (`self.SM_Decorative_Stone_006`) 0 "/Game/OldVillage/Materials/Meshspecific/MI_Decorative_Stones_001_dirty.MI_Decorative_Stones_001_dirty")
  (`PrimitiveComponent.SetMaterial` (`self.SM_Decorative_Stone_002`) 0 "/Game/OldVillage/Materials/Meshspecific/MI_Decorative_Stones_001_dirty.MI_Decorative_Stones_001_dirty")
  (`PrimitiveComponent.SetMaterial` (`self.SM_Decorative_Stone_010`) 0 "/Game/OldVillage/Materials/Meshspecific/MI_Decorative_Stones_001_dirty.MI_Decorative_Stones_001_dirty")
  (`PrimitiveComponent.SetMaterial` (`self.SM_Decorative_Stone_004`) 0 "/Game/OldVillage/Materials/Meshspecific/MI_Decorative_Stones_001_dirty.MI_Decorative_Stones_001_dirty")
  (`PrimitiveComponent.SetMaterial` (`self.SM_Decorative_Stone_009`) 0 "/Game/OldVillage/Materials/Meshspecific/MI_Decorative_Stones_001_dirty.MI_Decorative_Stones_001_dirty")
  (`PrimitiveComponent.SetMaterial` (`self.SM_Decorative_Stone_005`) 0 "/Game/OldVillage/Materials/Meshspecific/MI_Decorative_Stones_001_dirty.MI_Decorative_Stones_001_dirty")
  (`PrimitiveComponent.SetMaterial` (`self.SM_Decorative_Stone_0021`) 0 "/Game/OldVillage/Materials/Meshspecific/MI_Decorative_Stones_001_dirty.MI_Decorative_Stones_001_dirty")
  (switch `int` (`self.Add height to the fireplace (in meters)`)
    (:`0`
      (if (`self.Abbandoned building`)
        (`StaticMeshComponent.SetStaticMesh` _fireplace_2 "/Game/OldVillage/Meshes/Structure_Components/SM_Fireplace_002_abbandoned.SM_Fireplace_002_abbandoned")
        (`SceneComponent.K2_SetRelativeTransform` _fireplace_2 (`KismetMathLibrary.MakeTransform` (0.0 0.0 0.0) (struct)) false false)
        (if (`self.Add back wall`)
          (`StaticMeshComponent.SetStaticMesh` _staticmesh3 "/Game/OldVillage/Meshes/Structure_Components/SM_Fireplace_back_002.SM_Fireplace_back_002")
          (`SceneComponent.K2_SetRelativeTransform` _staticmesh3 (`KismetMathLibrary.MakeTransform` (0.0 0.0 0.0) (struct)) false false)
          (if (`self.Add back wall bottom`) :!label _label
            (`StaticMeshComponent.SetStaticMesh` _staticmesh7 "/Game/OldVillage/Meshes/Structure_Components/SM_Fireplace_step_006.SM_Fireplace_step_006")
            (`SceneComponent.K2_SetRelativeTransform` _staticmesh7 (`KismetMathLibrary.MakeTransform` (0.0 0.0 0.0) (struct)) false false))
          (`PrimitiveComponent.SetMaterial` (`self.StaticMesh4`) 0 (`self.Exterior Material Override`))
          (`PrimitiveComponent.SetMaterial` (`self.StaticMesh5`) 0 (`self.Exterior Material Override`))
          (`PrimitiveComponent.SetMaterial` (`self.StaticMesh6`) 0 (`self.Exterior Material Override`))
          (`PrimitiveComponent.SetMaterial` (`self.StaticMesh7`) 0 (`self.Exterior Material Override`))
          (`PrimitiveComponent.SetMaterial` (`self.StaticMesh3`) 0 (`self.Exterior Material Override`)))
        (elif (`self.Add back wall`)
          (`StaticMeshComponent.SetStaticMesh` _staticmesh3_2 "/Game/OldVillage/Meshes/Structure_Components/SM_Fireplace_back_002.SM_Fireplace_back_002")
          (`SceneComponent.K2_SetRelativeTransform` _staticmesh3_2 (`KismetMathLibrary.MakeTransform` (0.0 0.0 0.0) (struct)) false false)
          (goto _label))))
    (:`1`
      (if (`self.Abbandoned building`)
        (`StaticMeshComponent.SetStaticMesh` _fireplace_3 "/Game/OldVillage/Meshes/Structure_Components/SM_Fireplace_002_abbandoned.SM_Fireplace_002_abbandoned")
        (`SceneComponent.K2_SetRelativeTransform` _fireplace_3 (`KismetMathLibrary.MakeTransform` (0.0 0.0 0.0) (struct)) false false)
        (`StaticMeshComponent.SetStaticMesh` _staticmesh "/Game/OldVillage/Meshes/Structure_Components/SM_Fireplace_step_002_abbandoned.SM_Fireplace_step_002_abbandoned")
        (`SceneComponent.K2_SetRelativeTransform` _staticmesh (`KismetMathLibrary.MakeTransform` (0.0 0.0 0.0) (struct)) false false)
        (if (`self.Add back wall`)
          (`StaticMeshComponent.SetStaticMesh` _staticmesh3_3 "/Game/OldVillage/Meshes/Structure_Components/SM_Fireplace_back_002.SM_Fireplace_back_002")
          (`SceneComponent.K2_SetRelativeTransform` _staticmesh3_3 (`KismetMathLibrary.MakeTransform` (0.0 0.0 0.0) (struct)) false false)
          (`StaticMeshComponent.SetStaticMesh` _staticmesh4 "/Game/OldVillage/Meshes/Structure_Components/SM_Fireplace_step_005.SM_Fireplace_step_005")
          (`SceneComponent.K2_SetRelativeTransform` _staticmesh4 (`KismetMathLibrary.MakeTransform` (0.0 0.0 0.0) (struct)) false false)
          (goto _label))
        (else
          (`StaticMeshComponent.SetStaticMesh` _staticmesh_6 "/Game/OldVillage/Meshes/Structure_Components/SM_Fireplace_step_002.SM_Fireplace_step_002")
          (`SceneComponent.K2_SetRelativeTransform` _staticmesh_6 (`KismetMathLibrary.MakeTransform` (0.0 0.0 0.0) (struct)) false false)
          (if (`self.Add back wall`)
            (`StaticMeshComponent.SetStaticMesh` _staticmesh3_5 "/Game/OldVillage/Meshes/Structure_Components/SM_Fireplace_back_002.SM_Fireplace_back_002")
            (`SceneComponent.K2_SetRelativeTransform` _staticmesh3_5 (`KismetMathLibrary.MakeTransform` (0.0 0.0 0.0) (struct)) false false)
            (`StaticMeshComponent.SetStaticMesh` _staticmesh4_2 "/Game/OldVillage/Meshes/Structure_Components/SM_Fireplace_step_005.SM_Fireplace_step_005")
            (`SceneComponent.K2_SetRelativeTransform` _staticmesh4_2 (`KismetMathLibrary.MakeTransform` (0.0 0.0 0.0) (struct)) false false)
            (goto _label)))))
    (:`2`
      (if (`self.Abbandoned building`)
        (`StaticMeshComponent.SetStaticMesh` _fireplace_4 "/Game/OldVillage/Meshes/Structure_Components/SM_Fireplace_002_abbandoned.SM_Fireplace_002_abbandoned")
        (`SceneComponent.K2_SetRelativeTransform` _fireplace_4 (`KismetMathLibrary.MakeTransform` (0.0 0.0 0.0) (struct)) false false)
        (`StaticMeshComponent.SetStaticMesh` _staticmesh_3 "/Game/OldVillage/Meshes/Structure_Components/SM_Fireplace_step_002_abbandoned.SM_Fireplace_step_002_abbandoned")
        (`SceneComponent.K2_SetRelativeTransform` _staticmesh_3 (`KismetMathLibrary.MakeTransform` (0.0 0.0 0.0) (struct)) false false)
        (`StaticMeshComponent.SetStaticMesh` _staticmesh1 "/Game/OldVillage/Meshes/Structure_Components/SM_Fireplace_step_002_abbandoned.SM_Fireplace_step_002_abbandoned")
        (`SceneComponent.K2_SetRelativeTransform` _staticmesh1 (`KismetMathLibrary.MakeTransform` (0.0 0.0 100.0) (struct)) false false)
        (if (`self.Add back wall`)
          (`StaticMeshComponent.SetStaticMesh` _staticmesh3_4 "/Game/OldVillage/Meshes/Structure_Components/SM_Fireplace_back_002.SM_Fireplace_back_002")
          (`SceneComponent.K2_SetRelativeTransform` _staticmesh3_4 (`KismetMathLibrary.MakeTransform` (0.0 0.0 0.0) (struct)) false false)
          (`StaticMeshComponent.SetStaticMesh` _staticmesh4_3 "/Game/OldVillage/Meshes/Structure_Components/SM_Fireplace_step_005.SM_Fireplace_step_005")
          (`SceneComponent.K2_SetRelativeTransform` _staticmesh4_3 (`KismetMathLibrary.MakeTransform` (0.0 0.0 0.0) (struct)) false false)
          (`StaticMeshComponent.SetStaticMesh` _staticmesh5 "/Game/OldVillage/Meshes/Structure_Components/SM_Fireplace_step_005.SM_Fireplace_step_005")
          (`SceneComponent.K2_SetRelativeTransform` _staticmesh5 (`KismetMathLibrary.MakeTransform` (0.0 0.0 100.0) (struct)) false false)
          (goto _label))
        (else
          (`StaticMeshComponent.SetStaticMesh` _staticmesh_4 "/Game/OldVillage/Meshes/Structure_Components/SM_Fireplace_step_002.SM_Fireplace_step_002")
          (`SceneComponent.K2_SetRelativeTransform` _staticmesh_4 (`KismetMathLibrary.MakeTransform` (0.0 0.0 0.0) (struct)) false false)
          (`StaticMeshComponent.SetStaticMesh` _staticmesh1_3 "/Game/OldVillage/Meshes/Structure_Components/SM_Fireplace_step_002.SM_Fireplace_step_002")
          (`SceneComponent.K2_SetRelativeTransform` _staticmesh1_3 (`KismetMathLibrary.MakeTransform` (0.0 0.0 100.0) (struct)) false false)
          (if (`self.Add back wall`)
            (`StaticMeshComponent.SetStaticMesh` _staticmesh3_7 "/Game/OldVillage/Meshes/Structure_Components/SM_Fireplace_back_002.SM_Fireplace_back_002")
            (`SceneComponent.K2_SetRelativeTransform` _staticmesh3_7 (`KismetMathLibrary.MakeTransform` (0.0 0.0 0.0) (struct)) false false)
            (`StaticMeshComponent.SetStaticMesh` _staticmesh4_5 "/Game/OldVillage/Meshes/Structure_Components/SM_Fireplace_step_005.SM_Fireplace_step_005")
            (`SceneComponent.K2_SetRelativeTransform` _staticmesh4_5 (`KismetMathLibrary.MakeTransform` (0.0 0.0 0.0) (struct)) false false)
            (`StaticMeshComponent.SetStaticMesh` _staticmesh5_2 "/Game/OldVillage/Meshes/Structure_Components/SM_Fireplace_step_005.SM_Fireplace_step_005")
            (`SceneComponent.K2_SetRelativeTransform` _staticmesh5_2 (`KismetMathLibrary.MakeTransform` (0.0 0.0 100.0) (struct)) false false)
            (goto _label)))))
    (:`3`
      (if (`self.Abbandoned building`)
        (`StaticMeshComponent.SetStaticMesh` _fireplace "/Game/OldVillage/Meshes/Structure_Components/SM_Fireplace_002_abbandoned.SM_Fireplace_002_abbandoned")
        (`SceneComponent.K2_SetRelativeTransform` _fireplace (`KismetMathLibrary.MakeTransform` (0.0 0.0 0.0) (struct)) false false)
        (`StaticMeshComponent.SetStaticMesh` _staticmesh_2 "/Game/OldVillage/Meshes/Structure_Components/SM_Fireplace_step_002_abbandoned.SM_Fireplace_step_002_abbandoned")
        (`SceneComponent.K2_SetRelativeTransform` _staticmesh_2 (`KismetMathLibrary.MakeTransform` (0.0 0.0 0.0) (struct)) false false)
        (`StaticMeshComponent.SetStaticMesh` _staticmesh1_2 "/Game/OldVillage/Meshes/Structure_Components/SM_Fireplace_step_002_abbandoned.SM_Fireplace_step_002_abbandoned")
        (`SceneComponent.K2_SetRelativeTransform` _staticmesh1_2 (`KismetMathLibrary.MakeTransform` (0.0 0.0 100.0) (struct)) false false)
        (`StaticMeshComponent.SetStaticMesh` _staticmesh2 "/Game/OldVillage/Meshes/Structure_Components/SM_Fireplace_step_002_abbandoned.SM_Fireplace_step_002_abbandoned")
        (`SceneComponent.K2_SetRelativeTransform` _staticmesh2 (`KismetMathLibrary.MakeTransform` (0.0 0.0 200.0) (struct)) false false)
        (if (`self.Add back wall`)
          (`StaticMeshComponent.SetStaticMesh` _staticmesh3_6 "/Game/OldVillage/Meshes/Structure_Components/SM_Fireplace_back_002.SM_Fireplace_back_002")
          (`SceneComponent.K2_SetRelativeTransform` _staticmesh3_6 (`KismetMathLibrary.MakeTransform` (0.0 0.0 0.0) (struct)) false false)
          (`StaticMeshComponent.SetStaticMesh` _staticmesh4_4 "/Game/OldVillage/Meshes/Structure_Components/SM_Fireplace_step_005.SM_Fireplace_step_005")
          (`SceneComponent.K2_SetRelativeTransform` _staticmesh4_4 (`KismetMathLibrary.MakeTransform` (0.0 0.0 0.0) (struct)) false false)
          (`StaticMeshComponent.SetStaticMesh` _staticmesh5_3 "/Game/OldVillage/Meshes/Structure_Components/SM_Fireplace_step_005.SM_Fireplace_step_005")
          (`SceneComponent.K2_SetRelativeTransform` _staticmesh5_3 (`KismetMathLibrary.MakeTransform` (0.0 0.0 100.0) (struct)) false false)
          (`StaticMeshComponent.SetStaticMesh` _staticmesh6_2 "/Game/OldVillage/Meshes/Structure_Components/SM_Fireplace_step_005.SM_Fireplace_step_005")
          (`SceneComponent.K2_SetRelativeTransform` _staticmesh6_2 (`KismetMathLibrary.MakeTransform` (0.0 0.0 200.0) (struct)) false false)
          (goto _label))
        (else
          (`StaticMeshComponent.SetStaticMesh` _staticmesh_5 "/Game/OldVillage/Meshes/Structure_Components/SM_Fireplace_step_002.SM_Fireplace_step_002")
          (`SceneComponent.K2_SetRelativeTransform` _staticmesh_5 (`KismetMathLibrary.MakeTransform` (0.0 0.0 0.0) (struct)) false false)
          (`StaticMeshComponent.SetStaticMesh` _staticmesh1_4 "/Game/OldVillage/Meshes/Structure_Components/SM_Fireplace_step_002.SM_Fireplace_step_002")
          (`SceneComponent.K2_SetRelativeTransform` _staticmesh1_4 (`KismetMathLibrary.MakeTransform` (0.0 0.0 100.0) (struct)) false false)
          (`StaticMeshComponent.SetStaticMesh` _staticmesh2_2 "/Game/OldVillage/Meshes/Structure_Components/SM_Fireplace_step_002.SM_Fireplace_step_002")
          (`SceneComponent.K2_SetRelativeTransform` _staticmesh2_2 (`KismetMathLibrary.MakeTransform` (0.0 0.0 200.0) (struct)) false false)
          (if (`self.Add back wall`)
            (`StaticMeshComponent.SetStaticMesh` _staticmesh3_8 "/Game/OldVillage/Meshes/Structure_Components/SM_Fireplace_back_002.SM_Fireplace_back_002")
            (`SceneComponent.K2_SetRelativeTransform` _staticmesh3_8 (`KismetMathLibrary.MakeTransform` (0.0 0.0 0.0) (struct)) false false)
            (`StaticMeshComponent.SetStaticMesh` _staticmesh4_6 "/Game/OldVillage/Meshes/Structure_Components/SM_Fireplace_step_005.SM_Fireplace_step_005")
            (`SceneComponent.K2_SetRelativeTransform` _staticmesh4_6 (`KismetMathLibrary.MakeTransform` (0.0 0.0 0.0) (struct)) false false)
            (`StaticMeshComponent.SetStaticMesh` _staticmesh5_4 "/Game/OldVillage/Meshes/Structure_Components/SM_Fireplace_step_005.SM_Fireplace_step_005")
            (`SceneComponent.K2_SetRelativeTransform` _staticmesh5_4 (`KismetMathLibrary.MakeTransform` (0.0 0.0 100.0) (struct)) false false)
            (`StaticMeshComponent.SetStaticMesh` _staticmesh6 "/Game/OldVillage/Meshes/Structure_Components/SM_Fireplace_step_005.SM_Fireplace_step_005")
            (`SceneComponent.K2_SetRelativeTransform` _staticmesh6 (`KismetMathLibrary.MakeTransform` (0.0 0.0 200.0) (struct)) false false)
            (goto _label)))))))