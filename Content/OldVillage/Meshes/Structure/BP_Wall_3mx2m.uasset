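; Configurable 3m x 2m building wall piece for the Old Village set, switchable between basic wall, window and inward corner variants, with abandoned versions.
; The Construction Script applies material overrides and a stucco tint, then swaps meshes and transforms on preset components.
; Window options add shutters posed by clamped open/closed lerps and stone or wood surrounds.
; In abandoned windows, glass is selectable, and shutters and surrounds only follow a valid support choice.
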(fn `UserConstructionScript`
  (bind _returnvalue (`KismetMathLibrary.MakeTransform` (222.722534 -7.872087 37.132233) (struct :`Yaw` -89.999992) (1.0 1.0 1.0)))
  (bind _staticmesh11 (`self.StaticMesh11`))
  (bind _staticmesh12 (`self.StaticMesh12`))
  (bind _staticmesh13 (`self.StaticMesh13`))
  (bind _staticmesh10 (`self.StaticMesh10`))
  (bind _staticmesh8 (`self.StaticMesh8`))
  (bind _staticmesh9 (`self.StaticMesh9`))
  (bind _staticmesh8_2 (`self.StaticMesh8`))
  (bind _staticmesh9_2 (`self.StaticMesh9`))
  (bind _staticmesh11_2 (`self.StaticMesh11`))
  (bind _exterior_material_override (`self.Exterior Material Override`))
  (bind _staticmesh (`self.StaticMesh`))
  (bind _staticmesh_2 (`self.StaticMesh`))
  (bind _staticmesh_3 (`self.StaticMesh`))
  (bind _staticmesh_4 (`self.StaticMesh`))
  (bind _staticmesh_5 (`self.StaticMesh`))
  (bind _staticmesh_6 (`self.StaticMesh`))
  (bind _staticmesh1 (`self.StaticMesh1`))
  (bind _staticmesh3 (`self.StaticMesh3`))
  (bind _staticmesh4 (`self.StaticMesh4`))
  (bind _staticmesh5 (`self.StaticMesh5`))
  (bind _staticmesh6 (`self.StaticMesh6`))
  (bind _staticmesh7 (`self.StaticMesh7`))
  (bind _staticmesh_7 (`self.StaticMesh`))
  (bind _staticmesh1_2 (`self.StaticMesh1`))
  (bind _staticmesh4_2 (`self.StaticMesh4`))
  (bind _staticmesh5_2 (`self.StaticMesh5`))
  (bind _staticmesh6_2 (`self.StaticMesh6`))
  (bind _staticmesh7_2 (`self.StaticMesh7`))
  (bind _staticmesh2 (`self.StaticMesh2`))
  (bind _staticmesh_8 (`self.StaticMesh`))
  (bind _staticmesh2_2 (`self.StaticMesh2`))
  (bind _staticmesh2_3 (`self.StaticMesh2`))
  (bind _staticmesh3_2 (`self.StaticMesh3`))
  (bind _staticmesh2_4 (`self.StaticMesh2`))
  (bind _staticmesh3_3 (`self.StaticMesh3`))
  (bind _staticmesh8_3 (`self.StaticMesh8`))
  (bind _staticmesh9_3 (`self.StaticMesh9`))
  (bind _staticmesh11_3 (`self.StaticMesh11`))
  (bind _staticmesh12_2 (`self.StaticMesh12`))
  (bind _staticmesh13_2 (`self.StaticMesh13`))
  (bind _staticmesh10_2 (`self.StaticMesh10`))
  (bind _staticmesh8_4 (`self.StaticMesh8`))
  (bind _staticmesh9_4 (`self.StaticMesh9`))
  (bind _staticmesh11_4 (`self.StaticMesh11`))
  (bind _staticmesh12_3 (`self.StaticMesh12`))
  (bind _staticmesh13_3 (`self.StaticMesh13`))
  (bind _staticmesh10_3 (`self.StaticMesh10`))
  (bind _staticmesh8_5 (`self.StaticMesh8`))
  (bind _staticmesh9_5 (`self.StaticMesh9`))
  (bind _staticmesh11_5 (`self.StaticMesh11`))
  (`PrimitiveComponent.SetMaterial` _staticmesh_4 0 (`self.Interior Material Override`))
  (`PrimitiveComponent.SetMaterial` _staticmesh_4 1 _exterior_material_override)
  ;[1 1 1] Change stucco Color
  (bind _returnvalue_2 (`PrimitiveComponent.CreateDynamicMaterialInstance` (`self.StaticMesh`) 1 _exterior_material_override "None"))
  (`MaterialInstanceDynamic.SetVectorParameterValue` _returnvalue_2 "Material 2 Color multiplier" (`self.Stucco Color`))
  (switch `/Game/OldVillage/Meshes/Structure/Enumerators/BP_3mx2m_Enum` (`self.Choose component`)
    (:`NewEnumerator0`
      (if (`self.Abbandoned building`)
        ;[1 1 1] Basic Wall
        (`StaticMeshComponent.SetStaticMesh` _staticmesh_8 "/Game/OldVillage/Meshes/Structure_Components/SM_Wall_3mx2m_001_abbandoned.SM_Wall_3mx2m_001_abbandoned")
        (`SceneComponent.K2_SetRelativeTransform` _staticmesh_8 (`KismetMathLibrary.MakeTransform` (0.0 0.0 0.0) (struct)) false false)))
    (:`NewEnumerator1`
      (if (`self.Abbandoned building`)
        ;[1 1 1] Window 01 - Abbandoned
        ;;[1 1 1] Base
        (`StaticMeshComponent.SetStaticMesh` _staticmesh_6 "/Game/OldVillage/Meshes/Structure_Components/SM_Wall_3mx2m_window_001_component_abbandoned.SM_Wall_3mx2m_window_001_component_abbandoned")
        (`SceneComponent.K2_SetRelativeTransform` _staticmesh_6 (`KismetMathLibrary.MakeTransform` (0.0 0.0 0.0) (struct)) false false)
        ;;[1 1 1] Window body
        (`StaticMeshComponent.SetStaticMesh` _staticmesh1 "/Game/OldVillage/Meshes/Structure_Components/SM_Window_001_abbandoned_frame.SM_Window_001_abbandoned_frame")
        (`SceneComponent.K2_SetRelativeTransform` _staticmesh1 (`KismetMathLibrary.MakeTransform` (222.722534 -7.872087 37.132233) (struct :`Yaw` -89.999992) (1.0 1.0 1.0)) false false)
        (switch `int` (`self.Choose abbandoned window glass`)
          (:`0`
            ;;[1 1 1] Glass
            (`StaticMeshComponent.SetStaticMesh` _staticmesh2_2 "/Game/OldVillage/Meshes/Structure_Components/SM_Window_001_abbandoned_glass_001.SM_Window_001_abbandoned_glass_001" :!label _label)
            (`SceneComponent.K2_SetRelativeTransform` _staticmesh2_2 (`KismetMathLibrary.MakeTransform` (222.722534 -7.872087 37.132233) (struct :`Yaw` -89.999992) (1.0 1.0 1.0)) false false))
          (:`1`
            (goto _label))
          (:`2`
            ;;[1 1 1] Glass 2
            (`StaticMeshComponent.SetStaticMesh` _staticmesh2_3 "/Game/OldVillage/Meshes/Structure_Components/SM_Window_001_abbandoned_glass_002.SM_Window_001_abbandoned_glass_002")
            (`SceneComponent.K2_SetRelativeTransform` _staticmesh2_3 (`KismetMathLibrary.MakeTransform` (222.722534 -7.872087 37.132233) (struct :`Yaw` -89.999992) (1.0 1.0 1.0)) false false))
          (:`3`
            ;;[1 1 1] Glass 2
            (`StaticMeshComponent.SetStaticMesh` _staticmesh2_4 "/Game/OldVillage/Meshes/Structure_Components/SM_Window_001_abbandoned_glass_003.SM_Window_001_abbandoned_glass_003")
            (`SceneComponent.K2_SetRelativeTransform` _staticmesh2_4 (`KismetMathLibrary.MakeTransform` (222.722534 -7.872087 37.132233) (struct :`Yaw` -89.999992) (1.0 1.0 1.0)) false false))
          (:`4`
            ;;[1 1 1] Glass 4
            (`StaticMeshComponent.SetStaticMesh` _staticmesh2 "/Game/OldVillage/Meshes/Structure_Components/SM_Window_001_abbandoned_glass_004.SM_Window_001_abbandoned_glass_004")
            (`SceneComponent.K2_SetRelativeTransform` _staticmesh2 (`KismetMathLibrary.MakeTransform` (222.722534 -7.872087 37.132233) (struct :`Yaw` -89.999992) (1.0 1.0 1.0)) false false)))
        (switch `int` (`self.Choose abbandoned window support`)
          (:`1`
            ;;[1 1 1] Window support
            (`StaticMeshComponent.SetStaticMesh` _staticmesh3_2 "/Game/OldVillage/Meshes/Structure_Components/SM_Window_001_abbandoned_support_001.SM_Window_001_abbandoned_support_001")
            (`SceneComponent.K2_SetRelativeTransform` _staticmesh3_2 _returnvalue false false))
          (:`2`
            ;;[1 1 1] Window support
            (`StaticMeshComponent.SetStaticMesh` _staticmesh3_3 "/Game/OldVillage/Meshes/Structure_Components/SM_Window_001_abbandoned_support_002.SM_Window_001_abbandoned_support_002")
            (`SceneComponent.K2_SetRelativeTransform` _staticmesh3_3 _returnvalue false false))
          (:`3`
            ;;[1 1 1] Window support
            (`StaticMeshComponent.SetStaticMesh` _staticmesh3 "/Game/OldVillage/Meshes/Structure_Components/SM_Window_001_abbandoned_support_003.SM_Window_001_abbandoned_support_003")
            (`SceneComponent.K2_SetRelativeTransform` _staticmesh3 _returnvalue false false)))
        ;;[1 1 1] Shutters support
        (`StaticMeshComponent.SetStaticMesh` _staticmesh4 "/Game/OldVillage/Meshes/Structure_Components/SM_Window_Shutter_001_support_abbandoned.SM_Window_Shutter_001_support_abbandoned")
        (`SceneComponent.K2_SetRelativeTransform` _staticmesh4 (`KismetMathLibrary.MakeTransform` (77.500229 18.251007 39.752438) (struct :`Yaw` -89.999992)) false false)
        (`StaticMeshComponent.SetStaticMesh` _staticmesh5 "/Game/OldVillage/Meshes/Structure_Components/SM_Window_Shutter_001_support_abbandoned.SM_Window_Shutter_001_support_abbandoned")
        (`SceneComponent.K2_SetRelativeTransform` _staticmesh5 (`KismetMathLibrary.MakeTransform` (240.756271 18.250992 39.752438) (struct :`Yaw` -89.999992) (1.0 -1.0 1.0)) false false)
        ;;[1 1 1] Remove left shutter
        (if (not (`self.Remove left shutter`))
          ;;[1 1 1] Ledt Shutter
          (`StaticMeshComponent.SetStaticMesh` _staticmesh6 "/Game/OldVillage/Meshes/Structure_Components/SM_Window_Shutter_001_abbandoned.SM_Window_Shutter_001_abbandoned")
          (`SceneComponent.K2_SetRelativeTransform` _staticmesh6 (`KismetMathLibrary.MakeTransform` (77.500229 18.251007 39.752438) (struct :`Yaw` -90.0)) false false))
        ;;[1 1 1] Remove right shutter
        (if (not (`self.Remove right shutter`))
          ;;[1 1 1] Right Shutter
          (`StaticMeshComponent.SetStaticMesh` _staticmesh7 "/Game/OldVillage/Meshes/Structure_Components/SM_Window_Shutter_001_abbandoned.SM_Window_Shutter_001_abbandoned")
          (`SceneComponent.K2_SetRelativeTransform` _staticmesh7 (`KismetMathLibrary.MakeTransform` (240.756271 18.250992 39.752438) (struct :`Yaw` -90.0) (1.0 -1.0 1.0)) false false))
        ;;[1 1 1] Shutters movement
        (`SceneComponent.K2_SetRelativeRotation` _staticmesh6 (`KismetMathLibrary.RLerp` (`KismetMathLibrary.MakeRotator` 0.0 0.0 -90.0) (`KismetMathLibrary.MakeRotator` 0.0 0.0 100.0) (`KismetMathLibrary.FClamp` (`self.Left shutter - 1 = Open 0 = Closed`))) false false)
        (`SceneComponent.K2_SetRelativeRotation` _staticmesh7 (`KismetMathLibrary.RLerp` (`KismetMathLibrary.MakeRotator` 0.0 0.0 -90.0) (`KismetMathLibrary.MakeRotator` 0.0 0.0 -280.0) (`KismetMathLibrary.FClamp` (`self.Right shutter - 1 = Open 0 = Closed`))) false false)
        (else
          ;[1 1 1] Window 01
          ;;[1 1 1] Base
          (`StaticMeshComponent.SetStaticMesh` _staticmesh_7 "/Game/OldVillage/Meshes/Structure_Components/SM_Wall_3mx2m_window_001_component.SM_Wall_3mx2m_window_001_component")
          (`SceneComponent.K2_SetRelativeTransform` _staticmesh_7 (`KismetMathLibrary.MakeTransform` (0.0 0.0 0.0) (struct)) false false)
          ;;[1 1 1] Window body
          (`StaticMeshComponent.SetStaticMesh` _staticmesh1_2 "/Game/OldVillage/Meshes/Structure_Components/SM_Window_001.SM_Window_001")
          (`SceneComponent.K2_SetRelativeTransform` _staticmesh1_2 (`KismetMathLibrary.MakeTransform` (222.722534 -7.872087 37.132233) (struct :`Yaw` -89.999992) (1.0 1.0 1.0)) false false)
          ;;[1 1 1] Shutters support
          (`StaticMeshComponent.SetStaticMesh` _staticmesh4_2 "/Game/OldVillage/Meshes/Structure_Components/SM_Window_Shutter_001_support.SM_Window_Shutter_001_support")
          (`SceneComponent.K2_SetRelativeTransform` _staticmesh4_2 (`KismetMathLibrary.MakeTransform` (77.500229 18.251007 39.752438) (struct :`Yaw` -89.999992)) false false)
          (`StaticMeshComponent.SetStaticMesh` _staticmesh5_2 "/Game/OldVillage/Meshes/Structure_Components/SM_Window_Shutter_001_support.SM_Window_Shutter_001_support")
          (`SceneComponent.K2_SetRelativeTransform` _staticmesh5_2 (`KismetMathLibrary.MakeTransform` (240.756271 18.250992 39.752438) (struct :`Yaw` -89.999992) (1.0 -1.0 1.0)) false false)
          ;;[1 1 1] Remove left shutter
          (if (not (`self.Remove left shutter`))
            ;;[1 1 1] Ledt Shutter
            (`StaticMeshComponent.SetStaticMesh` _staticmesh6_2 "/Game/OldVillage/Meshes/Structure_Components/SM_Window_Shutter_001.SM_Window_Shutter_001")
            (`SceneComponent.K2_SetRelativeTransform` _staticmesh6_2 (`KismetMathLibrary.MakeTransform` (77.500229 18.251007 39.752438) (struct :`Yaw` -90.0)) false false))
          ;;[1 1 1] Remove right shutter
          (if (not (`self.Remove right shutter`))
            ;;[1 1 1] Right Shutter
            (`StaticMeshComponent.SetStaticMesh` _staticmesh7_2 "/Game/OldVillage/Meshes/Structure_Components/SM_Window_Shutter_001.SM_Window_Shutter_001")
            (`SceneComponent.K2_SetRelativeTransform` _staticmesh7_2 (`KismetMathLibrary.MakeTransform` (240.756271 18.250992 39.752438) (struct :`Yaw` -90.0) (1.0 -1.0 1.0)) false false))
          ;;[1 1 1] Shutters movement
          (`SceneComponent.K2_SetRelativeRotation` _staticmesh6_2 (`KismetMathLibrary.RLerp` (`KismetMathLibrary.MakeRotator` 0.0 0.0 -90.0) (`KismetMathLibrary.MakeRotator` 0.0 0.0 100.0) (`KismetMathLibrary.FClamp` (`self.Left shutter - 1 = Open 0 = Closed`))) false false)
          (`SceneComponent.K2_SetRelativeRotation` _staticmesh7_2 (`KismetMathLibrary.RLerp` (`KismetMathLibrary.MakeRotator` 0.0 0.0 -90.0) (`KismetMathLibrary.MakeRotator` 0.0 0.0 -280.0) (`KismetMathLibrary.FClamp` (`self.Right shutter - 1 = Open 0 = Closed`))) false false)))
      (switch `int` (`self.Choose window encase`)
        (:`1`
          ;[1 1 1] Encase
          (`StaticMeshComponent.SetStaticMesh` _staticmesh8_5 "/Game/OldVillage/Meshes/Structure/Decore/SM_Decorative_Stone_006.SM_Decorative_Stone_006")
          (`SceneComponent.K2_SetRelativeTransform` _staticmesh8_5 (`KismetMathLibrary.MakeTransform` (67.250305 -0.212769 50.401291) (struct :`Pitch` 1.937677 :`Yaw` -175.00473 :`Roll` 90.434914) (1.0 1.0 0.840121)) false false)
          (`StaticMeshComponent.SetStaticMesh` _staticmesh9_5 "/Game/OldVillage/Meshes/Structure/Decore/SM_Decorative_Stone_006.SM_Decorative_Stone_006")
          (`SceneComponent.K2_SetRelativeTransform` _staticmesh9_5 (`KismetMathLibrary.MakeTransform` (67.250275 2.569916 120.837669) (struct :`Pitch` -3.043361 :`Yaw` -0.000374 :`Roll` 89.999664)) false false)
          (`StaticMeshComponent.SetStaticMesh` _staticmesh11_5 "/Game/OldVillage/Meshes/Structure/Decore/SM_Decorative_Stone_005.SM_Decorative_Stone_005")
          (`SceneComponent.K2_SetRelativeTransform` _staticmesh11_5 (`KismetMathLibrary.MakeTransform` (110.70726 3.100082 178.875275) (struct :`Pitch` 90.0 :`Yaw` -26.565048 :`Roll` 63.434944) (1.0 1.0 0.934624)) false false)
          (`StaticMeshComponent.SetStaticMesh` _staticmesh12_3 "/Game/OldVillage/Meshes/Structure/Decore/SM_Decorative_Stone_004.SM_Decorative_Stone_004")
          (`SceneComponent.K2_SetRelativeTransform` _staticmesh12_3 (`KismetMathLibrary.MakeTransform` (212.22139 0.389267 177.318344) (struct :`Pitch` 90.0 :`Yaw` -26.565048 :`Roll` 63.434944) (1.0 0.918933 0.829561)) false false)
          (`StaticMeshComponent.SetStaticMesh` _staticmesh13_3 "/Game/OldVillage/Meshes/Structure/Decore/SM_Decorative_Stone_005.SM_Decorative_Stone_005")
          (`SceneComponent.K2_SetRelativeTransform` _staticmesh13_3 (`KismetMathLibrary.MakeTransform` (246.738022 -0.214615 109.966354) (struct :`Pitch` 0.000328 :`Yaw` -179.999878 :`Roll` 90.000404) (1.0 1.0 0.682101)) false false)
          (`StaticMeshComponent.SetStaticMesh` _staticmesh10_3 "/Game/OldVillage/Meshes/Structure/Decore/SM_Decorative_Stone_011.SM_Decorative_Stone_011")
          (`SceneComponent.K2_SetRelativeTransform` _staticmesh10_3 (`KismetMathLibrary.MakeTransform` (246.738022 -0.214615 47.92252) (struct :`Pitch` 0.000328 :`Yaw` -179.999878 :`Roll` 90.000404) (0.930527 1.000322 0.682422)) false false))
        (:`2`
          ;[1 1 1] Encase
          (`StaticMeshComponent.SetStaticMesh` _staticmesh8_3 "/Game/OldVillage/Meshes/Structure/Decore/SM_Decorative_Stone_011.SM_Decorative_Stone_011")
          (`SceneComponent.K2_SetRelativeTransform` _staticmesh8_3 (`KismetMathLibrary.MakeTransform` (71.743935 -0.174719 47.923546) (struct :`Pitch` -90.0 :`Yaw` -14.036254 :`Roll` -75.963432) (0.820643 1.000322 0.682422)) false false)
          (`StaticMeshComponent.SetStaticMesh` _staticmesh9_3 "/Game/OldVillage/Meshes/Structure/Decore/SM_Decorative_Stone_005.SM_Decorative_Stone_005")
          (`SceneComponent.K2_SetRelativeTransform` _staticmesh9_3 (`KismetMathLibrary.MakeTransform` (66.738037 -0.21498 109.967461) (struct :`Pitch` 1.4e-05 :`Roll` -89.999702) (1.0 1.0 0.682101)) false false)
          (`StaticMeshComponent.SetStaticMesh` _staticmesh11_3 "/Game/OldVillage/Meshes/Structure/Decore/SM_Decorative_Stone_005.SM_Decorative_Stone_005")
          (`SceneComponent.K2_SetRelativeTransform` _staticmesh11_3 (`KismetMathLibrary.MakeTransform` (110.70726 3.100082 178.875275) (struct :`Pitch` 90.0 :`Yaw` -26.565048 :`Roll` 63.434944) (1.0 1.0 -0.934624)) false false)
          (`StaticMeshComponent.SetStaticMesh` _staticmesh12_2 "/Game/OldVillage/Meshes/Structure/Decore/SM_Decorative_Stone_004.SM_Decorative_Stone_004")
          (`SceneComponent.K2_SetRelativeTransform` _staticmesh12_2 (`KismetMathLibrary.MakeTransform` (209.261902 1.269508 176.191116) (struct :`Pitch` 90.0 :`Yaw` -26.565062 :`Roll` -116.56501) (1.0 0.918933 0.829561)) false false)
          (`StaticMeshComponent.SetStaticMesh` _staticmesh13_2 "/Game/OldVillage/Meshes/Structure/Decore/SM_Decorative_Stone_006.SM_Decorative_Stone_006")
          (`SceneComponent.K2_SetRelativeTransform` _staticmesh13_2 (`KismetMathLibrary.MakeTransform` (247.250275 1.174819 120.837555) (struct :`Pitch` -3.043365 :`Yaw` 179.99971 :`Roll` 89.999603)) false false)
          (`StaticMeshComponent.SetStaticMesh` _staticmesh10_2 "/Game/OldVillage/Meshes/Structure/Decore/SM_Decorative_Stone_006.SM_Decorative_Stone_006")
          (`SceneComponent.K2_SetRelativeTransform` _staticmesh10_2 (`KismetMathLibrary.MakeTransform` (247.114868 1.339957 55.88102) (struct :`Pitch` 1.937677 :`Yaw` -175.00473 :`Roll` 90.434914) (1.0 0.630366 0.840121)) false false))
        (:`3`
          ;[1 1 1] Encase
          (`StaticMeshComponent.SetStaticMesh` _staticmesh8 "/Game/OldVillage/Meshes/Structure/Decore/SM_Decorative_Stone_006.SM_Decorative_Stone_006")
          (`SceneComponent.K2_SetRelativeTransform` _staticmesh8 (`KismetMathLibrary.MakeTransform` (67.593735 -0.258948 60.395287) (struct :`Pitch` 1.937677 :`Yaw` -175.00473 :`Roll` 90.434914) (1.0 0.65906 0.840121)) false false)
          (`StaticMeshComponent.SetStaticMesh` _staticmesh9 "/Game/OldVillage/Meshes/Structure/Decore/SM_Decorative_Stone_006.SM_Decorative_Stone_006")
          (`SceneComponent.K2_SetRelativeTransform` _staticmesh9 (`KismetMathLibrary.MakeTransform` (67.250275 2.569916 124.0) (struct :`Pitch` -3.043361 :`Yaw` -0.000374 :`Roll` 89.999664) (1.0 -1.0 1.0)) false false)
          (`StaticMeshComponent.SetStaticMesh` _staticmesh11 "/Game/OldVillage/Meshes/Structure/Decore/SM_Decorative_Stone_005.SM_Decorative_Stone_005")
          (`SceneComponent.K2_SetRelativeTransform` _staticmesh11 (`KismetMathLibrary.MakeTransform` (110.707253 0.693681 177.949966) (struct :`Pitch` -90.0 :`Yaw` 90.0 :`Roll` 179.999969) (1.0 1.0 0.934624)) false false)
          (`StaticMeshComponent.SetStaticMesh` _staticmesh12 "/Game/OldVillage/Meshes/Structure/Decore/SM_Decorative_Stone_004.SM_Decorative_Stone_004")
          (`SceneComponent.K2_SetRelativeTransform` _staticmesh12 (`KismetMathLibrary.MakeTransform` (212.22139 0.389267 177.318344) (struct :`Pitch` 90.0 :`Yaw` -26.565048 :`Roll` 63.434944) (1.0 0.918933 -0.829561)) false false)
          (`StaticMeshComponent.SetStaticMesh` _staticmesh13 "/Game/OldVillage/Meshes/Structure/Decore/SM_Decorative_Stone_005.SM_Decorative_Stone_005")
          (`SceneComponent.K2_SetRelativeTransform` _staticmesh13 (`KismetMathLibrary.MakeTransform` (246.738022 -0.214615 109.966354) (struct :`Pitch` 0.000328 :`Yaw` -179.999878 :`Roll` 90.000404) (1.0 1.0 -0.682101)) false false)
          (`StaticMeshComponent.SetStaticMesh` _staticmesh10 "/Game/OldVillage/Meshes/Structure/Decore/SM_Decorative_Stone_011.SM_Decorative_Stone_011")
          (`SceneComponent.K2_SetRelativeTransform` _staticmesh10 (`KismetMathLibrary.MakeTransform` (246.738022 -0.214615 47.92252) (struct :`Pitch` 0.000328 :`Yaw` -179.999878 :`Roll` 90.000404) (0.930527 1.000322 0.682422)) false false))
        (:`4`
          ;[1 1 1] Wood encase
          (if (`self.Abbandoned building`)
            (`StaticMeshComponent.SetStaticMesh` _staticmesh8_4 "/Game/OldVillage/Meshes/Structure_Components/SM_Pole_001_abbandoned.SM_Pole_001_abbandoned")
            (`SceneComponent.K2_SetRelativeTransform` _staticmesh8_4 (`KismetMathLibrary.MakeTransform` (84.800705 4.805449 35.271015) (struct) (1.0 0.368944 1.261044)) false false)
            (`StaticMeshComponent.SetStaticMesh` _staticmesh9_4 "/Game/OldVillage/Meshes/Structure_Components/SM_Pole_001_abbandoned.SM_Pole_001_abbandoned")
            (`SceneComponent.K2_SetRelativeTransform` _staticmesh9_4 (`KismetMathLibrary.MakeTransform` (61.179119 7.946863 159.586777) (struct :`Pitch` -90.0 :`Yaw` 160.528839 :`Roll` -160.528763) (0.999889 0.500223 1.892907)) false false)
            (`StaticMeshComponent.SetStaticMesh` _staticmesh11_4 "/Game/OldVillage/Meshes/Structure_Components/SM_Pole_001_abbandoned.SM_Pole_001_abbandoned")
            (`SceneComponent.K2_SetRelativeTransform` _staticmesh11_4 (`KismetMathLibrary.MakeTransform` (228.596298 5.778234 159.586777) (struct :`Pitch` -4.1e-05 :`Yaw` -179.999969 :`Roll` -179.999969) (1.0 0.368944 1.261044)) false false)
            (else
              (`StaticMeshComponent.SetStaticMesh` _staticmesh8_2 "/Game/OldVillage/Meshes/Structure_Components/SM_Pole_001.SM_Pole_001")
              (`SceneComponent.K2_SetRelativeTransform` _staticmesh8_2 (`KismetMathLibrary.MakeTransform` (84.800705 4.805449 35.271015) (struct) (1.0 0.368944 1.261044)) false false)
              (`StaticMeshComponent.SetStaticMesh` _staticmesh9_2 "/Game/OldVillage/Meshes/Structure_Components/SM_Pole_001.SM_Pole_001")
              (`SceneComponent.K2_SetRelativeTransform` _staticmesh9_2 (`KismetMathLibrary.MakeTransform` (61.179119 7.946863 159.586777) (struct :`Pitch` -90.0 :`Yaw` 160.528839 :`Roll` -160.528763) (0.999889 0.500223 1.892907)) false false)
              (`StaticMeshComponent.SetStaticMesh` _staticmesh11_2 "/Game/OldVillage/Meshes/Structure_Components/SM_Pole_001.SM_Pole_001")
              (`SceneComponent.K2_SetRelativeTransform` _staticmesh11_2 (`KismetMathLibrary.MakeTransform` (228.596298 5.778234 159.586777) (struct :`Pitch` -4.1e-05 :`Yaw` -179.999969 :`Roll` -179.999969) (1.0 0.368944 1.261044)) false false))))))
    (:`NewEnumerator2`
      ;[1 1 1] Right corner 90
      (if (`self.Abbandoned building`)
        (`StaticMeshComponent.SetStaticMesh` _staticmesh_2 "/Game/OldVillage/Meshes/Structure_Components/SM_Wall_3mx2m_Edge_L_001_abbandoned.SM_Wall_3mx2m_Edge_L_001_abbandoned")
        (`SceneComponent.K2_SetRelativeTransform` _staticmesh_2 (`KismetMathLibrary.MakeTransform` (0.0 0.0 0.0) (struct)) false false)
        (else
          (`StaticMeshComponent.SetStaticMesh` _staticmesh "/Game/OldVillage/Meshes/Structure_Components/SM_Wall_3mx2m_Edge_L_001.SM_Wall_3mx2m_Edge_L_001")
          (`SceneComponent.K2_SetRelativeTransform` _staticmesh (`KismetMathLibrary.MakeTransform` (0.0 0.0 0.0) (struct)) false false))))
    (:`NewEnumerator3`
      ;[1 1 1] Left Corner 90
      (if (`self.Abbandoned building`)
        (`StaticMeshComponent.SetStaticMesh` _staticmesh_5 "/Game/OldVillage/Meshes/Structure_Components/SM_Wall_3mx2m_Edge_R_001_abbandoned.SM_Wall_3mx2m_Edge_R_001_abbandoned")
        (`SceneComponent.K2_SetRelativeTransform` _staticmesh_5 (`KismetMathLibrary.MakeTransform` (300.0 0.0 0.0) (struct)) false false)
        (else
          (`StaticMeshComponent.SetStaticMesh` _staticmesh_3 "/Game/OldVillage/Meshes/Structure_Components/SM_Wall_3mx2m_Edge_R_001.SM_Wall_3mx2m_Edge_R_001")
          (`SceneComponent.K2_SetRelativeTransform` _staticmesh_3 (`KismetMathLibrary.MakeTransform` (300.0 0.0 0.0) (struct)) false false))))))