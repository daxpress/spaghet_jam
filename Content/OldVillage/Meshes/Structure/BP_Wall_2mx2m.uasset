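; Configurable modular 2m x 2m village wall piece, built in the Construction Script as plain wall, window or inward corner, with abandoned mesh variants.
; Material overrides cover interior and exterior, with a dynamic material instance tinting the stucco.
; A component selector swaps meshes and transforms on reused StaticMesh components, adding glass, supports, shutters, encasing and flowers per window type.
; Clamped 0–1 sliders lerp shutter rotation between closed and open.
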(fn `UserConstructionScript`
  (bind _staticmesh11 (`self.StaticMesh11`))
  (bind _staticmesh12 (`self.StaticMesh12`))
  (bind _staticmesh13 (`self.StaticMesh13`))
  (bind _staticmesh10 (`self.StaticMesh10`))
  (bind _staticmesh8 (`self.StaticMesh8`))
  (bind _staticmesh9 (`self.StaticMesh9`))
  (bind _staticmesh (`self.StaticMesh`))
  (bind _staticmesh_2 (`self.StaticMesh`))
  (bind _staticmesh_3 (`self.StaticMesh`))
  (bind _staticmesh_4 (`self.StaticMesh`))
  (bind _staticmesh_5 (`self.StaticMesh`))
  (bind _exterior_material_override (`self.Exterior Material Override`))
  (bind _staticmesh_6 (`self.StaticMesh`))
  (bind _staticmesh1 (`self.StaticMesh1`))
  (bind _staticmesh_7 (`self.StaticMesh`))
  (bind _staticmesh1_2 (`self.StaticMesh1`))
  (bind _staticmesh2 (`self.StaticMesh2`))
  (bind _staticmesh3 (`self.StaticMesh3`))
  (bind _staticmesh4 (`self.StaticMesh4`))
  (bind _staticmesh5 (`self.StaticMesh5`))
  (bind _staticmesh6 (`self.StaticMesh6`))
  (bind _staticmesh7 (`self.StaticMesh7`))
  (bind _staticmesh_8 (`self.StaticMesh`))
  (bind _staticmesh_9 (`self.StaticMesh`))
  (bind _staticmesh1_3 (`self.StaticMesh1`))
  (bind _staticmesh4_2 (`self.StaticMesh4`))
  (bind _staticmesh5_2 (`self.StaticMesh5`))
  (bind _staticmesh6_2 (`self.StaticMesh6`))
  (bind _staticmesh7_2 (`self.StaticMesh7`))
  (bind _staticmesh_10 (`self.StaticMesh`))
  (bind _staticmesh1_4 (`self.StaticMesh1`))
  (bind _staticmesh4_3 (`self.StaticMesh4`))
  (bind _staticmesh6_3 (`self.StaticMesh6`))
  (bind _staticmesh14 (`self.StaticMesh14`))
  (bind _staticmesh10_2 (`self.StaticMesh10`))
  (bind _staticmesh2_2 (`self.StaticMesh2`))
  (bind _staticmesh_11 (`self.StaticMesh`))
  (bind _staticmesh_12 (`self.StaticMesh`))
  (bind _staticmesh_13 (`self.StaticMesh`))
  (bind _staticmesh_14 (`self.StaticMesh`))
  (bind _staticmesh8_2 (`self.StaticMesh8`))
  (bind _staticmesh9_2 (`self.StaticMesh9`))
  (bind _staticmesh14_2 (`self.StaticMesh14`))
  (bind _staticmesh14_3 (`self.StaticMesh14`))
  (bind _staticmesh11_2 (`self.StaticMesh11`))
  (bind _staticmesh2_3 (`self.StaticMesh2`))
  (bind _staticmesh2_4 (`self.StaticMesh2`))
  (bind _staticmesh14_4 (`self.StaticMesh14`))
  (bind _staticmesh8_3 (`self.StaticMesh8`))
  (bind _staticmesh9_3 (`self.StaticMesh9`))
  (bind _staticmesh11_3 (`self.StaticMesh11`))
  (bind _staticmesh3_2 (`self.StaticMesh3`))
  (bind _staticmesh2_5 (`self.StaticMesh2`))
  (bind _staticmesh4_4 (`self.StaticMesh4`))
  (bind _staticmesh8_4 (`self.StaticMesh8`))
  (bind _staticmesh9_4 (`self.StaticMesh9`))
  (bind _staticmesh11_4 (`self.StaticMesh11`))
  (bind _staticmesh12_2 (`self.StaticMesh12`))
  (bind _staticmesh13_2 (`self.StaticMesh13`))
  (bind _staticmesh10_3 (`self.StaticMesh10`))
  (bind _staticmesh8_5 (`self.StaticMesh8`))
  (bind _staticmesh9_5 (`self.StaticMesh9`))
  (bind _staticmesh11_5 (`self.StaticMesh11`))
  (bind _staticmesh12_3 (`self.StaticMesh12`))
  (bind _staticmesh13_3 (`self.StaticMesh13`))
  (bind _staticmesh6_4 (`self.StaticMesh6`))
  (`PrimitiveComponent.SetMaterial` _staticmesh_5 0 (`self.Interior Material Override`))
  (`PrimitiveComponent.SetMaterial` _staticmesh_5 1 _exterior_material_override)
  ;[1 1 1] Change stucco Color
  (bind _returnvalue (`PrimitiveComponent.CreateDynamicMaterialInstance` (`self.StaticMesh`) 1 _exterior_material_override "None"))
  (`MaterialInstanceDynamic.SetVectorParameterValue` _returnvalue "Material 2 Color multiplier" (`self.Stucco Color`))
  (switch `/Game/OldVillage/Meshes/Structure/Enumerators/BP_2mx2m_enum` (`self.Choose component`)
    (:`NewEnumerator0`
      (if (`self.Abbandoned building`)
        ;[1 1 1] Basic Wall
        (`StaticMeshComponent.SetStaticMesh` _staticmesh_11 "/Game/OldVillage/Meshes/Structure_Components/SM_Wall_2mx2m_001_Abbandoned.SM_Wall_2mx2m_001_Abbandoned")
        (`SceneComponent.K2_SetRelativeTransform` _staticmesh_11 (`KismetMathLibrary.MakeTransform` (0.0 0.0 0.0) (struct)) false false)))
    (:`NewEnumerator1`
      (if (`self.Abbandoned building`)
        ;[1 1 1] Window 01 - Abbandoned
        ;;[1 1 1] Base
        (`StaticMeshComponent.SetStaticMesh` _staticmesh_7 "/Game/OldVillage/Meshes/Structure_Components/SM_Wall_2mx2m_window_002_component_abbandoned.SM_Wall_2mx2m_window_002_component_abbandoned")
        (`SceneComponent.K2_SetRelativeTransform` _staticmesh_7 (`KismetMathLibrary.MakeTransform` (0.0 0.0 0.0) (struct)) false false)
        ;;[1 1 1] Window body
        (`StaticMeshComponent.SetStaticMesh` _staticmesh1_2 "/Game/OldVillage/Meshes/Structure_Components/SM_Window_002_abbandoned_frame.SM_Window_002_abbandoned_frame")
        (`SceneComponent.K2_SetRelativeTransform` _staticmesh1_2 (`KismetMathLibrary.MakeTransform` (145.43895 -11.161145 39.555855) (struct :`Yaw` -90.0) (1.0 1.0 1.0)) false false)
        (switch `int` (`self.Choose abbandoned window glass`)
          (:`0`
            ;;[1 1 1] Glass
            (`StaticMeshComponent.SetStaticMesh` _staticmesh2_3 "/Game/OldVillage/Meshes/Structure_Components/SM_Window_002_abbandoned_glass_001.SM_Window_002_abbandoned_glass_001" :!label _label)
            (`SceneComponent.K2_SetRelativeTransform` _staticmesh2_3 (`KismetMathLibrary.MakeTransform` (145.43895 -11.161145 39.555855) (struct :`Yaw` -90.000008) (1.0 1.0 1.0)) false false))
          (:`1`
            (goto _label))
          (:`2`
            ;;[1 1 1] Glass 2
            (`StaticMeshComponent.SetStaticMesh` _staticmesh2_4 "/Game/OldVillage/Meshes/Structure_Components/SM_Window_002_abbandoned_glass_002.SM_Window_002_abbandoned_glass_002")
            (`SceneComponent.K2_SetRelativeTransform` _staticmesh2_4 (`KismetMathLibrary.MakeTransform` (145.43895 -11.161145 39.555855) (struct :`Yaw` -90.000008) (1.0 1.0 1.0)) false false))
          (:`3`
            ;;[1 1 1] Glass 2
            (`StaticMeshComponent.SetStaticMesh` _staticmesh2_2 "/Game/OldVillage/Meshes/Structure_Components/SM_Window_002_abbandoned_glass_003.SM_Window_002_abbandoned_glass_003")
            (`SceneComponent.K2_SetRelativeTransform` _staticmesh2_2 (`KismetMathLibrary.MakeTransform` (145.43895 -11.161145 39.555855) (struct :`Yaw` -90.000008) (1.0 1.0 1.0)) false false)))
        (switch `int` (`self.Choose abbandoned window support`)
          (:`1`
            ;;[1 1 1] Window support
            (`StaticMeshComponent.SetStaticMesh` _staticmesh3_2 "/Game/OldVillage/Meshes/Structure_Components/SM_Window_002_abbandoned_support_001.SM_Window_002_abbandoned_support_001")
            (`SceneComponent.K2_SetRelativeTransform` _staticmesh3_2 (`KismetMathLibrary.MakeTransform` (145.43895 -11.161145 39.555855) (struct :`Yaw` -90.000008) (1.0 1.0 1.0)) false false))
          (:`2`
            ;;[1 1 1] Window support
            (`StaticMeshComponent.SetStaticMesh` _staticmesh3 "/Game/OldVillage/Meshes/Structure_Components/SM_Window_002_abbandoned_support_002.SM_Window_002_abbandoned_support_002")
            (`SceneComponent.K2_SetRelativeTransform` _staticmesh3 (`KismetMathLibrary.MakeTransform` (145.43895 -11.161145 39.555855) (struct :`Yaw` -90.000008) (1.0 1.0 1.0)) false false)))
        ;;[1 1 1] Shutters support
        (`StaticMeshComponent.SetStaticMesh` _staticmesh4 "/Game/OldVillage/Meshes/Structure_Components/SM_Window_Shutter_002_abbandoned_support.SM_Window_Shutter_002_abbandoned_support")
        (`SceneComponent.K2_SetRelativeTransform` _staticmesh4 (`KismetMathLibrary.MakeTransform` (40.695007 11.019038 38.224361) (struct :`Yaw` -90.000008)) false false)
        (`StaticMeshComponent.SetStaticMesh` _staticmesh5 "/Game/OldVillage/Meshes/Structure_Components/SM_Window_Shutter_002_abbandoned_support.SM_Window_Shutter_002_abbandoned_support")
        (`SceneComponent.K2_SetRelativeTransform` _staticmesh5 (`KismetMathLibrary.MakeTransform` (162.126221 11.019085 38.224361) (struct :`Yaw` -90.000008) (1.0 -1.0 1.0)) false false)
        ;;[1 1 1] Remove left shutter
        (if (not (`self.Remove left shutter`))
          ;;[1 1 1] Ledt Shutter
          (`StaticMeshComponent.SetStaticMesh` _staticmesh6 "/Game/OldVillage/Meshes/Structure_Components/SM_Window_Shutter_002_abbandoned.SM_Window_Shutter_002_abbandoned")
          (`SceneComponent.K2_SetRelativeTransform` _staticmesh6 (`KismetMathLibrary.MakeTransform` (40.695007 11.019085 38.224361) (struct :`Yaw` -90.0)) false false))
        ;;[1 1 1] Remove right shutter
        (if (not (`self.Remove right shutter`))
          ;;[1 1 1] Right Shutter
          (`StaticMeshComponent.SetStaticMesh` _staticmesh7 "/Game/OldVillage/Meshes/Structure_Components/SM_Window_Shutter_002_abbandoned.SM_Window_Shutter_002_abbandoned")
          (`SceneComponent.K2_SetRelativeTransform` _staticmesh7 (`KismetMathLibrary.MakeTransform` (162.126221 11.019038 38.224361) (struct :`Yaw` -90.0) (1.0 -1.0 1.0)) false false))
        ;;[1 1 1] Shutters movement
        (`SceneComponent.K2_SetRelativeRotation` _staticmesh6 (`KismetMathLibrary.RLerp` (`KismetMathLibrary.MakeRotator` 0.0 0.0 -90.0) (`KismetMathLibrary.MakeRotator` 0.0 0.0 100.0) (`KismetMathLibrary.FClamp` (`self.Left shutter - 1 = Open 0 = Closed`))) false false)
        (`SceneComponent.K2_SetRelativeRotation` _staticmesh7 (`KismetMathLibrary.RLerp` (`KismetMathLibrary.MakeRotator` 0.0 0.0 -90.0) (`KismetMathLibrary.MakeRotator` 0.0 0.0 -280.0) (`KismetMathLibrary.FClamp` (`self.Right shutter - 1 = Open 0 = Closed`))) false false)
        (else
          ;[1 1 1] Window 01
          ;;[1 1 1] Base
          (`StaticMeshComponent.SetStaticMesh` _staticmesh_9 "/Game/OldVillage/Meshes/Structure_Components/SM_Wall_2mx2m_window_002_component.SM_Wall_2mx2m_window_002_component")
          (`SceneComponent.K2_SetRelativeTransform` _staticmesh_9 (`KismetMathLibrary.MakeTransform` (0.0 0.0 0.0) (struct)) false false)
          ;;[1 1 1] Window body
          (`StaticMeshComponent.SetStaticMesh` _staticmesh1_3 "/Game/OldVillage/Meshes/Structure_Components/SM_Window_002.SM_Window_002")
          (`SceneComponent.K2_SetRelativeTransform` _staticmesh1_3 (`KismetMathLibrary.MakeTransform` (145.43895 -11.161145 39.555855) (struct :`Yaw` -90.0) (1.0 1.0 1.0)) false false)
          ;;[1 1 1] Shutters support
          (`StaticMeshComponent.SetStaticMesh` _staticmesh4_2 "/Game/OldVillage/Meshes/Structure_Components/SM_Window_Shutter_002_support.SM_Window_Shutter_002_support")
          (`SceneComponent.K2_SetRelativeTransform` _staticmesh4_2 (`KismetMathLibrary.MakeTransform` (40.695007 11.019038 38.224361) (struct :`Yaw` -90.000008)) false false)
          (`StaticMeshComponent.SetStaticMesh` _staticmesh5_2 "/Game/OldVillage/Meshes/Structure_Components/SM_Window_Shutter_002_support.SM_Window_Shutter_002_support")
          (`SceneComponent.K2_SetRelativeTransform` _staticmesh5_2 (`KismetMathLibrary.MakeTransform` (162.126221 11.019085 38.224361) (struct :`Yaw` -90.000008) (1.0 -1.0 1.0)) false false)
          ;;[1 1 1] Remove left shutter
          (if (not (`self.Remove left shutter`))
            ;;[1 1 1] Ledt Shutter
            (`StaticMeshComponent.SetStaticMesh` _staticmesh6_2 "/Game/OldVillage/Meshes/Structure_Components/SM_Window_Shutter_002.SM_Window_Shutter_002")
            (`SceneComponent.K2_SetRelativeTransform` _staticmesh6_2 (`KismetMathLibrary.MakeTransform` (40.695007 11.019085 38.224361) (struct :`Yaw` -90.0)) false false))
          ;;[1 1 1] Remove right shutter
          (if (not (`self.Remove right shutter`))
            ;;[1 1 1] Right Shutter
            (`StaticMeshComponent.SetStaticMesh` _staticmesh7_2 "/Game/OldVillage/Meshes/Structure_Components/SM_Window_Shutter_002.SM_Window_Shutter_002")
            (`SceneComponent.K2_SetRelativeTransform` _staticmesh7_2 (`KismetMathLibrary.MakeTransform` (162.126221 11.019038 38.224361) (struct :`Yaw` -90.0) (1.0 -1.0 1.0)) false false))
          ;;[1 1 1] Shutters movement
          (`SceneComponent.K2_SetRelativeRotation` _staticmesh6_2 (`KismetMathLibrary.RLerp` (`KismetMathLibrary.MakeRotator` 0.0 0.0 -90.0) (`KismetMathLibrary.MakeRotator` 0.0 0.0 100.0) (`KismetMathLibrary.FClamp` (`self.Left shutter - 1 = Open 0 = Closed`))) false false)
          (`SceneComponent.K2_SetRelativeRotation` _staticmesh7_2 (`KismetMathLibrary.RLerp` (`KismetMathLibrary.MakeRotator` 0.0 0.0 -90.0) (`KismetMathLibrary.MakeRotator` 0.0 0.0 -280.0) (`KismetMathLibrary.FClamp` (`self.Right shutter - 1 = Open 0 = Closed`))) false false)))
      (switch `int` (`self.Choose window encase`)
        (:`1`
          ;[1 1 1] Encase
          (`StaticMeshComponent.SetStaticMesh` _staticmesh8_4 "/Game/OldVillage/Meshes/Structure/Decore/SM_Decorative_Stone_005.SM_Decorative_Stone_005")
          (`SceneComponent.K2_SetRelativeTransform` _staticmesh8_4 (`KismetMathLibrary.MakeTransform` (78.13604 -0.453182 179.645645) (struct :`Pitch` 90.0 :`Yaw` 45.0 :`Roll` 135.000534) (1.0 1.090106 0.693679)) false false)
          (`StaticMeshComponent.SetStaticMesh` _staticmesh9_4 "/Game/OldVillage/Meshes/Structure/Decore/SM_Decorative_Stone_013.SM_Decorative_Stone_013")
          (`SceneComponent.K2_SetRelativeTransform` _staticmesh9_4 (`KismetMathLibrary.MakeTransform` (142.281433 -0.940052 177.663177) (struct :`Pitch` 90.0 :`Yaw` -54.735611 :`Roll` 125.264351) (1.0 1.181178 1.54989)) false false)
          (`StaticMeshComponent.SetStaticMesh` _staticmesh11_4 "/Game/OldVillage/Meshes/Structure/Decore/SM_Decorative_Stone_006.SM_Decorative_Stone_006")
          (`SceneComponent.K2_SetRelativeTransform` _staticmesh11_4 (`KismetMathLibrary.MakeTransform` (169.832703 -1.145115 153.05632) (struct :`Yaw` -179.999969 :`Roll` -89.999931)) false false)
          (`StaticMeshComponent.SetStaticMesh` _staticmesh12_2 "/Game/OldVillage/Meshes/Structure/Decore/SM_Decorative_Stone_005.SM_Decorative_Stone_005")
          (`SceneComponent.K2_SetRelativeTransform` _staticmesh12_2 (`KismetMathLibrary.MakeTransform` (169.977493 -2.960155 72.790268) (struct :`Pitch` -0.000403 :`Yaw` -179.999649 :`Roll` 90.000008) (1.0 0.829976 0.646382)) false false)
          (`StaticMeshComponent.SetStaticMesh` _staticmesh13_2 "/Game/OldVillage/Meshes/Structure/Decore/SM_Decorative_Stone_006.SM_Decorative_Stone_006")
          (`SceneComponent.K2_SetRelativeTransform` _staticmesh13_2 (`KismetMathLibrary.MakeTransform` (30.341614 -2.496433 122.032784) (struct :`Yaw` -179.999969 :`Roll` 90.000137) (1.0 1.0 0.624664)) false false)
          (`StaticMeshComponent.SetStaticMesh` _staticmesh10_3 "/Game/OldVillage/Meshes/Structure/Decore/SM_Decorative_Stone_006.SM_Decorative_Stone_006")
          (`SceneComponent.K2_SetRelativeTransform` _staticmesh10_3 (`KismetMathLibrary.MakeTransform` (29.848206 -0.627018 45.756844) (struct :`Pitch` 0.000806 :`Yaw` -0.000214 :`Roll` 90.000267)) false false))
        (:`2`
          ;[1 1 1] Encase
          (`StaticMeshComponent.SetStaticMesh` _staticmesh8_5 "/Game/OldVillage/Meshes/Structure/Decore/SM_Decorative_Stone_007.SM_Decorative_Stone_007")
          (`SceneComponent.K2_SetRelativeTransform` _staticmesh8_5 (`KismetMathLibrary.MakeTransform` (30.395502 0.0 50.912361) (struct :`Roll` 89.999977) (0.869979 0.71003 1.0)) false false)
          (`StaticMeshComponent.SetStaticMesh` _staticmesh9_5 "/Game/OldVillage/Meshes/Structure/Decore/SM_Decorative_Stone_004.SM_Decorative_Stone_004")
          (`SceneComponent.K2_SetRelativeTransform` _staticmesh9_5 (`KismetMathLibrary.MakeTransform` (30.0 -1.624767 125.33577) (struct :`Roll` 89.999977) (1.0 1.12012 1.0)) false false)
          (`StaticMeshComponent.SetStaticMesh` _staticmesh11_5 "/Game/OldVillage/Meshes/Structure/Decore/SM_Decorative_Stone_005.SM_Decorative_Stone_005")
          (`SceneComponent.K2_SetRelativeTransform` _staticmesh11_5 (`KismetMathLibrary.MakeTransform` (110.979576 0.382065 178.041794) (struct :`Pitch` 90.0 :`Roll` 89.999947) (0.79 1.270351 1.0)) false false)
          (`StaticMeshComponent.SetStaticMesh` _staticmesh12_3 "/Game/OldVillage/Meshes/Structure/Decore/SM_Decorative_Stone_012.SM_Decorative_Stone_012")
          (`SceneComponent.K2_SetRelativeTransform` _staticmesh12_3 (`KismetMathLibrary.MakeTransform` (162.507996 -0.924071 153.001389) (struct :`Pitch` -90.0 :`Yaw` 9.462321 :`Roll` 80.537605) (1.0 1.0 0.589819)) false false)
          (`StaticMeshComponent.SetStaticMesh` _staticmesh13_3 "/Game/OldVillage/Meshes/Structure/Decore/SM_Decorative_Stone_012.SM_Decorative_Stone_012")
          (`SceneComponent.K2_SetRelativeTransform` _staticmesh13_3 (`KismetMathLibrary.MakeTransform` (168.618103 -3.850382 127.843262) (struct :`Roll` 89.999977) (0.869917 1.050134 1.0)) false false)
          (`StaticMeshComponent.SetStaticMesh` _staticmesh10_2 "/Game/OldVillage/Meshes/Structure/Decore/SM_Decorative_Stone_006.SM_Decorative_Stone_006")
          (`SceneComponent.K2_SetRelativeTransform` _staticmesh10_2 (`KismetMathLibrary.MakeTransform` (167.674759 -1.302166 79.171425) (struct :`Roll` 89.999977) (0.820066 1.0 1.0)) false false))
        (:`3`
          ;[1 1 1] Encase
          (`StaticMeshComponent.SetStaticMesh` _staticmesh8_2 "/Game/OldVillage/Meshes/Structure/Decore/SM_Decorative_Stone_011.SM_Decorative_Stone_011")
          (`SceneComponent.K2_SetRelativeTransform` _staticmesh8_2 (`KismetMathLibrary.MakeTransform` (34.996277 -2.035042 47.377724) (struct :`Pitch` -90.0 :`Yaw` -26.565048 :`Roll` 116.565063) (1.0 1.0 0.778741)) false false)
          (`StaticMeshComponent.SetStaticMesh` _staticmesh9_2 "/Game/OldVillage/Meshes/Structure/Decore/SM_Decorative_Stone_005.SM_Decorative_Stone_005")
          (`SceneComponent.K2_SetRelativeTransform` _staticmesh9_2 (`KismetMathLibrary.MakeTransform` (32.054451 -3.493461 116.398758) (struct :`Pitch` 0.188971 :`Yaw` -171.851685 :`Roll` 90.004166) (0.848325 -1.002721 0.778741)) false false)
          (`StaticMeshComponent.SetStaticMesh` _staticmesh11_2 "/Game/OldVillage/Meshes/Structure/Decore/SM_Decorative_Stone_005.SM_Decorative_Stone_005")
          (`SceneComponent.K2_SetRelativeTransform` _staticmesh11_2 (`KismetMathLibrary.MakeTransform` (61.42907 -2.034996 179.940918) (struct :`Pitch` -90.0 :`Yaw` 143.130096 :`Roll` -53.130096) (1.0 1.0 0.778741)) false false)
          (`StaticMeshComponent.SetStaticMesh` _staticmesh12 "/Game/OldVillage/Meshes/Structure/Decore/SM_Decorative_Stone_006.SM_Decorative_Stone_006")
          (`SceneComponent.K2_SetRelativeTransform` _staticmesh12 (`KismetMathLibrary.MakeTransform` (147.858582 -2.035011 179.940918) (struct :`Pitch` -85.742264 :`Yaw` 179.999512 :`Roll` -89.984077) (1.0 1.0 0.778741)) false false)
          (`StaticMeshComponent.SetStaticMesh` _staticmesh13 "/Game/OldVillage/Meshes/Structure/Decore/SM_Decorative_Stone_005.SM_Decorative_Stone_005")
          (`SceneComponent.K2_SetRelativeTransform` _staticmesh13 (`KismetMathLibrary.MakeTransform` (168.853027 -2.526054 110.170921) (struct :`Pitch` 0.473913 :`Yaw` 0.000118 :`Roll` -89.996155) (0.91905 1.0 0.778741)) false false)
          (`StaticMeshComponent.SetStaticMesh` _staticmesh10 "/Game/OldVillage/Meshes/Structure/Decore/SM_Decorative_Stone_012.SM_Decorative_Stone_012")
          (`SceneComponent.K2_SetRelativeTransform` _staticmesh10 (`KismetMathLibrary.MakeTransform` (164.355484 -2.526077 41.538967) (struct :`Pitch` -89.394432 :`Yaw` 179.984482 :`Roll` 90.011627) (0.91905 1.0 0.778741)) false false))
        (:`4`
          (if (`self.Abbandoned building`)
            (`StaticMeshComponent.SetStaticMesh` _staticmesh8 "/Game/OldVillage/Meshes/Structure_Components/SM_Pole_001_abbandoned.SM_Pole_001_abbandoned")
            (`SceneComponent.K2_SetRelativeTransform` _staticmesh8 (`KismetMathLibrary.MakeTransform` (28.321716 3.647732 164.608566) (struct :`Pitch` -4.1e-05 :`Yaw` -179.999969 :`Roll` -179.999969) (0.835832 0.473918 1.283909)) false false)
            (`StaticMeshComponent.SetStaticMesh` _staticmesh9 "/Game/OldVillage/Meshes/Structure_Components/SM_Pole_002_abbandoned.SM_Pole_002_abbandoned")
            (`SceneComponent.K2_SetRelativeTransform` _staticmesh9 (`KismetMathLibrary.MakeTransform` (171.982162 6.044788 164.608566) (struct :`Pitch` 88.818481 :`Yaw` 8.325159 :`Roll` 8.326858) (0.835832 0.504072 1.434415)) false false)
            (`StaticMeshComponent.SetStaticMesh` _staticmesh11 "/Game/OldVillage/Meshes/Structure_Components/SM_Pole_001_abbandoned.SM_Pole_001_abbandoned")
            (`SceneComponent.K2_SetRelativeTransform` _staticmesh11 (`KismetMathLibrary.MakeTransform` (174.094849 3.647747 35.692516) (struct) (0.835832 0.473918 1.324234)) false false)
            (else
              (`StaticMeshComponent.SetStaticMesh` _staticmesh8_3 "/Game/OldVillage/Meshes/Structure_Components/SM_Pole_001.SM_Pole_001")
              (`SceneComponent.K2_SetRelativeTransform` _staticmesh8_3 (`KismetMathLibrary.MakeTransform` (28.321716 3.647732 164.608566) (struct :`Pitch` -4.1e-05 :`Yaw` -179.999969 :`Roll` -179.999969) (0.835832 0.473918 1.283909)) false false)
              (`StaticMeshComponent.SetStaticMesh` _staticmesh9_3 "/Game/OldVillage/Meshes/Structure_Components/SM_Pole_002.SM_Pole_002")
              (`SceneComponent.K2_SetRelativeTransform` _staticmesh9_3 (`KismetMathLibrary.MakeTransform` (171.982162 6.044788 164.608566) (struct :`Pitch` 88.818481 :`Yaw` 8.325159 :`Roll` 8.326858) (0.835832 0.504072 1.434415)) false false)
              (`StaticMeshComponent.SetStaticMesh` _staticmesh11_3 "/Game/OldVillage/Meshes/Structure_Components/SM_Pole_001.SM_Pole_001")
              (`SceneComponent.K2_SetRelativeTransform` _staticmesh11_3 (`KismetMathLibrary.MakeTransform` (174.094849 3.647747 35.692516) (struct) (0.835832 0.473918 1.324234)) false false)))))
      (if (`self.Window Flowers`)
        (switch `int` (`self.Choose Flower`)
          (:`1`
            (`StaticMeshComponent.SetStaticMesh` _staticmesh14_4 "/Game/OldVillage/Meshes/Vegetation/SM_Flower__Window_001.SM_Flower__Window_001")
            (`SceneComponent.K2_SetRelativeTransform` _staticmesh14_4 (`KismetMathLibrary.MakeTransform` (91.871246 11.42564 33.579216) (struct)) false false))
          (:`2`
            (`StaticMeshComponent.SetStaticMesh` _staticmesh14 "/Game/OldVillage/Meshes/Vegetation/SM_Flower__Window_003.SM_Flower__Window_003")
            (`SceneComponent.K2_SetRelativeTransform` _staticmesh14 (`KismetMathLibrary.MakeTransform` (100.784027 8.583052 40.303425) (struct)) false false))
          (:`3`
            (`StaticMeshComponent.SetStaticMesh` _staticmesh14_3 "/Game/OldVillage/Meshes/Vegetation/SM_Flower__Window_002.SM_Flower__Window_002")
            (`SceneComponent.K2_SetRelativeTransform` _staticmesh14_3 (`KismetMathLibrary.MakeTransform` (98.65834 1.245066 23.826042) (struct)) false false)))))
    (:`NewEnumerator2`
      (if (`self.Abbandoned building`)
        ;[1 1 1] Window 02_Abbandoned
        ;;[1 1 1] Base
        (`StaticMeshComponent.SetStaticMesh` _staticmesh_8 "/Game/OldVillage/Meshes/Structure_Components/SM_Wall_2mx2m_window_003_abbandoned_component.SM_Wall_2mx2m_window_003_abbandoned_component")
        (`SceneComponent.K2_SetRelativeTransform` _staticmesh_8 (`KismetMathLibrary.MakeTransform` (0.0 0.0 0.0) (struct)) false false)
        ;;[1 1 1] Window body
        (`StaticMeshComponent.SetStaticMesh` _staticmesh1 "/Game/OldVillage/Meshes/Structure_Components/SM_Window_003_abbandoned_frame.SM_Window_003_abbandoned_frame")
        (`SceneComponent.K2_SetRelativeTransform` _staticmesh1 (`KismetMathLibrary.MakeTransform` (124.371246 -16.489357 52.227348) (struct :`Yaw` -89.999992) (0.745748 0.966496 0.956341)) false false)
        (switch `int` (`self.Choose abbandoned window glass`)
          (:`1`
            ;;[1 1 1] Glass
            (`StaticMeshComponent.SetStaticMesh` _staticmesh2_5 "/Game/OldVillage/Meshes/Structure_Components/SM_Window_003_abbandoned_glass_001.SM_Window_003_abbandoned_glass_001")
            (`SceneComponent.K2_SetRelativeTransform` _staticmesh2_5 (`KismetMathLibrary.MakeTransform` (124.371246 -16.489357 52.227348) (struct :`Yaw` -89.999992) (0.745748 0.966496 0.956341)) false false))
          (:`2`
            ;;[1 1 1] Glass
            (`StaticMeshComponent.SetStaticMesh` _staticmesh2 "/Game/OldVillage/Meshes/Structure_Components/SM_Window_003_abbandoned_glass_002.SM_Window_003_abbandoned_glass_002")
            (`SceneComponent.K2_SetRelativeTransform` _staticmesh2 (`KismetMathLibrary.MakeTransform` (124.371246 -16.489357 52.227348) (struct :`Yaw` -89.999992) (0.745748 0.966496 0.956341)) false false))
          (:`3`
            _))
        ;;[1 1 1] Shutters support
        (`StaticMeshComponent.SetStaticMesh` _staticmesh4_4 "/Game/OldVillage/Meshes/Structure_Components/SM_Window_Shutter_003_support_abbandoned.SM_Window_Shutter_003_support_abbandoned")
        (`SceneComponent.K2_SetRelativeTransform` _staticmesh4_4 (`KismetMathLibrary.MakeTransform` (66.938431 7.452263 53.735527) (struct :`Yaw` -90.0)) false false)
        ;;[1 1 1] Remove left shutter
        (if (not (`self.Remove left shutter`))
          ;;[1 1 1] Shutter
          (`StaticMeshComponent.SetStaticMesh` _staticmesh6_4 "/Game/OldVillage/Meshes/Structure_Components/SM_Window_Shutter_003_abbandoned.SM_Window_Shutter_003_abbandoned")
          (`SceneComponent.K2_SetRelativeTransform` _staticmesh6_4 (`KismetMathLibrary.MakeTransform` (66.938431 7.452263 53.735527) (struct :`Yaw` -90.0)) false false))
        ;;[1 1 1] Shutters movement
        (`SceneComponent.K2_SetRelativeRotation` _staticmesh6_4 (`KismetMathLibrary.RLerp` (`KismetMathLibrary.MakeRotator` 0.0 0.0 -94.0) (`KismetMathLibrary.MakeRotator` 0.0 0.0 97.0) (`KismetMathLibrary.FClamp` (`self.Left shutter - 1 = Open 0 = Closed`))) false false)
        (else
          ;[1 1 1] Window 02
          ;;[1 1 1] Base
          (`StaticMeshComponent.SetStaticMesh` _staticmesh_10 "/Game/OldVillage/Meshes/Structure_Components/SM_Wall_2mx2m_window_003_component.SM_Wall_2mx2m_window_003_component")
          (`SceneComponent.K2_SetRelativeTransform` _staticmesh_10 (`KismetMathLibrary.MakeTransform` (0.0 0.0 0.0) (struct)) false false)
          ;;[1 1 1] Window body
          (`StaticMeshComponent.SetStaticMesh` _staticmesh1_4 "/Game/OldVillage/Meshes/Structure_Components/SM_Window_003.SM_Window_003")
          (`SceneComponent.K2_SetRelativeTransform` _staticmesh1_4 (`KismetMathLibrary.MakeTransform` (124.371246 -16.489357 52.227348) (struct :`Yaw` -89.999992) (0.745748 0.966496 0.956341)) false false)
          ;;[1 1 1] Shutters support
          (`StaticMeshComponent.SetStaticMesh` _staticmesh4_3 "/Game/OldVillage/Meshes/Structure_Components/SM_Window_Shutter_003_support.SM_Window_Shutter_003_support")
          (`SceneComponent.K2_SetRelativeTransform` _staticmesh4_3 (`KismetMathLibrary.MakeTransform` (66.938431 7.452263 53.735527) (struct :`Yaw` -90.0)) false false)
          ;;[1 1 1] Remove left shutter
          (if (not (`self.Remove left shutter`))
            ;;[1 1 1] Ledt Shutter
            (`StaticMeshComponent.SetStaticMesh` _staticmesh6_3 "/Game/OldVillage/Meshes/Structure_Components/SM_Window_Shutter_003.SM_Window_Shutter_003")
            (`SceneComponent.K2_SetRelativeTransform` _staticmesh6_3 (`KismetMathLibrary.MakeTransform` (66.938431 7.452263 53.735527) (struct :`Yaw` -90.0)) false false))
          ;;[1 1 1] Shutters movement
          (`SceneComponent.K2_SetRelativeRotation` _staticmesh6_3 (`KismetMathLibrary.RLerp` (`KismetMathLibrary.MakeRotator` 0.0 0.0 -94.0) (`KismetMathLibrary.MakeRotator` 0.0 0.0 97.0) (`KismetMathLibrary.FClamp` (`self.Left shutter - 1 = Open 0 = Closed`))) false false)))
      (if (`self.Window Flowers`)
        (`StaticMeshComponent.SetStaticMesh` _staticmesh14_2 "/Game/OldVillage/Meshes/Vegetation/SM_Flower__Window_004.SM_Flower__Window_004")
        (`SceneComponent.K2_SetRelativeTransform` _staticmesh14_2 (`KismetMathLibrary.MakeTransform` (98.89225 0.545104 61.02829) (struct)) false false)))
    (:`NewEnumerator3`
      ;[1 1 1] Right corner 90
      (if (`self.Abbandoned building`)
        (`StaticMeshComponent.SetStaticMesh` _staticmesh_4 "/Game/OldVillage/Meshes/Structure_Components/SM_Wall_2mx2m_Edge_L_001_abbandoned.SM_Wall_2mx2m_Edge_L_001_abbandoned")
        (`SceneComponent.K2_SetRelativeTransform` _staticmesh_4 (`KismetMathLibrary.MakeTransform` (0.0 0.0 0.0) (struct)) false false)
        (else
          (`StaticMeshComponent.SetStaticMesh` _staticmesh_3 "/Game/OldVillage/Meshes/Structure_Components/SM_Wall_2mx2m_Edge_L_001.SM_Wall_2mx2m_Edge_L_001")
          (`SceneComponent.K2_SetRelativeTransform` _staticmesh_3 (`KismetMathLibrary.MakeTransform` (0.0 0.0 0.0) (struct)) false false))))
    (:`NewEnumerator5`
      ;[1 1 1] Right corner 45
      (if (`self.Abbandoned building`)
        (`StaticMeshComponent.SetStaticMesh` _staticmesh_12 "/Game/OldVillage/Meshes/Structure_Components/SM_Wall_2mx2m_Edge_R_45_001_abbandoned.SM_Wall_2mx2m_Edge_R_45_001_abbandoned")
        (`SceneComponent.K2_SetRelativeTransform` _staticmesh_12 (`KismetMathLibrary.MakeTransform` (0.0 0.0 0.0) (struct)) false false)
        (else
          (`StaticMeshComponent.SetStaticMesh` _staticmesh_13 "/Game/OldVillage/Meshes/Structure_Components/SM_Wall_2mx2m_Edge_R_45_001.SM_Wall_2mx2m_Edge_R_45_001")
          (`SceneComponent.K2_SetRelativeTransform` _staticmesh_13 (`KismetMathLibrary.MakeTransform` (0.0 0.0 0.0) (struct)) false false))))
    (:`NewEnumerator4`
      ;[1 1 1] Left Corner 90
      (if (`self.Abbandoned building`)
        (`StaticMeshComponent.SetStaticMesh` _staticmesh_2 "/Game/OldVillage/Meshes/Structure_Components/SM_Wall_2mx2m_Edge_R_001_abbandoned.SM_Wall_2mx2m_Edge_R_001_abbandoned")
        (`SceneComponent.K2_SetRelativeTransform` _staticmesh_2 (`KismetMathLibrary.MakeTransform` (200.0 0.0 0.0) (struct)) false false)
        (else
          (`StaticMeshComponent.SetStaticMesh` _staticmesh "/Game/OldVillage/Meshes/Structure_Components/SM_Wall_2mx2m_Edge_R_001.SM_Wall_2mx2m_Edge_R_001")
          (`SceneComponent.K2_SetRelativeTransform` _staticmesh (`KismetMathLibrary.MakeTransform` (200.0 0.0 0.0) (struct)) false false))))
    (:`NewEnumerator6`
      ;[1 1 1] Left Corner 45
      (if (`self.Abbandoned building`)
        (`StaticMeshComponent.SetStaticMesh` _staticmesh_6 "/Game/OldVillage/Meshes/Structure_Components/SM_Wall_2mx2m_Edge_L_45_001_abbandoned.SM_Wall_2mx2m_Edge_L_45_001_abbandoned")
        (`SceneComponent.K2_SetRelativeTransform` _staticmesh_6 (`KismetMathLibrary.MakeTransform` (200.0 0.0 0.0) (struct)) false false)
        (else
          (`StaticMeshComponent.SetStaticMesh` _staticmesh_14 "/Game/OldVillage/Meshes/Structure_Components/SM_Wall_2mx2m_Edge_L_45_001.SM_Wall_2mx2m_Edge_L_45_001")
          (`SceneComponent.K2_SetRelativeTransform` _staticmesh_14 (`KismetMathLibrary.MakeTransform` (200.0 0.0 0.0) (struct)) false false))))))