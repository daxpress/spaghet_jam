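; Modular 2m x 1m Old Village wall piece, configured entirely in the Construction Script, with no runtime logic.
; ChooseComponent selects a plain wall, window, or left/right 90°, 45° or curved corner, with AbbandonedBuilding selecting derelict variants.
; Windows add selectable bars and stone or pole surrounds on extra mesh components.
; Interior/exterior material overrides feed a stucco-tinted dynamic instance; curved corners swap slots and tint a hardcoded blend material instead.
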(fn `UserConstructionScript`
  (bind _staticmesh1 (`self.StaticMesh1`))
  (bind _static_mesh (`self.Static Mesh`))
  (bind _static_mesh_2 (`self.Static Mesh`))
  (bind _staticmesh5 (`self.StaticMesh5`))
  (bind _static_mesh_3 (`self.Static Mesh`))
  (bind _static_mesh_4 (`self.Static Mesh`))
  (bind _staticmesh1_2 (`self.StaticMesh1`))
  (bind _static_mesh_5 (`self.Static Mesh`))
  (bind _static_mesh_6 (`self.Static Mesh`))
  (bind _static_mesh_7 (`self.Static Mesh`))
  (bind _static_mesh_8 (`self.Static Mesh`))
  (bind _static_mesh_9 (`self.Static Mesh`))
  (bind _static_mesh_10 (`self.Static Mesh`))
  (bind _static_mesh_11 (`self.Static Mesh`))
  (bind _static_mesh_12 (`self.Static Mesh`))
  (bind _exterior_material_override (`self.Exterior Material Override`))
  (bind _staticmesh2 (`self.StaticMesh2`))
  (bind _staticmesh3 (`self.StaticMesh3`))
  (bind _staticmesh4 (`self.StaticMesh4`))
  (bind _staticmesh5_2 (`self.StaticMesh5`))
  (bind _staticmesh2_2 (`self.StaticMesh2`))
  (bind _staticmesh3_2 (`self.StaticMesh3`))
  (bind _staticmesh4_2 (`self.StaticMesh4`))
  (bind _staticmesh5_3 (`self.StaticMesh5`))
  (bind _static_mesh_13 (`self.Static Mesh`))
  (bind _static_mesh_14 (`self.Static Mesh`))
  (bind _staticmesh2_3 (`self.StaticMesh2`))
  (bind _staticmesh1_3 (`self.StaticMesh1`))
  (bind _staticmesh2_4 (`self.StaticMesh2`))
  (bind _staticmesh3_3 (`self.StaticMesh3`))
  (bind _staticmesh4_3 (`self.StaticMesh4`))
  (bind _staticmesh5_4 (`self.StaticMesh5`))
  (bind _staticmesh2_5 (`self.StaticMesh2`))
  (bind _staticmesh3_4 (`self.StaticMesh3`))
  (bind _staticmesh4_4 (`self.StaticMesh4`))
  (bind _staticmesh5_5 (`self.StaticMesh5`))
  (bind _staticmesh3_5 (`self.StaticMesh3`))
  (bind _staticmesh4_5 (`self.StaticMesh4`))
  (`PrimitiveComponent.SetMaterial` _static_mesh 0 (`self.Interior Material Override`))
  (`PrimitiveComponent.SetMaterial` _static_mesh 1 _exterior_material_override)
  ;[1 1 1] Change stucco Color
  (bind _returnvalue (`PrimitiveComponent.CreateDynamicMaterialInstance` (`self.Static Mesh`) 1 _exterior_material_override "None"))
  (`MaterialInstanceDynamic.SetVectorParameterValue` _returnvalue "Material 2 Color multiplier" (`self.Stucco Color`))
  (switch `/Game/OldVillage/Meshes/Structure/Enumerators/BP_2mx1m_enum` (`self.Choose component`)
    (:`NewEnumerator0`
      ;[1 1 1] Basic Wall
      (if (`self.Abbandoned Building`)
        (`StaticMeshComponent.SetStaticMesh` _static_mesh_13 "/Game/OldVillage/Meshes/Structure_Components/SM_Wall_2mx1m_001_abbandoned.SM_Wall_2mx1m_001_abbandoned")
        (`SceneComponent.K2_SetRelativeTransform` _static_mesh_13 (`KismetMathLibrary.MakeTransform` (0.0 0.0 0.0) (struct) (1.0 1.0 1.0)) false false)))
    (:`NewEnumerator5`
      (if (`self.Abbandoned Building`)
        ;[1 1 1] Base
        (`StaticMeshComponent.SetStaticMesh` (`self.Static Mesh`) "/Game/OldVillage/Meshes/Structure_Components/SM_Wall_2mx1m_window_001_abbandoned.SM_Wall_2mx1m_window_001_abbandoned")
        (else
          ;[1 1 1] Base
          (`StaticMeshComponent.SetStaticMesh` (`self.Static Mesh`) "/Game/OldVillage/Meshes/Structure_Components/SM_Wall_2mx1m_window_001.SM_Wall_2mx1m_window_001")))
      (switch `int` (`self.Choose Bars`)
        (:`1`
          ;[1 1 1] Bars
          (`StaticMeshComponent.SetStaticMesh` _staticmesh1 "/Game/OldVillage/Meshes/Structure_Components/SM_Bars_001.SM_Bars_001")
          (`SceneComponent.K2_SetRelativeTransform` _staticmesh1 (`KismetMathLibrary.MakeTransform` (0.0 0.0 0.0) (struct) (1.0 1.0 1.0)) false false))
        (:`2`
          (`StaticMeshComponent.SetStaticMesh` _staticmesh1_2 "/Game/OldVillage/Meshes/Structure_Components/SM_Bars_003.SM_Bars_003")
          (`SceneComponent.K2_SetRelativeTransform` _staticmesh1_2 (`KismetMathLibrary.MakeTransform` (0.0 0.0 0.0) (struct) (1.0 1.0 1.0)) false false))
        (:`3`
          (`StaticMeshComponent.SetStaticMesh` _staticmesh1_3 "/Game/OldVillage/Meshes/Structure_Components/SM_Bars_002.SM_Bars_002")
          (`SceneComponent.K2_SetRelativeTransform` _staticmesh1_3 (`KismetMathLibrary.MakeTransform` (0.0 0.0 0.0) (struct) (1.0 1.0 1.0)) false false)))
      (if (`self.Abbandoned Building`)
        (`PrimitiveComponent.SetMaterial` (`self.StaticMesh1`) 0 "/Game/OldVillage/Materials/Meshspecific/MI_Fireplace_tools_001_Rusty.MI_Fireplace_tools_001_Rusty"))
      (switch `int` (`self.Choose window encase`)
        (:`1`
          ;[1 1 1] Encase
          (`StaticMeshComponent.SetStaticMesh` _staticmesh2_4 "/Game/OldVillage/Meshes/Structure/Decore/SM_Decorative_Stone_007.SM_Decorative_Stone_007")
          (`SceneComponent.K2_SetRelativeTransform` _staticmesh2_4 (`KismetMathLibrary.MakeTransform` (54.321754 -11.474844 54.031212) (struct :`Pitch` -90.0) (1.110878 0.651156 1.0)) false false)
          (`StaticMeshComponent.SetStaticMesh` _staticmesh3_3 "/Game/OldVillage/Meshes/Structure/Decore/SM_Decorative_Stone_005.SM_Decorative_Stone_005")
          (`SceneComponent.K2_SetRelativeTransform` _staticmesh3_3 (`KismetMathLibrary.MakeTransform` (100.0 -10.146889 79.033096) (struct :`Yaw` 89.999977) (1.0 -1.0 -1.0)) false false)
          (`StaticMeshComponent.SetStaticMesh` _staticmesh4_3 "/Game/OldVillage/Meshes/Structure/Decore/SM_Decorative_Stone_008.SM_Decorative_Stone_008")
          (`SceneComponent.K2_SetRelativeTransform` _staticmesh4_3 (`KismetMathLibrary.MakeTransform` (148.884323 -11.474852 54.739952) (struct :`Pitch` -90.0) (1.19096 0.651156 1.0)) false false)
          (`StaticMeshComponent.SetStaticMesh` _staticmesh5_4 "/Game/OldVillage/Meshes/Structure/Decore/SM_Decorative_Stone_005.SM_Decorative_Stone_005")
          (`SceneComponent.K2_SetRelativeTransform` _staticmesh5_4 (`KismetMathLibrary.MakeTransform` (100.0 -10.146851 31.525509) (struct :`Yaw` 89.999977) (1.0 1.0 1.0)) false false))
        (:`2`
          (`StaticMeshComponent.SetStaticMesh` _staticmesh2_5 "/Game/OldVillage/Meshes/Structure/Decore/SM_Decorative_Stone_006.SM_Decorative_Stone_006")
          (`SceneComponent.K2_SetRelativeTransform` _staticmesh2_5 (`KismetMathLibrary.MakeTransform` (54.706921 -9.647203 54.558296) (struct :`Yaw` -89.999969 :`Roll` 89.999962) (0.961507 0.759642 1.0)) false false)
          (`StaticMeshComponent.SetStaticMesh` _staticmesh3_4 "/Game/OldVillage/Meshes/Structure/Decore/SM_Decorative_Stone_005.SM_Decorative_Stone_005")
          (`SceneComponent.K2_SetRelativeTransform` _staticmesh3_4 (`KismetMathLibrary.MakeTransform` (103.99382 -10.146828 77.781204) (struct :`Yaw` 89.999977) (1.0 0.859593 -1.0)) false false)
          (`StaticMeshComponent.SetStaticMesh` _staticmesh4_4 "/Game/OldVillage/Meshes/Structure/Decore/SM_Decorative_Stone_006.SM_Decorative_Stone_006")
          (`SceneComponent.K2_SetRelativeTransform` _staticmesh4_4 (`KismetMathLibrary.MakeTransform` (148.239334 -11.474729 49.323219) (struct :`Yaw` -89.999947 :`Roll` -89.999893) (0.940926 0.642852 1.0)) false false)
          (`StaticMeshComponent.SetStaticMesh` _staticmesh5_5 "/Game/OldVillage/Meshes/Structure/Decore/SM_Decorative_Stone_005.SM_Decorative_Stone_005")
          (`SceneComponent.K2_SetRelativeTransform` _staticmesh5_5 (`KismetMathLibrary.MakeTransform` (100.144753 -10.146667 29.470009) (struct :`Yaw` 89.999977) (1.0 -0.80841 -1.0)) false false))
        (:`3`
          (`StaticMeshComponent.SetStaticMesh` _staticmesh2 "/Game/OldVillage/Meshes/Structure/Decore/SM_Decorative_Stone_006.SM_Decorative_Stone_006")
          (`SceneComponent.K2_SetRelativeTransform` _staticmesh2 (`KismetMathLibrary.MakeTransform` (53.411507 -11.475012 60.766285) (struct :`Yaw` -89.999947 :`Roll` -89.999893) (-0.940926 0.642852 1.0)) false false)
          (`StaticMeshComponent.SetStaticMesh` _staticmesh3 "/Game/OldVillage/Meshes/Structure/Decore/SM_Decorative_Stone_005.SM_Decorative_Stone_005")
          (`SceneComponent.K2_SetRelativeTransform` _staticmesh3 (`KismetMathLibrary.MakeTransform` (98.930344 -10.146811 77.781204) (struct :`Yaw` 89.999977) (-1.0 -0.779565 -1.0)) false false)
          (`StaticMeshComponent.SetStaticMesh` _staticmesh4 "/Game/OldVillage/Meshes/Structure/Decore/SM_Decorative_Stone_006.SM_Decorative_Stone_006")
          (`SceneComponent.K2_SetRelativeTransform` _staticmesh4 (`KismetMathLibrary.MakeTransform` (145.674622 -9.647234 52.126915) (struct :`Pitch` 4.1e-05 :`Yaw` -89.999969 :`Roll` 89.999962) (-0.961507 0.759642 1.0)) false false)
          (`StaticMeshComponent.SetStaticMesh` _staticmesh5_2 "/Game/OldVillage/Meshes/Structure/Decore/SM_Decorative_Stone_005.SM_Decorative_Stone_005")
          (`SceneComponent.K2_SetRelativeTransform` _staticmesh5_2 (`KismetMathLibrary.MakeTransform` (96.220215 -10.146767 29.470009) (struct :`Yaw` 89.999977) (-1.0 0.80841 -1.0)) false false))
        (:`4`
          (if (`self.Abbandoned Building`)
            (`StaticMeshComponent.SetStaticMesh` _staticmesh2_3 "/Game/OldVillage/Meshes/Structure_Components/SM_Pole_002_abbandoned.SM_Pole_002_abbandoned")
            (`SceneComponent.K2_SetRelativeTransform` _staticmesh2_3 (`KismetMathLibrary.MakeTransform` (50.914761 3.28194 36.720535) (struct :`Pitch` -7e-06 :`Yaw` -7e-06 :`Roll` -1.2e-05) (0.626252 1.426453 0.390851)) false false)
            (`StaticMeshComponent.SetStaticMesh` _staticmesh3_5 "/Game/OldVillage/Meshes/Structure_Components/SM_Pole_001_abbandoned.SM_Pole_001_abbandoned")
            (`SceneComponent.K2_SetRelativeTransform` _staticmesh3_5 (`KismetMathLibrary.MakeTransform` (51.634727 5.492479 74.225685) (struct :`Pitch` -90.0) (0.626252 1.23985 1.020725)) false false)
            (`StaticMeshComponent.SetStaticMesh` _staticmesh4_5 "/Game/OldVillage/Meshes/Structure_Components/SM_Pole_002_abbandoned.SM_Pole_002_abbandoned")
            (`SceneComponent.K2_SetRelativeTransform` _staticmesh4_5 (`KismetMathLibrary.MakeTransform` (151.792511 1.888466 75.388474) (struct :`Pitch` 1.4e-05 :`Yaw` -179.999878 :`Roll` 179.999939) (0.626252 1.394532 0.390851)) false false)
            (`StaticMeshComponent.SetStaticMesh` _staticmesh5 "/Game/OldVillage/Meshes/Structure_Components/SM_Pole_001_abbandoned.SM_Pole_001_abbandoned")
            (`SceneComponent.K2_SetRelativeTransform` _staticmesh5 (`KismetMathLibrary.MakeTransform` (152.288208 6.153652 36.720535) (struct :`Pitch` 90.0 :`Yaw` 1.9e-05) (0.626252 1.394532 1.020725)) false false)
            (else
              (`StaticMeshComponent.SetStaticMesh` _staticmesh2_2 "/Game/OldVillage/Meshes/Structure_Components/SM_Pole_002.SM_Pole_002")
              (`SceneComponent.K2_SetRelativeTransform` _staticmesh2_2 (`KismetMathLibrary.MakeTransform` (50.914761 3.28194 36.720535) (struct :`Pitch` -7e-06 :`Yaw` -7e-06 :`Roll` -1.2e-05) (0.626252 1.426453 0.390851)) false false)
              (`StaticMeshComponent.SetStaticMesh` _staticmesh3_2 "/Game/OldVillage/Meshes/Structure_Components/SM_Pole_001.SM_Pole_001")
              (`SceneComponent.K2_SetRelativeTransform` _staticmesh3_2 (`KismetMathLibrary.MakeTransform` (51.634727 5.492479 74.225685) (struct :`Pitch` -90.0) (0.626252 1.23985 1.020725)) false false)
              (`StaticMeshComponent.SetStaticMesh` _staticmesh4_2 "/Game/OldVillage/Meshes/Structure_Components/SM_Pole_002.SM_Pole_002")
              (`SceneComponent.K2_SetRelativeTransform` _staticmesh4_2 (`KismetMathLibrary.MakeTransform` (151.792511 1.888466 75.388474) (struct :`Pitch` 1.4e-05 :`Yaw` -179.999878 :`Roll` 179.999939) (0.626252 1.394532 0.390851)) false false)
              (`StaticMeshComponent.SetStaticMesh` _staticmesh5_3 "/Game/OldVillage/Meshes/Structure_Components/SM_Pole_001.SM_Pole_001")
              (`SceneComponent.K2_SetRelativeTransform` _staticmesh5_3 (`KismetMathLibrary.MakeTransform` (152.288208 6.153652 36.720535) (struct :`Pitch` 90.0 :`Yaw` 1.9e-05) (0.626252 1.394532 1.020725)) false false))))))
    (:`NewEnumerator1`
      (if (`self.Abbandoned Building`)
        ;[1 1 1] Corner 90 IN R
        (`StaticMeshComponent.SetStaticMesh` _static_mesh_10 "/Game/OldVillage/Meshes/Structure_Components/SM_Wall_2mx1m_Edge_L_001_abbandoned.SM_Wall_2mx1m_Edge_L_001_abbandoned")
        (`SceneComponent.K2_SetRelativeTransform` _static_mesh_10 (`KismetMathLibrary.MakeTransform` (0.0 0.0 0.0) (struct) (1.0 1.0 1.0)) false false)
        (else
          (`StaticMeshComponent.SetStaticMesh` _static_mesh_9 "/Game/OldVillage/Meshes/Structure_Components/SM_Wall_2mx1m_Edge_L_001.SM_Wall_2mx1m_Edge_L_001")
          (`SceneComponent.K2_SetRelativeTransform` _static_mesh_9 (`KismetMathLibrary.MakeTransform` (0.0 0.0 0.0) (struct) (1.0 1.0 1.0)) false false))))
    (:`NewEnumerator6`
      (if (`self.Abbandoned Building`)
        ;[1 1 1] Corner 45 IN R
        (`StaticMeshComponent.SetStaticMesh` _static_mesh_2 "/Game/OldVillage/Meshes/Structure_Components/SM_Wall_2mx1m_Edge_45_R_001_abbandoned.SM_Wall_2mx1m_Edge_45_R_001_abbandoned")
        (`SceneComponent.K2_SetRelativeTransform` _static_mesh_2 (`KismetMathLibrary.MakeTransform` (0.0 0.0 0.0) (struct) (1.0 1.0 1.0)) false false)
        (else
          (`StaticMeshComponent.SetStaticMesh` _static_mesh_3 "/Game/OldVillage/Meshes/Structure_Components/SM_Wall_2mx1m_Edge_45_R_001.SM_Wall_2mx1m_Edge_45_R_001")
          (`SceneComponent.K2_SetRelativeTransform` _static_mesh_3 (`KismetMathLibrary.MakeTransform` (0.0 0.0 0.0) (struct) (1.0 1.0 1.0)) false false))))
    (:`NewEnumerator9`
      ;[1 1 1] Change stucco Color
      (`PrimitiveComponent.SetMaterial` (`self.Static Mesh`) 1 (`self.Interior Material Override`))
      (`PrimitiveComponent.SetMaterial` (`self.Static Mesh`) 0 (`self.Exterior Material Override`))
      (bind _returnvalue_2 (`PrimitiveComponent.CreateDynamicMaterialInstance` (`self.Static Mesh`) 0 "/Game/OldVillage/Materials/Tileable/MI_Blend_Stones_Exterior_001_to_Stucco_fine_001_parallax.MI_Blend_Stones_Exterior_001_to_Stucco_fine_001_parallax" "None"))
      (`MaterialInstanceDynamic.SetVectorParameterValue` _returnvalue_2 "Material 2 Color multiplier" (`self.Stucco Color`))
      (if (`self.Abbandoned Building`)
        ;[1 1 1] Corner curved R
        (`StaticMeshComponent.SetStaticMesh` _static_mesh_6 "/Game/OldVillage/Meshes/Structure_Components/SM_Wall_2mx1m_Edge_curved_R_001_abbandoned.SM_Wall_2mx1m_Edge_curved_R_001_abbandoned")
        (`SceneComponent.K2_SetRelativeTransform` _static_mesh_6 (`KismetMathLibrary.MakeTransform` (0.0 0.0 0.0) (struct) (1.0 1.0 1.0)) false false)
        (else
          (`StaticMeshComponent.SetStaticMesh` _static_mesh_5 "/Game/OldVillage/Meshes/Structure_Components/SM_Wall_2mx1m_Edge_curved_R_001.SM_Wall_2mx1m_Edge_curved_R_001")
          (`SceneComponent.K2_SetRelativeTransform` _static_mesh_5 (`KismetMathLibrary.MakeTransform` (0.0 0.0 0.0) (struct) (1.0 1.0 1.0)) false false))))
    (:`NewEnumerator2`
      (if (`self.Abbandoned Building`)
        ;[1 1 1] Corner 90 IN L
        (`StaticMeshComponent.SetStaticMesh` _static_mesh_8 "/Game/OldVillage/Meshes/Structure_Components/SM_Wall_2mx1m_Edge_R_001_abbandoned.SM_Wall_2mx1m_Edge_R_001_abbandoned")
        (`SceneComponent.K2_SetRelativeTransform` _static_mesh_8 (`KismetMathLibrary.MakeTransform` (200.0 0.0 0.0) (struct) (1.0 1.0 1.0)) false false)
        (else
          (`StaticMeshComponent.SetStaticMesh` _static_mesh_7 "/Game/OldVillage/Meshes/Structure_Components/SM_Wall_2mx1m_Edge_R_001.SM_Wall_2mx1m_Edge_R_001")
          (`SceneComponent.K2_SetRelativeTransform` _static_mesh_7 (`KismetMathLibrary.MakeTransform` (200.0 0.0 0.0) (struct) (1.0 1.0 1.0)) false false))))
    (:`NewEnumerator7`
      (if (`self.Abbandoned Building`)
        ;[1 1 1] Corner 45 IN L
        (`StaticMeshComponent.SetStaticMesh` _static_mesh_12 "/Game/OldVillage/Meshes/Structure_Components/SM_Wall_2mx1m_Edge_45_L_001_abbandoned.SM_Wall_2mx1m_Edge_45_L_001_abbandoned")
        (`SceneComponent.K2_SetRelativeTransform` _static_mesh_12 (`KismetMathLibrary.MakeTransform` (200.0 0.0 0.0) (struct) (1.0 1.0 1.0)) false false)
        (else
          (`StaticMeshComponent.SetStaticMesh` _static_mesh_11 "/Game/OldVillage/Meshes/Structure_Components/SM_Wall_2mx1m_Edge_45_L_001.SM_Wall_2mx1m_Edge_45_L_001")
          (`SceneComponent.K2_SetRelativeTransform` _static_mesh_11 (`KismetMathLibrary.MakeTransform` (200.0 0.0 0.0) (struct) (1.0 1.0 1.0)) false false))))
    (:`NewEnumerator8`
      ;[1 1 1] Change stucco Color
      (`PrimitiveComponent.SetMaterial` (`self.Static Mesh`) 1 (`self.Interior Material Override`))
      (`PrimitiveComponent.SetMaterial` (`self.Static Mesh`) 0 (`self.Exterior Material Override`))
      (bind _returnvalue_3 (`PrimitiveComponent.CreateDynamicMaterialInstance` (`self.Static Mesh`) 0 "/Game/OldVillage/Materials/Tileable/MI_Blend_Stones_Exterior_001_to_Stucco_fine_001_parallax.MI_Blend_Stones_Exterior_001_to_Stucco_fine_001_parallax" "None"))
      (`MaterialInstanceDynamic.SetVectorParameterValue` _returnvalue_3 "Material 2 Color multiplier" (`self.Stucco Color`))
      (if (`self.Abbandoned Building`)
        ;[1 1 1] Corner curved L
        (`StaticMeshComponent.SetStaticMesh` _static_mesh_14 "/Game/OldVillage/Meshes/Structure_Components/SM_Wall_2mx1m_Edge_curved_L_001_abbandoned.SM_Wall_2mx1m_Edge_curved_L_001_abbandoned")
        (`SceneComponent.K2_SetRelativeTransform` _static_mesh_14 (`KismetMathLibrary.MakeTransform` (200.0 0.0 0.0) (struct) (1.0 1.0 1.0)) false false)
        (else
          (`StaticMeshComponent.SetStaticMesh` _static_mesh_4 "/Game/OldVillage/Meshes/Structure_Components/SM_Wall_2mx1m_Edge_curved_L_001.SM_Wall_2mx1m_Edge_curved_L_001")
          (`SceneComponent.K2_SetRelativeTransform` _static_mesh_4 (`KismetMathLibrary.MakeTransform` (200.0 0.0 0.0) (struct) (1.0 1.0 1.0)) false false))))))