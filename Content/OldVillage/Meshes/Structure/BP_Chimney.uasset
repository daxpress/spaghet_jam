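; BP_Chimney is a configurable chimney prop for the OldVillage structure meshes, built entirely in the construction script.
; ChooseComponent selects the variant: Flat 01 swaps the main mesh to the flat chimney, while Inclined 01 leaves it unchanged.
; After that switch, four components receive the same decorative stone mesh at hard-coded transforms around the chimney, using negative scales to mirror it.
; The event graph holds only disabled placeholder events.
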(fn `UserConstructionScript`
  (bind _staticmesh2 (`self.StaticMesh2`))
  (bind _staticmesh3 (`self.StaticMesh3`))
  (bind _staticmesh4 (`self.StaticMesh4`))
  (bind _staticmesh1 (`self.StaticMesh1`))
  (switch `/Game/OldVillage/Meshes/Structure/Enumerators/BP_Chimney_Enum` (`self.Choose Component`)
    (:`NewEnumerator0`
      _)
    (:`NewEnumerator1`
      (`StaticMeshComponent.SetStaticMesh` (`self.StaticMesh`) "/Game/OldVillage/Meshes/Structure_Components/SM_Chimney_flat_001.SM_Chimney_flat_001")))
  (`StaticMeshComponent.SetStaticMesh` _staticmesh1 "/Game/OldVillage/Meshes/Structure/Decore/SM_Decorative_Stone_005.SM_Decorative_Stone_005")
  (`SceneComponent.K2_SetRelativeTransform` _staticmesh1 (`KismetMathLibrary.MakeTransform` (-18.408001 -1.069945 89.767464) (struct :`Pitch` 90.0) (-0.550012 -0.490495 -1.172192)) false false)
  (`StaticMeshComponent.SetStaticMesh` _staticmesh2 "/Game/OldVillage/Meshes/Structure/Decore/SM_Decorative_Stone_005.SM_Decorative_Stone_005")
  (`SceneComponent.K2_SetRelativeTransform` _staticmesh2 (`KismetMathLibrary.MakeTransform` (0.901924 28.869675 89.767456) (struct :`Pitch` 90.0 :`Yaw` 180.0 :`Roll` -89.999474) (-0.560021 -0.454043 -1.397821)) false false)
  (`StaticMeshComponent.SetStaticMesh` _staticmesh3 "/Game/OldVillage/Meshes/Structure/Decore/SM_Decorative_Stone_005.SM_Decorative_Stone_005")
  (`SceneComponent.K2_SetRelativeTransform` _staticmesh3 (`KismetMathLibrary.MakeTransform` (19.097778 -0.407778 89.767464) (struct :`Pitch` 90.0 :`Yaw` 179.960312 :`Roll` -0.039307) (-0.559058 -0.49051 -1.2479)) false false)
  (`StaticMeshComponent.SetStaticMesh` _staticmesh4 "/Game/OldVillage/Meshes/Structure/Decore/SM_Decorative_Stone_005.SM_Decorative_Stone_005")
  (`SceneComponent.K2_SetRelativeTransform` _staticmesh4 (`KismetMathLibrary.MakeTransform` (0.901449 -29.965054 89.767456) (struct :`Pitch` 90.0 :`Yaw` 180.0 :`Roll` -89.999474) (-0.560021 -0.454043 -1.211604)) false false))