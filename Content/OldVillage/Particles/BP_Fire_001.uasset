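; Fire effect actor that flickers and sways two point lights to mimic firelight.
; On BeginPlay a timeline drives both light intensities, the first at four times the curve value, and feeds MoveComponentTo calls that shift each light along a differently scaled movement curve.
; The construction script exposes shadow casting for the main light and a switch that shows or hides both lights.
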(event `self.ReceiveBeginPlay`
  (bind (_direction _light_instensity _light1_movement) (`Timeline|Timeline_0`)
    (:`Update`
      (`LightComponent.SetIntensity` (`self.PointLight`) (* _light_instensity 4.0))
      (`LightComponent.SetIntensity` (`self.PointLight1`) _light_instensity)
      (`|ExecutionSequence`
        (:`then_0`
          (`KismetSystemLibrary.MoveComponentTo` (`self.PointLight`) (* _light1_movement (0.2 0.2 0.2))))
        (:`then_1`
          (`KismetSystemLibrary.MoveComponentTo` (`self.PointLight1`) (* _light1_movement (0.1 -0.2 0.1))))))))

(event `self.ReceiveTick`
  (params (DeltaSeconds :type "Float (single-precision)")))

(fn `UserConstructionScript`
  (bind _pointlight (`self.PointLight`))
  (`LightComponentBase.SetCastShadows` _pointlight (`self.Cast Shadows`))
  (`SceneComponent.SetVisibility` _pointlight (`self.Movable light switch`) false)
  (`SceneComponent.SetVisibility` (`self.PointLight1`) (`self.Movable light switch`) false))