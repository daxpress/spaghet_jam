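; Construction-script spline tool that repeats a static mesh along a spline as deformed spline mesh segments.
; It adds one segment per whole MeshLength of spline, leaving any shorter remainder uncovered.
; Each segment samples position, tangent and scale at both ends, with normalized tangents resized by MeshLength and TangentScale.
; The up vector comes from the segment midpoint, and end rolls are computed relative to that midpoint's rotation to follow banking.
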(fn `UserConstructionScript`
  (locals (last_roll :type "Float (double-precision)"))
  (bind _mesh_length (`self.mesh_length`))
  (bind _spline (`self.Spline`))
  (bind _returnvalue (* (`self.mesh_length`) (`self.tangent_scale`)))
  ;[1 1 1] loop along length of spline
  (for _index (range (`KismetMathLibrary.FTrunc` (/ (`SplineComponent.GetSplineLength` _spline) _mesh_length)))
    ;[1 1 1] create mesh
    (bind _returnvalue_2 (`AddComponent|NODE_AddSplineMeshComponent-6`))
    (`SplineMeshComponent.SetForwardAxis` _returnvalue_2 (`self.mesh_forward_axis`) true)
    (`StaticMeshComponent.SetStaticMesh` _returnvalue_2 (`self.mesh`))
    (`SceneComponent.K2_AttachToComponent` _returnvalue_2 null "None" "KeepRelative" "KeepRelative" "KeepRelative" true)
    (bind _returnvalue_3 (* _index _mesh_length))
    (bind _returnvalue_4 (* (+ _index 1) _mesh_length))
    (bind _returnvalue_5 (`KismetMathLibrary.Lerp` _returnvalue_3 _returnvalue_4 0.5))
    ;[1 1 1] position
    (`SplineMeshComponent.SetSplineUpDir` _returnvalue_2 (`KismetMathLibrary.Normal` (`SplineComponent.GetUpVectorAtDistanceAlongSpline` _spline _returnvalue_5 "Local")) true)
    (`SplineMeshComponent.SetStartAndEnd` _returnvalue_2 (`SplineComponent.GetLocationAtDistanceAlongSpline` _spline _returnvalue_3 "Local") (* (`KismetMathLibrary.Normal` (`SplineComponent.GetTangentAtDistanceAlongSpline` _spline _returnvalue_3 "Local")) _returnvalue) (`SplineComponent.GetLocationAtDistanceAlongSpline` _spline _returnvalue_4 "Local") (* (`KismetMathLibrary.Normal` (`SplineComponent.GetTangentAtDistanceAlongSpline` _spline _returnvalue_4 "Local")) _returnvalue) true)
    (bind _returnvalue_6 (`KismetMathLibrary.NegateRotator` (`SplineComponent.GetRotationAtDistanceAlongSpline` _spline _returnvalue_5 "Local")))
    ;[1 1 1] roll
    (`SplineMeshComponent.SetStartRoll` _returnvalue_2 (`KismetMathLibrary.DegreesToRadians` (.roll (`KismetMathLibrary.ComposeRotators` (`SplineComponent.GetRotationAtDistanceAlongSpline` _spline _returnvalue_3 "Local") _returnvalue_6))) true)
    (`SplineMeshComponent.SetEndRoll` _returnvalue_2 (`KismetMathLibrary.DegreesToRadians` (.roll (`KismetMathLibrary.ComposeRotators` (`SplineComponent.GetRotationAtDistanceAlongSpline` _spline _returnvalue_4 "Local") _returnvalue_6))) true)
    ;[1 1 1] scale
    (`SplineMeshComponent.SetStartScale` _returnvalue_2 (`KismetMathLibrary.MakeVector2D` (.y (`SplineComponent.GetScaleAtDistanceAlongSpline` _spline _returnvalue_3)) (.z (`SplineComponent.GetScaleAtDistanceAlongSpline` _spline _returnvalue_3))) true)
    (`SplineMeshComponent.SetEndScale` _returnvalue_2 (`KismetMathLibrary.MakeVector2D` (.y (`SplineComponent.GetScaleAtDistanceAlongSpline` _spline _returnvalue_4)) (.z (`SplineComponent.GetScaleAtDistanceAlongSpline` _spline _returnvalue_4))) true)))