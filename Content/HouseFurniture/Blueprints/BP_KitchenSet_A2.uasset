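; Interactive kitchen furniture set with doors that swing open and drawer-like cabinet parts that slide out.
; FurnitureTrace prints a "Press E" prompt, and FurnitureAction compares the traced component against six meshes to pick the part to move.
; Each part has its own FlipFlop that plays or reverses a Timeline, lerping rotation for the four doors or location for the two sliding cabinets.
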(event `self.FurnitureTrace`
  ;[1 1 1] DebugInfo
  (`KismetSystemLibrary.PrintText` "Press E" true false (struct :`R` 1.0 :`G` 1.0 :`B` 1.0 :`A` 1.0) 0.0))

(event `self.FurnitureAction`
  (params (TraceComponent :type "SceneComponent Object Reference"))
  (bind _staticmeshcomponent2 (`self.StaticMeshComponent2`))
  (bind _sm_kitchenset_a1_doorb1 (`self.SM_KitchenSet_A1_DoorB1`))
  (bind _sm_kitchenset_a1_cabinet_a2 (`self.SM_KitchenSet_A1_Cabinet_A2`))
  (bind _staticmeshcomponent1 (`self.StaticMeshComponent1`))
  (bind _sm_kitchenset_a1_doorb2 (`self.SM_KitchenSet_A1_DoorB2`))
  (bind _sm_kitchenset_a1_cabinet_a1 (`self.SM_KitchenSet_A1_Cabinet_A1`))
  ;[1 1 1] InteractionPart
  (if (== TraceComponent _staticmeshcomponent1)
    (`/Engine/EditorBlueprintResources/StandardMacros.FlipFlop`
      (:`A`
        (bind (_direction _alpha) (`Timeline|Timeline_0` :!label _label)
          (:`Update`
            (`SceneComponent.K2_SetRelativeRotation` _staticmeshcomponent1 (`KismetMathLibrary.RLerp` (struct) (struct :`Yaw` 90.0) _alpha) false false))))
      (:`B`
        (goto _label :!via `Reverse`)))
    (elif (== TraceComponent _staticmeshcomponent2)
      (`/Engine/EditorBlueprintResources/StandardMacros.FlipFlop`
        (:`A`
          (bind (_direction_2 _alpha_2) (`Timeline|Timeline_1` :!label _label_2)
            (:`Update`
              (`SceneComponent.K2_SetRelativeRotation` _staticmeshcomponent2 (`KismetMathLibrary.RLerp` (struct) (struct :`Yaw` -90.0) _alpha_2) false false))))
        (:`B`
          (goto _label_2 :!via `Reverse`)))
      (elif (== TraceComponent _sm_kitchenset_a1_doorb1)
        (`/Engine/EditorBlueprintResources/StandardMacros.FlipFlop`
          (:`A`
            (bind (_direction_3 _alpha_3) (`Timeline|Timeline_2` :!label _label_3)
              (:`Update`
                (`SceneComponent.K2_SetRelativeRotation` _sm_kitchenset_a1_doorb1 (`KismetMathLibrary.RLerp` (struct) (struct :`Yaw` -90.0) _alpha_3) false false))))
          (:`B`
            (goto _label_3 :!via `Reverse`)))
        (elif (== TraceComponent _sm_kitchenset_a1_doorb2)
          (`/Engine/EditorBlueprintResources/StandardMacros.FlipFlop`
            (:`A`
              (bind (_direction_4 _alpha_4) (`Timeline|Timeline_4` :!label _label_4)
                (:`Update`
                  (`SceneComponent.K2_SetRelativeRotation` _sm_kitchenset_a1_doorb2 (`KismetMathLibrary.RLerp` (struct) (struct :`Yaw` 90.0) _alpha_4) false false))))
            (:`B`
              (goto _label_4 :!via `Reverse`)))
          (elif (== TraceComponent _sm_kitchenset_a1_cabinet_a1)
            (`/Engine/EditorBlueprintResources/StandardMacros.FlipFlop`
              (:`A`
                (bind (_direction_5 _alpha_5) (`Timeline|Timeline_5` :!label _label_5)
                  (:`Update`
                    (`SceneComponent.K2_SetRelativeLocation` _sm_kitchenset_a1_cabinet_a1 (`KismetMathLibrary.VLerp` (74.184219 6.342057 72.795769) (74.184219 41.342056 72.795769) _alpha_5) false false))))
              (:`B`
                (goto _label_5 :!via `Reverse`)))
            (elif (== TraceComponent _sm_kitchenset_a1_cabinet_a2)
              (`/Engine/EditorBlueprintResources/StandardMacros.FlipFlop`
                (:`A`
                  (bind (_direction_6 _alpha_6) (`Timeline|Timeline_3` :!label _label_6)
                    (:`Update`
                      (`SceneComponent.K2_SetRelativeLocation` _sm_kitchenset_a1_cabinet_a2 (`KismetMathLibrary.VLerp` (106.702774 6.342043 72.795769) (106.702774 41.342041 72.795769) _alpha_6) false false))))
                (:`B`
                  (goto _label_6 :!via `Reverse`))))))))))

(fn `UserConstructionScript`)