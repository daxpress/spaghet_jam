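; BP_Microwave_A1 is an interactive microwave furniture Blueprint that shows a "Press E" prompt when traced.
; Each FurnitureAction alternates through a FlipFlop between playing and reversing a timeline that rotates StaticMeshComponent1, likely the door, by 90 degrees.
; The point light turns on when opening starts.
; It turns off when the timeline finishes in the closing state, provided the light's relative yaw is near zero.
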(event `/Game/HouseFurniture/Blueprints/Character/BP_Demo_Interface.FurnitureTrace`
  ;[1 1 1] DebugInfo
  (`KismetSystemLibrary.PrintText` "Press E" true false (struct :`R` 1.0 :`G` 1.0 :`B` 1.0 :`A` 1.0) 0.0))

(event `/Game/HouseFurniture/Blueprints/Character/BP_Demo_Interface.FurnitureAction`
  (params (TraceComponent :type "SceneComponent Object Reference"))
  (bind (_relativerotation_roll _relativerotation_pitch _relativerotation_yaw) (`KismetMathLibrary.BreakRotator` (`SceneComponent.RelativeRotation` (`self.PointLight`))))
  ;[1 1 1] InteractionPart
  (bind _isa (`/Engine/EditorBlueprintResources/StandardMacros.FlipFlop`)
    (:`A`
      (`LightComponent.SetIntensity` (`self.PointLight`) 20.0)
      (bind (_direction _alpha) (`Timeline|Timeline_0` :!label _label)
        (:`Update`
          (`SceneComponent.K2_SetRelativeRotation` (`self.StaticMeshComponent1`) (`KismetMathLibrary.RLerp` (struct) (struct :`Yaw` 90.0) _alpha) false false))
        (:`Finished`
          (if (and (not _isa) (`KismetMathLibrary.NearlyEqual_FloatFloat` _relativerotation_yaw 0.0 0.1))
            (`LightComponent.SetIntensity` (`self.PointLight`) 0.0)))))
    (:`B`
      (goto _label :!via `Reverse`))))

(fn `UserConstructionScript`)