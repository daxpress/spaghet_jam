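; BP_Door_Inside_A is an interior house door that swings open and closed on interaction.
; FurnitureTrace prints a "Press E" prompt, and FurnitureAction plays or reverses a timeline depending on IsClosed.
; The timeline drives the Door's relative yaw and marks it open only at 90 degrees or more, so reversing immediately counts as closed.
; The construction script applies the Element0 material to the door.
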(event `/Game/HouseFurniture/Blueprints/Character/BP_Demo_Interface.FurnitureTrace`
  (`KismetSystemLibrary.PrintText` "Press E" true false (struct :`R` 1.0 :`G` 1.0 :`B` 1.0 :`A` 1.0) 0.0))

(event `/Game/HouseFurniture/Blueprints/Character/BP_Demo_Interface.FurnitureAction`
  (params (TraceComponent :type "SceneComponent Object Reference"))
  (if (`self.IsClosed`)
    (bind (_direction _newtrack_1) (`Timeline|Timeline_0` :!label _label)
      (:`Update`
        (`SceneComponent.K2_SetRelativeRotation` (`self.Door`) (`KismetMathLibrary.MakeRotator` 0.0 0.0 _newtrack_1) false false)
        (if (>= _newtrack_1 90.0)
          (set `self.IsClosed` false)
          (else
            (set `self.IsClosed` true)))))
    (else
      (goto _label :!via `Reverse`))))

(fn `UserConstructionScript`
  (`PrimitiveComponent.SetMaterial` (`self.Door`) 0 (`self.Element 0`)))