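; BP_WorkingTable_A2 is an interactive house furniture work table with two sliding parts, likely drawers.
; FurnitureTrace shows a "Press E" prompt, and FurnitureAction checks which mesh component was traced.
; Each of the two handled meshes has its own FlipFlop that plays or reverses a timeline, lerping its relative location along Y to slide it out and back.
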(event `/Game/HouseFurniture/Blueprints/Character/BP_Demo_Interface.FurnitureTrace`
  ;[1 1 1] DebugInfo
  (`KismetSystemLibrary.PrintText` "Press E" true false (struct :`R` 1.0 :`G` 1.0 :`B` 1.0 :`A` 1.0) 0.0))

(event `/Game/HouseFurniture/Blueprints/Character/BP_Demo_Interface.FurnitureAction`
  (params (TraceComponent :type "SceneComponent Object Reference"))
  (bind _staticmeshcomponent4 (`self.StaticMeshComponent4`))
  (bind _staticmeshcomponent5 (`self.StaticMeshComponent5`))
  ;[1 1 1] InteractionPart
  (if (== TraceComponent _staticmeshcomponent4)
    (`/Engine/EditorBlueprintResources/StandardMacros.FlipFlop`
      (:`A`
        (bind (_direction _alpha) (`Timeline|Timeline_0` :!label _label)
          (:`Update`
            (`SceneComponent.K2_SetRelativeLocation` _staticmeshcomponent4 (`KismetMathLibrary.VLerp` (68.162262 42.63739 59.002033) (68.162262 82.63739 59.002033) _alpha) false false))))
      (:`B`
        (goto _label :!via `Reverse`)))
    (elif (== TraceComponent _staticmeshcomponent5)
      (`/Engine/EditorBlueprintResources/StandardMacros.FlipFlop`
        (:`A`
          (bind (_direction_2 _alpha_2) (`Timeline|Timeline_1` :!label _label_2)
            (:`Update`
              (`SceneComponent.K2_SetRelativeLocation` _staticmeshcomponent5 (`KismetMathLibrary.VLerp` (68.162262 42.63739 26.901754) (68.162262 82.63739 26.901754) _alpha_2) false false))))
        (:`B`
          (goto _label_2 :!via `Reverse`))))))

(fn `UserConstructionScript`)