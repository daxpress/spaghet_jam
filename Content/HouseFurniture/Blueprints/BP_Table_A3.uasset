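; BP_Table_A3 is an interactive table with two moving parts that slide out and back along local Y.
; FurnitureTrace prints a "Press E" prompt.
; FurnitureAction matches the traced component to StaticMeshComponent0 or StaticMeshComponent1, and each has its own FlipFlop that plays or reverses a timeline.
; Each timeline lerps its mesh's relative location between two hardcoded positions, without sweeping.
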(event `/Game/HouseFurniture/Blueprints/Character/BP_Demo_Interface.FurnitureTrace`
  ;[1 1 1] DebugInfo
  (`KismetSystemLibrary.PrintText` "Press E" true false (struct :`R` 1.0 :`G` 1.0 :`B` 1.0 :`A` 1.0) 0.0))

(event `/Game/HouseFurniture/Blueprints/Character/BP_Demo_Interface.FurnitureAction`
  (params (TraceComponent :type "SceneComponent Object Reference"))
  (bind _staticmeshcomponent0 (`self.StaticMeshComponent0`))
  (bind _staticmeshcomponent1 (`self.StaticMeshComponent1`))
  ;[1 1 1] InteractionPart
  (if (== TraceComponent _staticmeshcomponent1)
    (`/Engine/EditorBlueprintResources/StandardMacros.FlipFlop`
      (:`A`
        (bind (_direction _alpha) (`Timeline|Timeline_0` :!label _label)
          (:`Update`
            (`SceneComponent.K2_SetRelativeLocation` _staticmeshcomponent1 (`KismetMathLibrary.VLerp` (-36.021614 14.188148 72.9245) (-36.021614 34.188148 72.9245) _alpha) false false))))
      (:`B`
        (goto _label :!via `Reverse`)))
    (elif (== TraceComponent _staticmeshcomponent0)
      (`/Engine/EditorBlueprintResources/StandardMacros.FlipFlop`
        (:`A`
          (bind (_direction_2 _alpha_2) (`Timeline|Timeline_1` :!label _label_2)
            (:`Update`
              (`SceneComponent.K2_SetRelativeLocation` _staticmeshcomponent0 (`KismetMathLibrary.VLerp` (36.509773 14.188164 72.9245) (36.509773 34.188148 72.9245) _alpha_2) false false))))
        (:`B`
          (goto _label_2 :!via `Reverse`))))))

(fn `UserConstructionScript`)