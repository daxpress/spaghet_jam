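; BP_ChildBed_A1 is an interactive child's bed with two parts that slide out and back on player interaction.
; FurnitureTrace prints a "Press E" debug prompt.
; FurnitureAction checks which mesh component was traced, then uses that component's own FlipFlop to play or reverse its timeline.
; Each timeline lerps the mesh's relative location along Y between hardcoded closed and open positions, without sweep.
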(event `/Game/HouseFurniture/Blueprints/Character/BP_Demo_Interface.FurnitureTrace`
  ;[1 1 1] DebugInfo
  (`KismetSystemLibrary.PrintText` "Press E" true false (struct :`R` 1.0 :`G` 1.0 :`B` 1.0 :`A` 1.0) 0.0))

(event `/Game/HouseFurniture/Blueprints/Character/BP_Demo_Interface.FurnitureAction`
  (params (TraceComponent :type "SceneComponent Object Reference"))
  (bind _staticmeshcomponent1 (`self.StaticMeshComponent1`))
  (bind _staticmeshcomponent2 (`self.StaticMeshComponent2`))
  ;[1 1 1] InteractionPart
  (if (== TraceComponent _staticmeshcomponent1)
    (`/Engine/EditorBlueprintResources/StandardMacros.FlipFlop`
      (:`A`
        (bind (_direction _alpha) (`Timeline|Timeline_0` :!label _label)
          (:`Update`
            (`SceneComponent.K2_SetRelativeLocation` _staticmeshcomponent1 (`KismetMathLibrary.VLerp` (43.497124 -39.051018 0.000336) (43.497124 -89.051018 0.000336) _alpha) false false))))
      (:`B`
        (goto _label :!via `Reverse`)))
    (elif (== TraceComponent _staticmeshcomponent2)
      (`/Engine/EditorBlueprintResources/StandardMacros.FlipFlop`
        (:`A`
          (bind (_direction_2 _alpha_2) (`Timeline|Timeline_1` :!label _label_2)
            (:`Update`
              (`SceneComponent.K2_SetRelativeLocation` _staticmeshcomponent2 (`KismetMathLibrary.VLerp` (-49.128971 -39.051018 0.000336) (-49.128971 -89.051018 0.000336) _alpha_2) false false))))
        (:`B`
          (goto _label_2 :!via `Reverse`))))))

(fn `UserConstructionScript`)