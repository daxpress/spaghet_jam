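; BP_Cabinet_C1 is an interactive furniture cabinet with two hinged doors and four sliding drawers that the player opens and closes.
; A FurnitureTrace event prints a "Press E" prompt, and FurnitureAction checks which mesh component was traced.
; Each part has its own FlipFlop that plays or reverses a timeline, lerping door yaw rotation or drawer position along local Y.
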(event `self.FurnitureTrace`
  ;[1 1 1] DebugInfo
  (`KismetSystemLibrary.PrintText` "Press E" true false (struct :`R` 1.0 :`G` 1.0 :`B` 1.0 :`A` 1.0) 0.0))

(event `self.FurnitureAction`
  (params (TraceComponent :type "SceneComponent Object Reference"))
  (bind _staticmeshcomponent6 (`self.StaticMeshComponent6`))
  (bind _staticmeshcomponent2 (`self.StaticMeshComponent2`))
  (bind _staticmeshcomponent3 (`self.StaticMeshComponent3`))
  (bind _staticmeshcomponent1 (`self.StaticMeshComponent1`))
  (bind _staticmeshcomponent4 (`self.StaticMeshComponent4`))
  (bind _staticmeshcomponent5 (`self.StaticMeshComponent5`))
  ;[1 1 1] InteractionPart
  (if (== TraceComponent _staticmeshcomponent1)
    (`/Engine/EditorBlueprintResources/StandardMacros.FlipFlop`
      (:`A`
        (bind (_direction _alpha) (`Timeline|Timeline_0` :!label _label)
          (:`Update`
            (`SceneComponent.K2_SetRelativeRotation` _staticmeshcomponent1 (`KismetMathLibrary.RLerp` (struct) (struct :`Yaw` -90.0) _alpha) false false))))
      (:`B`
        (goto _label :!via `Reverse`)))
    (elif (== TraceComponent _staticmeshcomponent2)
      (`/Engine/EditorBlueprintResources/StandardMacros.FlipFlop`
        (:`A`
          (bind (_direction_2 _alpha_2) (`Timeline|Timeline_1` :!label _label_2)
            (:`Update`
              (`SceneComponent.K2_SetRelativeRotation` _staticmeshcomponent2 (`KismetMathLibrary.RLerp` (struct) (struct :`Yaw` 90.0) _alpha_2) false false))))
        (:`B`
          (goto _label_2 :!via `Reverse`)))
      (elif (== TraceComponent _staticmeshcomponent3)
        (`/Engine/EditorBlueprintResources/StandardMacros.FlipFlop`
          (:`A`
            (bind (_direction_3 _alpha_3) (`Timeline|Timeline_2` :!label _label_3)
              (:`Update`
                (`SceneComponent.K2_SetRelativeLocation` _staticmeshcomponent3 (`KismetMathLibrary.VLerp` (0.766682 22.999462 16.309891) (0.766682 47.999462 16.309891) _alpha_3) false false))))
          (:`B`
            (goto _label_3 :!via `Reverse`)))
        (elif (== TraceComponent _staticmeshcomponent4)
          (`/Engine/EditorBlueprintResources/StandardMacros.FlipFlop`
            (:`A`
              (bind (_direction_4 _alpha_4) (`Timeline|Timeline_3` :!label _label_4)
                (:`Update`
                  (`SceneComponent.K2_SetRelativeLocation` _staticmeshcomponent4 (`KismetMathLibrary.VLerp` (0.766682 22.999462 34.33057) (0.766682 47.999462 34.33057) _alpha_4) false false))))
            (:`B`
              (goto _label_4 :!via `Reverse`)))
          (elif (== TraceComponent _staticmeshcomponent5)
            (`/Engine/EditorBlueprintResources/StandardMacros.FlipFlop`
              (:`A`
                (bind (_direction_5 _alpha_5) (`Timeline|Timeline_4` :!label _label_5)
                  (:`Update`
                    (`SceneComponent.K2_SetRelativeLocation` _staticmeshcomponent5 (`KismetMathLibrary.VLerp` (0.766682 22.999462 52.397987) (0.766682 47.999462 52.397987) _alpha_5) false false))))
              (:`B`
                (goto _label_5 :!via `Reverse`)))
            (elif (== TraceComponent _staticmeshcomponent6)
              (`/Engine/EditorBlueprintResources/StandardMacros.FlipFlop`
                (:`A`
                  (bind (_direction_6 _alpha_6) (`Timeline|Timeline_5` :!label _label_6)
                    (:`Update`
                      (`SceneComponent.K2_SetRelativeLocation` _staticmeshcomponent6 (`KismetMathLibrary.VLerp` (0.766682 22.999462 70.222336) (0.766682 47.999462 70.222336) _alpha_6) false false))))
                (:`B`
                  (goto _label_6 :!via `Reverse`))))))))))

(fn `UserConstructionScript`)