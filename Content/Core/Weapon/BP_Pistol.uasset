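; Pistol weapon that can be picked up through interaction, equipped, fired and reloaded.
; Primary use fires a hitscan trace from the user's eye view with random spread, applying damage on hit and leaving persistent debug lines.
; Tertiary use refills from inventory ammo, which is consumed before the CanReload check.
; Fire and reload montages lock both actions until completion, and equip events toggle mesh visibility.
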(event `/Game/Core/EquippableItem/BPI_EquippableItem.PrimaryUse`
  (params (User :type "/Game/Core/BP_MainCharacter Object Reference"))
  (bind (_outlocation _outrotation) (`self.GetActorEyesViewPoint` User))
  (bind _returnvalue (`self.GetOwner`))
  (bind (_hitresult_bblockinghit _hitresult_binitialoverlap _hitresult_time _hitresult_distance _hitresult_location _hitresult_impactpoint _hitresult_normal _hitresult_impactnormal _hitresult_physmat _hitresult_hitactor) (`GameplayStatics.BreakHitResult` (`self.HitResult`)))
  (bind (_spreaderrorpitch_x _spreaderrorpitch_y) (`KismetMathLibrary.BreakVector2D` (`self.SpreadErrorPitch`)))
  (bind (_spreaderroryaw_x _spreaderroryaw_y) (`KismetMathLibrary.BreakVector2D` (`self.SpreadErrorYaw`)))
  (if (and (`self.bCanShoot`) (> (`self.CurrentAmmo`) 0))
    (`/Engine/EditorBlueprintResources/StandardMacros.DecrementInt` (`self.CurrentAmmo`)
      (:`  `
        (bind _outhit (`KismetSystemLibrary.LineTraceSingle` _outlocation (+ _outlocation (* (`KismetMathLibrary.Conv_RotatorToVector` (`KismetMathLibrary.MakeRotator` (.roll _outrotation) (+ (.pitch _outrotation) (`KismetMathLibrary.RandomFloatInRange` _spreaderrorpitch_x _spreaderrorpitch_y)) (+ (.yaw _outrotation) (`KismetMathLibrary.RandomFloatInRange` _spreaderroryaw_x _spreaderroryaw_y)))) (`self.Range`))) "TraceTypeQuery1" true (`|MakeArray` User self :!type "Actor Object Reference") "Persistent"))
        (set `self.HitResult` _outhit)
        (`|PlayMontage` (`self.Body`) "/Game/Animations/Pistol/AM_Pistol_Fire_01.AM_Pistol_Fire_01"
          (:`then`
            (set `self.bCanShoot` false)
            (set `self.bCanReload` false)
            (if _hitresult_bblockinghit
              (`GameplayStatics.ApplyDamage` _hitresult_hitactor (`self.Damage`) (`self.GetInstigatorController` _returnvalue) _returnvalue)))
          (:`OnCompleted`
            (set `self.bCanShoot` true)
            (set `self.bCanReload` true)))))))

(event `/Game/Core/EquippableItem/BPI_EquippableItem.TertiaryUse`
  (params (User :type "/Game/Core/BP_MainCharacter Object Reference"))
  (bind _returnvalue (`InventoryComponent.ConsumeFromInventory` (`/Game/Core/BP_MainCharacter.Inventory` User) (`self.AmmoType`) (- (`self.MaxAmmo`) (`self.CurrentAmmo`))))
  (set `self.AmmoFromInventory` _returnvalue)
  (if (and (`self.bCanReload`) (> _returnvalue 0))
    (`|PlayMontage` (`self.Body`) "/Game/Animations/Pistol/AM_Pistol_ReloadPartial.AM_Pistol_ReloadPartial"
      (:`then`
        (set `self.bCanShoot` false)
        (set `self.bCanReload` false))
      (:`OnCompleted`
        (set `self.CurrentAmmo` (+ (`self.CurrentAmmo`) (`self.AmmoFromInventory`)))
        (set `self.bCanShoot` true)
        (set `self.bCanReload` true)))))

(event `/Game/Core/Interaction/BPI_Interactable.Interact`
  (params (Interactor :type "/Game/Core/BP_MainCharacter Object Reference"))
  (`self.SetOwner` Interactor)
  (set `/Game/Core/BP_MainCharacter.Pistol` self Interactor)
  (`/Game/Core/BP_MainCharacter.EquipItem` Interactor self))

(event `/Game/Core/EquippableItem/BPI_EquippableItem.OnEquipment`
  (`PrimitiveComponent.SetCollisionEnabled` (`self.InteractionVolume`) "NoCollision")
  (`SceneComponent.SetVisibility` (`self.Body`) true true))

(event `/Game/Core/EquippableItem/BPI_EquippableItem.OnUnequip`
  (`SceneComponent.SetVisibility` (`self.Body`) false true))

(event `self.ReceiveBeginPlay`
  (set `self.CurrentAmmo` (`self.MaxAmmo`)))

(fn `GetEquippedRelativeLocation`
  (returns (RelativeLocation :type "Transform Structure"))
  (return (`self.EquippedRelativeLocation`)))

(fn `UserConstructionScript`)