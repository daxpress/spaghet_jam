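; Equippable hitscan firearm that fires from the user's camera, reloads from their inventory and reports ammo counts through an update event.
; Primary use sphere-traces along a randomly spread aim with persistent debug drawing, applies point damage and plays camera shake.
; Tertiary use consumes inventory ammo before checking reload eligibility, then refills the magazine when the montage completes.
; Pistol montages gate firing and reloading, while equip events toggle mesh visibility.
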(event `/Game/Core/EquippableItem/BPI_EquippableItem.PrimaryUse`
  (params (User :type "/Game/Core/BP_MainCharacter Object Reference"))
  (bind _returnvalue (`self.GetOwner`))
  (bind (_hitresult_bblockinghit _hitresult_binitialoverlap _hitresult_time _hitresult_distance _hitresult_location _hitresult_impactpoint _hitresult_normal _hitresult_impactnormal _hitresult_physmat _hitresult_hitactor) (`GameplayStatics.BreakHitResult` (`self.HitResult`)))
  (bind (_spreaderrorpitch_x _spreaderrorpitch_y) (`KismetMathLibrary.BreakVector2D` (`self.SpreadErrorPitch`)))
  (bind (_spreaderroryaw_x _spreaderroryaw_y) (`KismetMathLibrary.BreakVector2D` (`self.SpreadErrorYaw`)))
  (bind (_returnvalue_location _returnvalue_rotation) (`KismetMathLibrary.BreakTransform` (`SceneComponent.K2_GetComponentToWorld` (`/Game/Core/BP_MainCharacter.Camera` User))))
  (if (and (`self.bCanShoot`) (> (`self.CurrentAmmo`) 0))
    (`/Engine/EditorBlueprintResources/StandardMacros.DecrementInt` (`self.CurrentAmmo`)
      (:`  `
        (bind _outhit (`KismetSystemLibrary.SphereTraceSingle` _returnvalue_location (+ _returnvalue_location (* (`KismetMathLibrary.Conv_RotatorToVector` (`KismetMathLibrary.MakeRotator` (.roll _returnvalue_rotation) (+ (.pitch _returnvalue_rotation) (`KismetMathLibrary.RandomFloatInRange` _spreaderrorpitch_x _spreaderrorpitch_y)) (+ (.yaw _returnvalue_rotation) (`KismetMathLibrary.RandomFloatInRange` _spreaderroryaw_x _spreaderroryaw_y)))) (`self.Range`))) (`self.BulletRadius`) "TraceTypeQuery2" true (`|MakeArray` User self :!type "Actor Object Reference") "Persistent"))
        (set `self.HitResult` _outhit)
        (`|PlayMontage` (`self.Body`) "/Game/Animations/Pistol/AM_Pistol_Fire_01.AM_Pistol_Fire_01"
          (:`then`
            (set `self.bCanShoot` false)
            (set `self.bCanReload` false)
            (`PlayerController.ClientStartCameraShake` :`self` (`GameplayStatics.GetPlayerController` 0) :`Shake` "/Game/Core/CameraShakes/LCS_Shoot.LCS_Shoot_C")
            (bind _returnvalue_2 (`InventoryComponent.GetQuantity` (`/Game/Core/BP_MainCharacter.Inventory` User) (`self.AmmoType`)))
            (`self.On Weapon Ammo Update` (make `IntPoint` (`self.CurrentAmmo`) (`self.MaxAmmo`)) _returnvalue_2)
            (if _hitresult_bblockinghit
              (`GameplayStatics.ApplyPointDamage` _hitresult_hitactor (`self.Damage`) _hitresult_normal (`self.HitResult`) (`self.GetInstigatorController` _returnvalue) _returnvalue "/Game/Core/Weapon/BP_Damage.BP_Damage_C")))
          (:`OnCompleted`
            (set `self.bCanShoot` true)
            (set `self.bCanReload` true)))))))

(event `/Game/Core/EquippableItem/BPI_EquippableItem.TertiaryUse`
  (params (User :type "/Game/Core/BP_MainCharacter Object Reference"))
  (bind _ammotype (`self.AmmoType`))
  (bind _inventory (`/Game/Core/BP_MainCharacter.Inventory` User))
  (bind _returnvalue (`InventoryComponent.ConsumeFromInventory` _inventory _ammotype (- (`self.MaxAmmo`) (`self.CurrentAmmo`))))
  (set `self.AmmoFromInventory` _returnvalue)
  (if (and (`self.bCanReload`) (> _returnvalue 0))
    (`|PlayMontage` (`self.Body`) (select `bool` (> (`self.CurrentAmmo`) 0) :`false` "/Game/Animations/Pistol/AM_Pistol_ReloadEmpty.AM_Pistol_ReloadEmpty" :`true` "/Game/Animations/Pistol/AM_Pistol_ReloadPartial.AM_Pistol_ReloadPartial" :!type "AnimMontage Object Reference")
      (:`then`
        (set `self.bCanShoot` false)
        (set `self.bCanReload` false))
      (:`OnCompleted`
        (set `self.CurrentAmmo` (+ (`self.CurrentAmmo`) (`self.AmmoFromInventory`)))
        (set `self.bCanShoot` true)
        (set `self.bCanReload` true)
        (bind _returnvalue_2 (`InventoryComponent.GetQuantity` _inventory _ammotype))
        (`self.On Weapon Ammo Update` (make `IntPoint` (`self.CurrentAmmo`) (`self.MaxAmmo`)) _returnvalue_2)))))

(event `/Game/Core/EquippableItem/BPI_EquippableItem.OnEquipment`
  (`SceneComponent.SetVisibility` (`self.Body`) true true)
  (`self.On Weapon Ammo Update` (make `IntPoint` (`self.CurrentAmmo`) (`self.MaxAmmo`)) (`self.AmmoFromInventory`)))

(event `/Game/Core/EquippableItem/BPI_EquippableItem.OnUnequip`
  (`SceneComponent.SetVisibility` (`self.Body`) false true))

(event `self.ReceiveBeginPlay`
  (set `self.CurrentAmmo` (`self.MaxAmmo`)))

(fn `GetEquippedRelativeLocation`
  (returns (RelativeLocation :type "Transform Structure"))
  (return (`self.EquippedRelativeLocation`)))

(fn `UserConstructionScript`)