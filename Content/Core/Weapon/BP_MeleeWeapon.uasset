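; Base-style melee weapon (a baton, per its sound names) that shows or hides itself on equip and unequip.
; Primary use sphere-traces from the user's camera along its forward vector and plays the attack montage on the user's mesh.
; Point damage and a hit sound apply as the montage starts, not on a swing notify.
; Attacks stay locked until the montage completes and a delay elapses.
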(event `/Game/Core/EquippableItem/BPI_EquippableItem.OnUnequip`
  (`SceneComponent.SetVisibility` (`self.DefaultSceneRoot`) false true))

(event `/Game/Core/EquippableItem/BPI_EquippableItem.OnEquipment`
  (`SceneComponent.SetVisibility` (`self.DefaultSceneRoot`) true true)
  (`GameplayStatics.PlaySound2D` "/Game/Audio/MC/ChangeToManganello.ChangeToManganello" 1.0 1.0 0.0 null null))

(event `/Game/Core/EquippableItem/BPI_EquippableItem.PrimaryUse`
  (params (User :type "/Game/Core/BP_MainCharacter Object Reference"))
  (bind (_hitresult_bblockinghit _hitresult_binitialoverlap _hitresult_time _hitresult_distance _hitresult_location _hitresult_impactpoint _hitresult_normal _hitresult_impactnormal _hitresult_physmat _hitresult_hitactor) (`GameplayStatics.BreakHitResult` (`self.HitResult`)))
  (bind _user (`self.User`))
  (if (`self.bCanAttack`)
    (bind _output_get (set `self.User` User))
    (bind (_returnvalue_location _returnvalue_rotation) (`KismetMathLibrary.BreakTransform` (`SceneComponent.K2_GetComponentToWorld` (`/Game/Core/BP_MainCharacter.Camera` _output_get))))
    (bind _outhit (`KismetSystemLibrary.SphereTraceSingle` _returnvalue_location (+ _returnvalue_location (* (`KismetMathLibrary.Conv_RotatorToVector` _returnvalue_rotation) (`self.Range`))) 2.0 "TraceTypeQuery2" true (`|MakeArray` User self :!type "Actor Object Reference")))
    (set `self.HitResult` _outhit)
    (`|PlayMontage` (`Character.Mesh` (`self.User`)) "/Game/Animations/Character/AM_MeleeAttack01.AM_MeleeAttack01"
      (:`then`
        (set `self.bCanAttack` false)
        (if _hitresult_bblockinghit
          (`GameplayStatics.ApplyPointDamage` _hitresult_hitactor (`self.MeleeDamage`) _hitresult_normal (`self.HitResult`) (`Pawn.GetController` _user) _user "/Game/Core/Weapon/BP_Damage.BP_Damage_C")
          (`GameplayStatics.PlaySoundAtLocation` "/Game/Audio/Enemies/Aliens/Alien_HitManganello.Alien_HitManganello" _hitresult_location (struct) 1.0 1.0 0.0 null null null null)))
      (:`OnCompleted`
        (`KismetSystemLibrary.Delay` (`self.TimeBetweenAttacks`))
        (set `self.bCanAttack` true)))))

(fn `GetEquippedRelativeLocation`
  (returns (RelativeLocation :type "Transform Structure"))
  (return))

(fn `UserConstructionScript`)