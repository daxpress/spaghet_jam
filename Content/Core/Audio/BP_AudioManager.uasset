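; Audio manager that drives adaptive audio and bell cues from enemy activation and deaths.
; On BeginPlay it binds to every BP_Enemy, switching the Audio component's Status parameter on activation and again when the active count reaches zero.
; Early kills trigger delayed bells with a matching subtitle widget, also playable as a starting cue.
; From the sixth kill onward, it sets the kill index and fires the End trigger instead.
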(event `self.ReceiveBeginPlay`
  (bind _outactors (`GameplayStatics.GetAllActorsOfClass` "/Game/Core/Enemy/BP_Enemy.BP_Enemy_C"))
  (bind _output_get (set `self.Enemies` _outactors))
  (for _array_element _output_get
    (add `/Game/Core/Enemy/BP_Enemy.EnemyActivated` _array_element (`|CreateDelegate` :!event `OnEnemyActivated`))
    (add `/Game/Core/Enemy/BP_Enemy.EnemyDeath` _array_element (`|CreateDelegate` :!event `OnEnemyDeath`))))

(event `OnEnemyActivated`
  (`/Engine/EditorBlueprintResources/StandardMacros.IncrementInt` (`self.ActiveEnemies`)
    (:`  `
      (`AudioParameterControllerInterface.SetIntParameter` (`self.Audio`) "Status" 1))))

(event `OnEnemyDeath`
  (bind _audio (`self.Audio`))
  (`|ExecutionSequence`
    (:`then_0`
      (bind _result (`/Engine/EditorBlueprintResources/StandardMacros.DecrementInt` (`self.ActiveEnemies`))
        (:`  `
          (bind _output_get (set `self.ActiveEnemies` (`KismetMathLibrary.Clamp` _result 0 2)))
          (if (== _output_get 0)
            (`AudioParameterControllerInterface.SetIntParameter` (`self.Audio`) "Status" 2)))))
    (:`then_1`
      (bind _result_2 (`/Engine/EditorBlueprintResources/StandardMacros.IncrementInt` (`self.DeadEnemies`))
        (:`  `
          (if (< _result_2 6)
            (`KismetSystemLibrary.Delay` (`self.AfterKillBellsDelay`))
            (`self.PlayBells`)
            (else
              (`AudioParameterControllerInterface.SetIntParameter` _audio "IndexKill" 1)
              (`AudioParameterControllerInterface.SetTriggerParameter` _audio "End"))))))))

(event `PlayStartingBells`
  (`self.PlayBells`))

(fn `PlayBells`
  (bind _deadenemies (`self.DeadEnemies`))
  (`AudioParameterControllerInterface.SetIntParameter` (`self.Bells`) "EnemiesKilled" _deadenemies)
  (`AudioComponent.Play` (`self.Bells`) 0.0)
  (bind _returnvalue (`|CreateWidget` "/Game/Core/UI/Widget_Subtitle.Widget_Subtitle_C" (`GameplayStatics.GetPlayerController` 0) (select `int` _deadenemies :`0` "/Game/Audio/Ambience/Bells/01_Bells6_IniziamoBene.01_Bells6_IniziamoBene" :`1` "/Game/Audio/Ambience/Bells/02_Bells5_Ma_mmm.02_Bells5_Ma_mmm" :`2` "/Game/Audio/Ambience/Bells/03_Bells4_AhCheSchifo.03_Bells4_AhCheSchifo" :`3` "/Game/Audio/Ambience/Bells/04_Bells3.04_Bells3" :`4` "/Game/Audio/Ambience/Bells/05_Bells2.05_Bells2" :`5` "/Game/Audio/Ambience/Bells/06_Bell_1_mmm.06_Bell_1_mmm" :!type "SoundWave Object Reference")))
  (`UserWidget.AddToPlayerScreen` _returnvalue 1))

(fn `UserConstructionScript`)