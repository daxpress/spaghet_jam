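; BP_Medkit is a health pickup that heals the main character.
; On overlap it casts the other actor to BP_MainCharacter and calls its own Interact event only if that character's Health is below MaxHealth.
; Interact heals the interactor by HealAmmount, plays a 2D pickup sound and destroys the medkit, with no health check of its own.
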(event `/Game/Core/Interaction/BPI_Interactable.Interact`
  (params (Interactor :type "/Game/Core/BP_MainCharacter Object Reference"))
  (`/Game/Core/BP_MainCharacter.Heal` Interactor (`self.HealAmmount`))
  (`GameplayStatics.PlaySound2D` "/Game/Audio/MC/MC_PickUp_Object.MC_PickUp_Object" 1.0 1.0 0.0 null null)
  (`self.K2_DestroyActor`))

(event `self.ReceiveActorBeginOverlap`
  (params (OtherActor :type "Actor Object Reference"))
  (bind _asbp_main_character (cast `/Game/Core/BP_MainCharacter` OtherActor))
  (if (< (`/Game/Core/BP_MainCharacter.Health` _asbp_main_character) (`/Game/Core/BP_MainCharacter.MaxHealth` _asbp_main_character))
    (`/Game/Core/Interaction/BPI_Interactable.Interact` _asbp_main_character)))

(fn `UserConstructionScript`)