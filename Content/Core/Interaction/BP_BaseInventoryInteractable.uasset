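; Base inventory pickup actor that grants pistol ammo to whoever interacts with it, then destroys itself.
; The Interact event adds to the interactor's PistolAmmo an amount taken from RangeValue.
; RangeValue works as a min/max pair: equal bounds give a fixed amount, otherwise a random integer within the truncated bounds is used.
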(event `/Game/Core/Interaction/BPI_Interactable.Interact`
  (params (Interactor :type "/Game/Core/BP_MainCharacter Object Reference"))
  (bind (_rangevalue_x _rangevalue_y) (`KismetMathLibrary.BreakVector2D` (`self.RangeValue`)))
  (set `/Game/Core/BP_MainCharacter.PistolAmmo` (+ (`/Game/Core/BP_MainCharacter.PistolAmmo` Interactor) (select `bool` (== _rangevalue_x _rangevalue_y) :`false` (`KismetMathLibrary.RandomIntegerInRange` (`KismetMathLibrary.FTrunc` _rangevalue_x) (`KismetMathLibrary.FTrunc` _rangevalue_y)) :`true` (`KismetMathLibrary.FTrunc` _rangevalue_y))) Interactor)
  (`self.K2_DestroyActor` self))

(fn `UserConstructionScript`)