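; Player character Blueprint for a first-person combat game with health, stamina-limited sprint, a flashlight and a kill-count victory.
; Enhanced Input drives movement and actions, with spawned pistol and melee weapons swapped through a montage and used via BPI_EquippableItem.
; Tick updates stamina, camera-shake head bob and footstep audio, whose tempo follows sprint state and terrain comes from downward surface traces.
; Death shows game over; victory plays a sequence, then loads the main menu.
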(event `PlaySound_Ambience`
  (`GameplayStatics.PlaySound2D` "/Game/Audio/Ambience/Ambience_Neutral.Ambience_Neutral" 1.0 1.0 0.0 null null))

(event `self.ReceiveBeginPlay`
  (set `self.BaseMovementSpeed` (`CharacterMovementComponent.MaxWalkSpeed` (`self.CharacterMovement`)))
  (set `self.Stamina` (`self.MaxStamina`))
  (`self.InitInventory`)
  (bind _asplayer_controller (cast `PlayerController` (`self.GetController`)))
  (bind _returnvalue (pcsubsystem `EnhancedInputLocalPlayerSubsystem` _asplayer_controller))
  (`/Engine/EditorBlueprintResources/StandardMacros.IsValid` _returnvalue
    (:`Is Valid`
      (`EnhancedInputSubsystemInterface.AddMappingContext` _returnvalue "/Game/Core/Input/IMC_MainCharacter.IMC_MainCharacter" 0 (struct))
      (`self.PlaySound_Ambience`)
      (`KismetSystemLibrary.K2_SetTimerDelegate` (`|CreateDelegate` :!event `TraceForMaterial`) 0.05 true true)
      (`AudioComponent.SetFloatParameter` (`self.Audio`) "BPM" (`self.WalkAudioFrequency`)))))

(event `self.K2_OnStartCrouch`
  (params (HalfHeightAdjust :type "Float (single-precision)") (ScaledHalfHeightAdjust :type "Float (single-precision)"))
  ; Movement
  ;; Crouch
  (`SceneComponent.K2_SetRelativeLocation` (`self.Camera`) (`KismetMathLibrary.MakeVector` 0.0 0.0 (- (`self.BaseEyeHeight`) HalfHeightAdjust)) false true))

(event `self.ReceiveTick`
  (params (DeltaSeconds :type "Float (single-precision)"))
  (`|ExecutionSequence`
    (:`then_0`
      (if (`self.bSprinting`)
        (if (> (`KismetMathLibrary.VSize` (`self.GetVelocity`)) 0.0)
          (bind _output_get (set `self.Stamina` (`KismetMathLibrary.FClamp` (- (`self.Stamina`) DeltaSeconds) 0.0 (`self.MaxStamina`))))
          (if (`KismetMathLibrary.NearlyEqual_FloatFloat` _output_get 0.0 0.1)
            (`self.StopSprint`))
          (else
            (`self.StopSprint`)))
        (else
          (set `self.Stamina` (`KismetMathLibrary.FClamp` (+ (`self.Stamina`) DeltaSeconds) 0.0 (`self.MaxStamina`))))))
    (:`then_1`
      (`self.Camera HeadBobbing`))
    (:`then_2`
      (if (and (`NavMovementInterface.IsMovingOnGround` (`self.CharacterMovement`)) (> (`KismetMathLibrary.VSize` (`self.GetVelocity`)) 0.0))
        (if (not (`AudioComponent.IsPlaying` (`self.Audio`)))
          (`AudioComponent.Play` (`self.Audio`) 0.0))
        (elif (`AudioComponent.IsPlaying` (`self.Audio`))
          (`AudioComponent.Stop` (`self.Audio`)))))))

(event `self.K2_OnEndCrouch`
  (params (HalfHeightAdjust :type "Float (single-precision)") (ScaledHalfHeightAdjust :type "Float (single-precision)"))
  ; Movement
  ;; Crouch
  (`SceneComponent.K2_SetRelativeLocation` (`self.Camera`) (`KismetMathLibrary.MakeVector` 0.0 0.0 (`self.BaseEyeHeight`)) false true))

(event `StartSprint`
  ; Movement
  ;; Sprint
  (if (and (> (`self.Stamina`) (* (`self.MaxStamina`) 0.3)) (> (`KismetMathLibrary.VSize` (`self.GetVelocity`)) 0.0))
    (set `self.bSprinting` true)
    (set `CharacterMovementComponent.MaxWalkSpeed` (+ (`self.BaseMovementSpeed`) (`self.SprintSpeed`)) (`self.CharacterMovement`))
    (`AudioComponent.SetFloatParameter` (`self.Audio`) "BPM" (`self.SprintAudioFrequency`))))

(event `self.ReceiveAnyDamage`
  (params (Damage :type "Float (single-precision)") (DamageType :type "DamageType Object Reference") (InstigatedBy :type "Controller Object Reference") (DamageCauser :type "Actor Object Reference"))
  (bind _returnvalue (`GameplayStatics.GetPlayerController` 0))
  (if (> (`self.Health`) 0.0)
    (bind _output_get (set `self.Health` (- (`self.Health`) Damage)))
    (`PlayerController.ClientStartCameraShake` :`self` (`GameplayStatics.GetPlayerController` 0) :`Shake` "/Game/Core/CameraShakes/LCS_Hit.LCS_Hit_C")
    (if (<= (`self.Health`) 0.0)
      ; Death
      (`|ExecutionSequence`
        (:`then_0`
          (`self.DisableInput` _returnvalue)
          (bind _returnvalue_2 (`|CreateWidget` "/Game/Core/UI/Widget_GameOver.Widget_GameOver_C" _returnvalue))
          (`UserWidget.AddToPlayerScreen` _returnvalue_2 0)
          (`KismetSystemLibrary.Delay` 1.0)
          (`GameplayStatics.SetGamePaused` true))
        (:`then_1`
          (`GameplayStatics.PlaySound2D` "/Game/Audio/MC/DEATH/MS_Death.MS_Death" 1.0 1.0 0.0 null null))))))

(event `StopSprint`
  ; Movement
  ;; Sprint
  (set `self.bSprinting` false)
  (set `CharacterMovementComponent.MaxWalkSpeed` (`self.BaseMovementSpeed`) (`self.CharacterMovement`))
  (`AudioComponent.SetFloatParameter` (`self.Audio`) "BPM" (`self.WalkAudioFrequency`)))

(event `EquipItem`
  (params (Actor :type "Actor Object Reference"))
  (if (`self.bCanSwitch`)
    (set `self.bCanSwitch` false)
    (`|PlayMontage` (`self.Mesh`) "/Game/Animations/Character/AM_Extraction.AM_Extraction"
      (:`then`
        (message `/Game/Core/EquippableItem/BPI_EquippableItem.OnUnequip` (`self.CurrentEquippedItem`))
        (bind _output_get (set `self.CurrentEquippedItem` Actor))
        (`self.On Player Equip Item` _output_get)
        (`self.K2_AttachToComponent` _output_get (`self.Mesh`) "WeaponSocket" "SnapToTarget" "SnapToTarget" "KeepRelative" true)
        (message `/Game/Core/EquippableItem/BPI_EquippableItem.OnEquipment` _output_get))
      (:`OnCompleted`
        (set `self.bCanSwitch` true :!label _label))
      (:`OnBlendOut`
        (goto _label)))))

(event `TraceForMaterial`
  (bind _returnvalue (`self.K2_GetActorLocation`))
  (bind _audio (`self.Audio`))
  (bind _outhit (`KismetSystemLibrary.LineTraceSingle` _returnvalue (+ _returnvalue (* (`KismetMathLibrary.NegateVector` (`self.GetActorUpVector`)) 100.0)) "TraceTypeQuery1"))
  (`/Engine/EditorBlueprintResources/StandardMacros.IsValid` (`.PhysMat` (`GameplayStatics.BreakHitResult` _outhit))
    (:`Is Valid`
      (`/Engine/EditorBlueprintResources/StandardMacros.IsValid` _audio
        (:`Is Valid`
          (`AudioParameterControllerInterface.SetIntParameter` _audio "Terrain" (select `EPhysicalSurface` (`PhysicalMaterial.SurfaceType` (`.PhysMat` (`GameplayStatics.BreakHitResult` _outhit))) :`SurfaceType1` 1 :`SurfaceType2` 2 :`SurfaceType3` 3)))))
    (:`Is Not Valid`
      (`AudioParameterControllerInterface.SetIntParameter` (`self.Audio`) "Terrain" 0))))

(event `WinImpl`
  (bind _asplayer_controller (cast `PlayerController` (`self.GetController`)))
  (`EnhancedInputSubsystemInterface.RemoveMappingContext` (pcsubsystem `EnhancedInputLocalPlayerSubsystem` _asplayer_controller) "/Game/Core/Input/IMC_MainCharacter.IMC_MainCharacter" (struct))
  (`KismetSystemLibrary.Delay` 3.0)
  (`PlayerController.ClientStopCameraShake` (`GameplayStatics.GetPlayerController` 0) "/Game/Core/CameraShakes/LCS_Walk.LCS_Walk_C" true)
  (`PlayerController.ClientStopCameraShake` (`GameplayStatics.GetPlayerController` 0) "/Game/Core/CameraShakes/LCS_Idle.LCS_Idle_C" true)
  (`PlayerController.ClientStopCameraShake` (`GameplayStatics.GetPlayerController` 0) "/Game/Core/CameraShakes/LCS_Sprint.LCS_Sprint_C" true)
  (bind _ashud_gameplay (cast `/Game/Core/UI/HUD_Gameplay` (`PlayerController.GetHUD` (`GameplayStatics.GetPlayerController` 0))))
  (`/Game/Core/UI/HUD_Gameplay.RemoveHud` _ashud_gameplay)
  (bind (_outactor _returnvalue) (`LevelSequencePlayer.CreateLevelSequencePlayer` "/Game/Animations/Endgame/WinSequence.WinSequence"))
  (`MovieSceneSequencePlayer.Play` _returnvalue)
  (add `MovieSceneSequencePlayer.OnFinished` _returnvalue (delegate `BackToMenu`)))

(event `BackToMenu`
  (`GameplayStatics.OpenLevelBySoftObjectPtr` "/Game/Core/UI/MainMenu/L_MainMenu.L_MainMenu"))

(event `EnhancedInput|/Game/Core/Input/IA_SelectPistol`
  (params (ActionValue :type Boolean) (ElapsedSeconds :type "Float (double-precision)") (TriggeredSeconds :type "Float (double-precision)") (InputAction :type "InputAction Object Reference" :default "/Game/Core/Input/IA_SelectPistol.IA_SelectPistol"))
  ; Weapon Selection
  (:`Triggered`
    (if (not (== (`self.CurrentEquippedItem`) (`self.Pistol`)))
      (`self.EquipItem` (`self.Pistol`)))))

(event `EnhancedInput|/Game/Core/Input/IA_MovementForward`
  (params (ActionValue :type "Float (double-precision)") (ElapsedSeconds :type "Float (double-precision)") (TriggeredSeconds :type "Float (double-precision)") (InputAction :type "InputAction Object Reference" :default "/Game/Core/Input/IA_MovementForward.IA_MovementForward"))
  ; Movement
  (:`Triggered`
    (`self.AddMovementInput` (`self.GetActorForwardVector`) ActionValue)))

(event `EnhancedInput|/Game/Core/Input/IA_SelectMelee`
  (params (ActionValue :type Boolean) (ElapsedSeconds :type "Float (double-precision)") (TriggeredSeconds :type "Float (double-precision)") (InputAction :type "InputAction Object Reference" :default "/Game/Core/Input/IA_SelectMelee.IA_SelectMelee"))
  ; Weapon Selection
  (:`Triggered`
    (if (not (== (`self.CurrentEquippedItem`) (`self.Melee`)))
      (`self.EquipItem` (`self.Melee`)))))

(event `EnhancedInput|/Game/Core/Input/IA_MovementRight`
  (params (ActionValue :type "Float (double-precision)") (ElapsedSeconds :type "Float (double-precision)") (TriggeredSeconds :type "Float (double-precision)") (InputAction :type "InputAction Object Reference" :default "/Game/Core/Input/IA_MovementRight.IA_MovementRight"))
  ; Movement
  (:`Triggered`
    (`self.AddMovementInput` (`self.GetActorRightVector`) ActionValue)))

(event `EnhancedInput|/Game/Core/Input/IA_Pause`
  (params (ActionValue :type Boolean) (ElapsedSeconds :type "Float (double-precision)") (TriggeredSeconds :type "Float (double-precision)") (InputAction :type "InputAction Object Reference" :default "/Game/Core/Input/IA_Pause.IA_Pause"))
  (:`Triggered`
    (`GameplayStatics.SetGamePaused` true)
    (bind _returnvalue (`|CreateWidget` "/Game/Core/UI/Widget_Pause.Widget_Pause_C" (`GameplayStatics.GetPlayerController` 0)))
    (`UserWidget.AddToPlayerScreen` _returnvalue 0)))

(event `EnhancedInput|/Game/Core/Input/IA_Sprint`
  (params (ActionValue :type Boolean) (ElapsedSeconds :type "Float (double-precision)") (TriggeredSeconds :type "Float (double-precision)") (InputAction :type "InputAction Object Reference" :default "/Game/Core/Input/IA_Sprint.IA_Sprint"))
  ; Movement
  (:`Triggered`
    (if (not (`self.bSprinting`))
      (`self.StartSprint`)))
  (:`Completed`
    (`self.StopSprint`)))

(event `EnhancedInput|/Game/Core/Input/IA_Aim`
  (params (ActionValue :type "Vector2D Structure") (ElapsedSeconds :type "Float (double-precision)") (TriggeredSeconds :type "Float (double-precision)") (InputAction :type "InputAction Object Reference" :default "/Game/Core/Input/IA_Aim.IA_Aim"))
  (:`Triggered`
    (bind _result (`/Engine/EditorBlueprintResources/StandardMacros.NegateFloat` ActionValue_Y)
      (:`  `
        (`self.AddControllerPitchInput` _result)
        (`self.AddControllerYawInput` ActionValue_X)))))

(event `EnhancedInput|/Game/Core/Input/IA_MainAction`
  (params (ActionValue :type Boolean) (ElapsedSeconds :type "Float (double-precision)") (TriggeredSeconds :type "Float (double-precision)") (InputAction :type "InputAction Object Reference" :default "/Game/Core/Input/IA_MainAction.IA_MainAction"))
  ; Actions
  (:`Triggered`
    (bind _currentequippeditem (`self.CurrentEquippedItem`)
      (:`then`
        (if (`KismetSystemLibrary.DoesImplementInterface` _currentequippeditem "/Game/Core/EquippableItem/BPI_EquippableItem.BPI_EquippableItem_C")
          (message `/Game/Core/EquippableItem/BPI_EquippableItem.PrimaryUse` (`self.CurrentEquippedItem`) self)))
      (:`else`))))

(event `EnhancedInput|/Game/Core/Input/IA_SecondaryAction`
  (params (ActionValue :type Boolean) (ElapsedSeconds :type "Float (double-precision)") (TriggeredSeconds :type "Float (double-precision)") (InputAction :type "InputAction Object Reference" :default "/Game/Core/Input/IA_SecondaryAction.IA_SecondaryAction"))
  (bind _audiotorch (`self.AudioTorch`))
  (bind _audiotorch_2 (`self.AudioTorch`))
  ; Actions
  (:`Triggered`
    (if (`SceneComponent.IsVisible` (`self.SpotLight`))
      (`SceneComponent.SetVisibility` (`self.SpotLight`) false true)
      (`AudioComponent.SetSound` _audiotorch "/Game/Audio/Torch/Torcia_Off_02.Torcia_Off_02")
      (`AudioComponent.Play` _audiotorch 0.0)
      (else
        (`SceneComponent.SetVisibility` (`self.SpotLight`) true true)
        (`AudioComponent.SetSound` _audiotorch_2 "/Game/Audio/Torch/Torcia_On_02.Torcia_On_02")
        (`AudioComponent.Play` _audiotorch_2 0.0)))))

(event `EnhancedInput|/Game/Core/Input/IA_TertiaryAction`
  (params (ActionValue :type Boolean) (ElapsedSeconds :type "Float (double-precision)") (TriggeredSeconds :type "Float (double-precision)") (InputAction :type "InputAction Object Reference" :default "/Game/Core/Input/IA_TertiaryAction.IA_TertiaryAction"))
  ; Actions
  (:`Triggered`
    (bind _currentequippeditem (`self.CurrentEquippedItem`)
      (:`then`
        (if (`KismetSystemLibrary.DoesImplementInterface` _currentequippeditem "/Game/Core/EquippableItem/BPI_EquippableItem.BPI_EquippableItem_C")
          (message `/Game/Core/EquippableItem/BPI_EquippableItem.TertiaryUse` (`self.CurrentEquippedItem`) self)))
      (:`else`))))

(fn `AddEnemeyKilled`
  (bind _result (`/Engine/EditorBlueprintResources/StandardMacros.IncrementInt` (`self.EnemiesKilled`))
    (:`  `
      (if (>= _result (`self.VictoryLimit`))
        (`self.Win`)))))

(fn `Camera HeadBobbing`
  (`PlayerController.ClientStartCameraShake` :`self` (`GameplayStatics.GetPlayerController` 0) :`Shake` (select `bool` (> (`KismetMathLibrary.VSize` (`self.GetVelocity`)) 0.0) :`false` "/Game/Core/CameraShakes/LCS_Idle.LCS_Idle_C" :`true` (select `bool` (`self.bSprinting`) :`false` "/Game/Core/CameraShakes/LCS_Walk.LCS_Walk_C" :`true` "/Game/Core/CameraShakes/LCS_Sprint.LCS_Sprint_C" :!type "CameraShakeBase Class Reference"))))

(fn `Heal`
  (params (`Heal Amount` :type "Float (double-precision)"))
  (bind _output_get (set `self.Health` (`KismetMathLibrary.FClamp` (+ (`self.Health`) `Heal Amount`) 0.0 (`self.MaxHealth`))))
  (`KismetSystemLibrary.PrintString` (`KismetStringLibrary.Conv_DoubleToString` _output_get)))

(fn `InitInventory`
  (bind _returnvalue (`|SpawnActorFromClass` "/Game/Core/Weapon/BP_Weapon.BP_Weapon_C" (`self.GetTransform`) "AlwaysSpawn" "MultiplyWithRoot" self self))
  (set `self.Pistol` _returnvalue)
  (bind _returnvalue_2 (`|SpawnActorFromClass` "/Game/Core/Weapon/BP_MeleeWeapon.BP_MeleeWeapon_C" (`self.GetTransform`) "AlwaysSpawn" "MultiplyWithRoot" self self))
  (bind _output_get (set `self.Melee` _returnvalue_2))
  (`/Game/Core/Weapon/BP_MeleeWeapon.OnUnequip` _output_get)
  (`self.EquipItem` (`self.Pistol`)))

(fn `UserConstructionScript`)

(fn `Win`
  (`self.WinImpl`))