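; Enemy character that waits disguised as another mesh, then transforms and attacks the player.
; Player proximity or damage triggers the transformation and starts continuous AI MoveTo pursuit; a hit on the disguise only transforms it.
; While active, a timer fires attacks inside the attack area, playing Chooser-selected montages and sphere-tracing forward to apply point damage.
; Health loss leads to death, which credits the player's kill count and plays a death montage.
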(event `self.ReceiveBeginPlay`
  (bind _asbp_main_character (cast `/Game/Core/BP_MainCharacter` (`GameplayStatics.GetPlayerPawn` 0)))
  (set `self.MainCharacter` _asbp_main_character))

(event `self.ReceiveTick`
  (params (DeltaSeconds :type "Float (single-precision)"))
  (bind (_returnvalue_roll _returnvalue_pitch) (`KismetMathLibrary.BreakRotator` (`self.K2_GetActorRotation`)))
  (bind (_returnvalue_roll_2 _returnvalue_pitch_2 _returnvalue_yaw) (`KismetMathLibrary.BreakRotator` (`KismetMathLibrary.RInterpTo` (`self.K2_GetActorRotation`) (`self.GetControlRotation`) DeltaSeconds (`self.TurnRate`))))
  (if (`self.IsAlive`)
    (`|ExecutionSequence`
      (:`then_0`
        (`self.K2_SetActorRotation` (`KismetMathLibrary.MakeRotator` _returnvalue_roll _returnvalue_pitch _returnvalue_yaw) true))
      (:`then_1`
        (if (`self.bActive`)
          (bind _output_get (set `self.AttackTimer` (`KismetMathLibrary.FClamp` (+ DeltaSeconds (`self.AttackTimer`)) 0.0 (`self.TimeBetweenAttacks`))))
          (if (and (>= _output_get (`self.TimeBetweenAttacks`)) (`self.bAttack`))
            (`self.Attack`)))))))

(event `self.ReceiveControllerChanged`
  (params (OldController :type "Controller Object Reference") (NewController :type "Controller Object Reference"))
  (bind _asaicontroller (cast `AIController` NewController))
  (set `self.AIController` _asaicontroller))

(event `Attack`
  (bind _returnvalue (`self.K2_GetActorLocation`))
  ; Actions
  ;; Attack
  (if (`self.IsAlive`)
    (set `self.AttackTimer` 0.0)
    (bind _result (`|EvaluateChooser2`)
      (:`execute`
        (`|PlayMontage` (`self.Mesh`) _result
          (:`then`
            (bind _outhit (`KismetSystemLibrary.SphereTraceSingle` :`Start` _returnvalue :`End` (+ _returnvalue (* (`self.GetActorForwardVector`) (`self.AttackRange`))) :`Radius` 15.0 :`TraceChannel` "TraceTypeQuery2" :`DrawDebugType` "ForDuration"))
            (bind (_bblockinghit _binitialoverlap _time _distance _location _impactpoint _normal _impactnormal _physmat _hitactor) (`GameplayStatics.BreakHitResult` _outhit))
            (if (and _bblockinghit (== _hitactor (`self.MainCharacter`)))
              (`GameplayStatics.ApplyPointDamage` _hitactor (`self.EnemyDamage`) _normal _outhit (`self.AIController`) self "/Game/Core/Weapon/BP_Damage.BP_Damage_C"))))))))

(event `self.AttackArea.OnComponentBeginOverlap`
  (params (OverlappedComponent :type "PrimitiveComponent Object Reference") (OtherActor :type "Actor Object Reference") (OtherComp :type "PrimitiveComponent Object Reference") (OtherBodyIndex :type Integer) (bFromSweep :type Boolean) (SweepResult :type "HitResult Structure (by ref)"))
  ; Actions
  ;; Attack
  (if (== OtherActor (`self.MainCharacter`))
    (set `self.bAttack` true)))

(event `self.AttackArea.OnComponentEndOverlap`
  (params (OverlappedComponent :type "PrimitiveComponent Object Reference") (OtherActor :type "Actor Object Reference") (OtherComp :type "PrimitiveComponent Object Reference") (OtherBodyIndex :type Integer))
  ; Actions
  ;; Attack
  (if (== OtherActor (`self.MainCharacter`))
    (set `self.bAttack` false)))

(event `FollowActor`
  ; Actions
  (`self.FollowTask`
    (:`then`)
    (:`else`
      (if (and (`self.bActive`) (`self.IsAlive`))
        (bind _maincharacter (`self.MainCharacter`)
          (:`then`
            (bind _asynctaskproxy (`AITask_MoveTo.AIMoveTo` (`self.AIController`) (0.0 0.0 0.0) _maincharacter 70.0 "Default" "Default" true false true "Enable")
              (:`then`
                (set `self.FollowTask` _asynctaskproxy))))
          (:`else`))))))

(event `Transformation`
  ; Actions
  ;; Transformation
  (`|ExecutionSequence`
    (:`then_0`
      (`PrimitiveComponent.SetCollisionEnabled` (`self.DisguiseMesh`) "NoCollision")
      (`SceneComponent.SetVisibility` (`self.DisguiseMesh`) false true))
    (:`then_1`
      (`PrimitiveComponent.SetCollisionEnabled` (`self.Mesh`) "QueryOnly")
      (`SceneComponent.SetVisibility` (`self.Mesh`) true true))
    (:`then_2`
      (`AudioComponent.Play` (`self.Audio`) 0.0))
    (:`then_3`
      (set `self.bActive` true))))

(event `self.DisguiseMesh.OnComponentHit`
  (params (HitComponent :type "PrimitiveComponent Object Reference") (OtherActor :type "Actor Object Reference") (OtherComp :type "PrimitiveComponent Object Reference") (NormalImpulse :type "Vector Structure") (Hit :type "HitResult Structure (by ref)"))
  ; Actions
  ;; Transformation
  ;;; Add VFX
  (`self.Transformation`))

(event `self.ActivationArea.OnComponentBeginOverlap`
  (params (OverlappedComponent :type "PrimitiveComponent Object Reference") (OtherActor :type "Actor Object Reference") (OtherComp :type "PrimitiveComponent Object Reference") (OtherBodyIndex :type Integer) (bFromSweep :type Boolean) (SweepResult :type "HitResult Structure (by ref)"))
  (if (and (`self.bActive`) (`self.IsAlive`))
    _
    (elif (== OtherActor (`self.MainCharacter`))
      (`self.Transformation`)
      (`KismetSystemLibrary.Delay` 0.5)
      (`self.FollowActor`))))

(event `self.ReceivePointDamage`
  (params (Damage :type "Float (single-precision)") (DamageType :type "DamageType Object Reference") (HitLocation :type "Vector Structure") (HitNormal :type "Vector Structure") (HitComponent :type "PrimitiveComponent Object Reference") (BoneName :type Name) (ShotFromDirection :type "Vector Structure") (InstigatedBy :type "Controller Object Reference") (DamageCauser :type "Actor Object Reference") (HitInfo :type "HitResult Structure (by ref)"))
  ; Damaged
  (if (`self.IsAlive`)
    (`|ExecutionSequence`
      (:`then_0`
        (bind _output_get (set `self.Health` (- (`self.Health`) Damage)))
        (if (< _output_get 0.0)
          (`/Game/Core/BP_MainCharacter.AddEnemeyKilled` (`self.MainCharacter`))
          (`self.Death`)))
      (:`then_1`
        (if (not (`self.bActive`))
          (`self.Transformation`)
          (`KismetSystemLibrary.Delay` 0.5)
          (`self.FollowActor`))))))

(event `Death`
  ; Damaged
  (`PrimitiveComponent.SetCollisionEnabled` (`self.Mesh`) "QueryAndPhysics")
  (`PrimitiveComponent.SetCollisionEnabled` (`self.CapsuleComponent`) "NoCollision")
  (`PrimitiveComponent.SetCollisionEnabled` (`self.AttackArea`) "NoCollision")
  (`PrimitiveComponent.SetCollisionEnabled` (`self.ActivationArea`) "NoCollision")
  (bind _result (`|EvaluateChooser2`)
    (:`execute`
      (`|PlayMontage` (`self.Mesh`) _result
        (:`then`
          (`AudioParameterControllerInterface.SetTriggerParameter` (`self.Audio`) "Death"))
        (:`OnBlendOut`
          (set `self.bDeathAnimation` true))))))

(fn `IsAlive`
  (returns (ReturnValue :type Boolean))
  (return (> (`self.Health`) 0.0)))

(fn `UserConstructionScript`)